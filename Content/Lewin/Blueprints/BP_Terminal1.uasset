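; Terminal Blueprint tied to a rover ID, with replicated screen, animation, special mode, widget, battery and access-denied state.
; GetRoverDataByID scans RoverTable row by row and returns the entry whose ID matches RoverID.
; The Battery RepNotify copies the value into BatteryTarget when the liquid material instance is valid.
; The other RepNotifies, the construction script and the TerminalType construct and BeginPlay hooks are empty.
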(fn ConstructionScript)

(fn GetRoverDatabyID
  (bind _outrownames (DataTable|GetDataTableRowNames "/Game/Balduin/RoverTable.RoverTable"))
  (for _array_element _outrownames
    (bind _returnvalue (Utilities|GetDataTableRow "/Game/Balduin/RoverTable.RoverTable" _array_element)
      (:then
        (if (== (.ID (Utilities|Struct|BreakST_Rover _returnvalue)) (Variables|Default|GetRoverID))
          (return _returnvalue))))))

(fn OnRepScreenon)

(fn OnRepStartAnimation)

(fn OnRepSpecialModeActive)

(fn OnRepHideWidgetWB)

(fn OnRepBattery
  (Utilities|IsValid (Variables|Default|GetLiquidInstanceMAT)
    (:Is%20Valid
      (Variables|Default|SetBatteryTarget (Variables|Default|GetBattery)))))

(fn OnRepAccessDenied)

(fn TerminalTypeConstruct)

(fn TerminalTypeEventBeginPlay)