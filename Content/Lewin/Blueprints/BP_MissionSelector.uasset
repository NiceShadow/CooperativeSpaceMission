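; Mission selector station actor where players adjust X/Y values on a select screen and log in to three assign slots for the chosen mission.
; Five interaction points are gated by overlap boxes and occupancy, with local outlines and progress widgets.
; The server forwards X/Y changes and multicasts occupancy updates.
; OnRep handlers for mission activation, start and stop switch interaction collision and clear assignments, using flipped booleans as replicated triggers.
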(event OnComponentBeginOverlap(BoxX)
  (params (OverlappedComponent :type Primitive%20Component%20Object%20Reference) (OtherActor :type Actor%20Object%20Reference) (OtherComp :type Primitive%20Component%20Object%20Reference) (OtherBodyIndex :type Integer) (bFromSweep :type Boolean) (SweepResult :type Hit%20Result%20Structure%20%28by%20ref%29))
  ;[1 1 1] Reset characters Trace if (end) overlapping necessary interact overalp box
  (Class|BPOutline|ResetInteractionTrace(Message) OtherActor))

(event OnComponentEndOverlap(BoxX)
  (params (OverlappedComponent :type Primitive%20Component%20Object%20Reference) (OtherActor :type Actor%20Object%20Reference) (OtherComp :type Primitive%20Component%20Object%20Reference) (OtherBodyIndex :type Integer))
  ;[1 1 1] Reset characters Trace if (end) overlapping necessary interact overalp box
  (Class|BPOutline|ResetInteractionTrace(Message) OtherActor))

(event OnComponentBeginOverlap(BoxY)
  (params (OverlappedComponent :type Primitive%20Component%20Object%20Reference) (OtherActor :type Actor%20Object%20Reference) (OtherComp :type Primitive%20Component%20Object%20Reference) (OtherBodyIndex :type Integer) (bFromSweep :type Boolean) (SweepResult :type Hit%20Result%20Structure%20%28by%20ref%29))
  ;[1 1 1] Reset characters Trace if (end) overlapping necessary interact overalp box
  (Class|BPOutline|ResetInteractionTrace(Message) OtherActor))

(event OnComponentEndOverlap(BoxY)
  (params (OverlappedComponent :type Primitive%20Component%20Object%20Reference) (OtherActor :type Actor%20Object%20Reference) (OtherComp :type Primitive%20Component%20Object%20Reference) (OtherBodyIndex :type Integer))
  ;[1 1 1] Reset characters Trace if (end) overlapping necessary interact overalp box
  (Class|BPOutline|ResetInteractionTrace(Message) OtherActor))

(event OnComponentBeginOverlap(BoxAssign)
  (params (OverlappedComponent :type Primitive%20Component%20Object%20Reference) (OtherActor :type Actor%20Object%20Reference) (OtherComp :type Primitive%20Component%20Object%20Reference) (OtherBodyIndex :type Integer) (bFromSweep :type Boolean) (SweepResult :type Hit%20Result%20Structure%20%28by%20ref%29))
  ;[1 1 1] Reset characters Trace if (end) overlapping necessary interact overalp box
  (Class|BPOutline|ResetInteractionTrace(Message) OtherActor))

(event OnComponentEndOverlap(BoxAssign)
  (params (OverlappedComponent :type Primitive%20Component%20Object%20Reference) (OtherActor :type Actor%20Object%20Reference) (OtherComp :type Primitive%20Component%20Object%20Reference) (OtherBodyIndex :type Integer))
  ;[1 1 1] Reset characters Trace if (end) overlapping necessary interact overalp box
  (Class|BPOutline|ResetInteractionTrace(Message) OtherActor))

(event Custom|UpdateOpeningPercentX
  (params (newPercent :type Float%20%28single-precision%29))
  ;[1 1 1] UpdateOpeningProgressX
  (bind _aswb_interaction (Utilities|Casting|CastToWB_Interaction (UserInterface|GetUserWidgetObject (Variables|Default|GetWidgetInteractionX))))
  (Default|SetProgress _aswb_interaction newPercent))

(event Custom|ChangeY_value
  (params (add :type Boolean) (in :type Boolean))
  ;[1 1 1] Update XY valus on server
  (Default|IncreaseYvalue (Variables|Default|GetMissionSelectScreen) add in))

(event Custom|SetInteractionToLeaveOption
  (params (ID :type Integer) (in :type Boolean))
  ;[1 1 1] Show Logout option after loggin in to an assign button
  (if in
    (Variables|Default|SetLogoutID? ID)
    (else
      (Variables|Default|SetLogoutID? -1)
      (if (> ID 1)
        (CallFunction|UpdateOpeningAssing ID 0.0))))
  (bind _aswb_interaction (Utilities|Casting|CastToWB_Interaction (Utilities|Select :Index ID :Option%200 0 :Option%201 0 :Option%202 (UserInterface|GetUserWidgetObject (Variables|Default|GetWidgetInteractionA1)) :Option%203 (UserInterface|GetUserWidgetObject (Variables|Default|GetWidgetInteractionA2)) :Option%204 (UserInterface|GetUserWidgetObject (Variables|Default|GetWidgetInteractionA3)))))
  (Default|LogoutOption _aswb_interaction in))

(event Custom|CacnelX
  ;[1 1 1] Update XY valus on server
  (Default|CancelX (Variables|Default|GetMissionSelectScreen)))

(event Custom|CancelY
  ;[1 1 1] Update XY valus on server
  (Default|CancelY (Variables|Default|GetMissionSelectScreen)))

(event Custom|MissionStart
  ;[1 1 1] Start Mission
  (Variables|Default|SetStartMission (not (Variables|Default|GetStartMission)))
  (Utilities|FlowControl|Delay 1.0)
  (Variables|Default|SetDeactivateMissionEffect (not (Variables|Default|GetDeactivateMissionEffect))))

(event Custom|ShowInteraction
  (params (In :type Boolean) (ID :type Integer) (useHidden :type Boolean))
  (bind _cubex (Variables|Default|GetCubeX))
  (bind _cubey (Variables|Default|GetCubeY))
  (bind _widgetinteractiona2 (Variables|Default|GetWidgetInteractionA2))
  (bind _a1 (Variables|Default|GetA1))
  (bind _a2 (Variables|Default|GetA2))
  (bind _a3 (Variables|Default|GetA3))
  (bind _widgetinteractionx (Variables|Default|GetWidgetInteractionX))
  (bind _widgetinteractiona3 (Variables|Default|GetWidgetInteractionA3))
  (bind _widgetinteractiona1 (Variables|Default|GetWidgetInteractionA1))
  (bind _widgetinteractiony (Variables|Default|GetWidgetInteractionY))
  (bind _returnvalue (Utilities|Select :Index ID :Option%200 _cubex :Option%201 _cubey :Option%202 _a1 :Option%203 _a2 :Option%204 _a3))
  (bind _returnvalue_2 (Utilities|Select :Index ID :Option%200 _widgetinteractionx :Option%201 _widgetinteractiony :Option%202 _widgetinteractiona1 :Option%203 _widgetinteractiona2 :Option%204 _widgetinteractiona3))
  ;[1 1 1] Show Interaction info widgets locally
  (if useHidden
    (if In
      (Rendering|SetRenderCustomDepth _returnvalue false))
    (Development|SetHiddeninGame _returnvalue_2 In false)
    (else
      (Rendering|SetRenderCustomDepth _returnvalue In)
      (Rendering|SetVisibility _returnvalue_2 In false))))

(event Custom|UpdateOpeningPercentY
  (params (newPercent :type Float%20%28single-precision%29))
  ;[1 1 1] UpdateOpeningProgressX
  (bind _aswb_interaction (Utilities|Casting|CastToWB_Interaction (UserInterface|GetUserWidgetObject (Variables|Default|GetWidgetInteractionY))))
  (Default|SetProgress _aswb_interaction newPercent))

(event Custom|ChangeX_value
  (params (add :type Boolean) (in :type Boolean))
  ;[1 1 1] Update XY valus on server
  (Default|IncreaseXvalue (Variables|Default|GetMissionSelectScreen) add in))

(event Custom|SetOccupiedOnServer
  (params (Occupied :type Boolean) (ID :type Integer))
  ;[1 1 1] Set Occupied On Server
  (Utilities|Array|SetArrayElem (Variables|Default|GetOccupied) ID Occupied)
  (CallFunction|UpdateInteractionWidgetMulticast (not Occupied) ID))

(event Custom|OnMissionActivated
  (params (In :type Boolean))
  ;[1 1 1] Cancel Mission Assign for all if Mission activated (selected)
  (bind _output_get (Variables|Default|SetMissionActivateReplicated In))
  (if (not _output_get)
    (bind _asbp_our_gm (Utilities|Casting|CastToBP_OurGM (Game|GetGameMode)))
    (Default|ThrowPlayersOutOfMissionAssignment _asbp_our_gm)))

(event Custom|UpdateInteractionWidgetMulticast
  (params (bNewVisibility :type Boolean) (ID :type Integer))
  ;[1 1 1] Update interaction widget in case someone different currently wants to interact
  (if bNewVisibility
    (if (Variables|Default|GetWantToFocus)
      (if (== ID (Variables|Default|GetFocusingID))
        (CallFunction|ShowInteraction bNewVisibility ID false :!label _label)))
    (else
      (goto _label))))

(event Custom|UpdateOpeningAssing
  (params (Index :type Integer) (InPercent :type Float%20%28single-precision%29))
  ;[1 1 1] UpdateOpeningProgress Assign Button
  (bind _aswb_interaction (Utilities|Casting|CastToWB_Interaction (UserInterface|GetUserWidgetObject (Utilities|Select :Index Index :Option%200 0 :Option%201 0 :Option%202 (Variables|Default|GetWidgetInteractionA1) :Option%203 (Variables|Default|GetWidgetInteractionA2) :Option%204 (Variables|Default|GetWidgetInteractionA3)))))
  (Default|SetProgress _aswb_interaction InPercent))

(event Custom|MissionStop
  ;[1 1 1] Stop Mission
  (Variables|Default|SetStopMission (not (Variables|Default|GetStopMission))))

(event EventOutlinewithIDChar
  (params (ID :type Integer) (In :type Boolean) (Char :type Character%20Object%20Reference))
  ;[1 1 1] Outline if available
  (Variables|Default|SetWantToFocus In)
  (Variables|Default|SetFocusingID ID)
  (if (Variables|Default|GetWantToFocus)
    (if (Math|Boolean|ANDBoolean (or (== (Variables|Default|GetLogoutID?) (Variables|Default|GetFocusingID)) (not (Utilities|Array|Get(acopy) (Variables|Default|GetOccupied) (Variables|Default|GetFocusingID)))) (CallFunction|IsOverlappingTrigger Char (Variables|Default|GetFocusingID)) (select (> (Variables|Default|GetFocusingID) 1) (or (== (Variables|Default|GetLogoutID?) (Variables|Default|GetFocusingID)) (< (Variables|Default|GetLogoutID?) 0)) true))
      (Variables|Default|SetFocused true)
      (CallFunction|ShowInteraction (Variables|Default|GetFocused) (Variables|Default|GetFocusingID) false :!label _label))
    (else
      (Variables|Default|SetFocused false)
      (goto _label))))

(event EventBeginPlay
  ;[1 1 1] Event Begin Play
  (Utilities|FlowControl|Delay 0.2)
  ;[1 1 1] Deactivate Mission Selector interaction at beginning if no mission currently selected
  (if (not (Variables|Default|GetMissionActivateReplicated))
    (CallFunction|EnableAssignInteractActors false false false)))

(fn ConstructionScript)

(fn IsOverlappingTrigger
  (params (Other :type Actor%20Object%20Reference) (ID :type Integer))
  (bind _boxassign (Variables|Default|GetBoxAssign))
  (return (Collision|IsOverlappingActor (Utilities|Select :Index ID :Option%200 (Variables|Default|GetBoxX) :Option%201 (Variables|Default|GetBoxY) :Option%202 _boxassign :Option%203 _boxassign :Option%204 _boxassign) Other :!class /Script/Engine.PrimitiveComponent)))

(fn OnRepMissionActivateReplicated
  (bind _occupied (Variables|Default|GetOccupied))
  (Development|SetHiddeninGame (Variables|Default|Getclosing) (Variables|Default|GetMissionActivateReplicated) false)
  (CallFunction|EnableAssignInteractActors (Variables|Default|GetMissionActivateReplicated) false false)
  (if (not (Variables|Default|GetMissionActivateReplicated))
    (Utilities|Array|SetArrayElem _occupied 2 false)
    (Utilities|Array|SetArrayElem _occupied 3 false)
    (Utilities|Array|SetArrayElem _occupied 4 false)))

(fn EnableAssignInteractActors
  (params (setActivated :type Boolean) (andXY :type Boolean) (onlyXY :type Boolean))
  (LocalVariables|SetActivate setActivated)
  (if onlyXY
    (bind _asbp_interaction_actor (Utilities|Casting|CastToBP_InteractionActor (Variables|/Script/Engine.ChildActorComponent|GetChildActor (Variables|Default|GetChildActorX)) :!label _label))
    (Default|ActivateCollision _asbp_interaction_actor (LocalVariables|GetActivate))
    (bind _asbp_interaction_actor_2 (Utilities|Casting|CastToBP_InteractionActor (Variables|/Script/Engine.ChildActorComponent|GetChildActor (Variables|Default|GetChildActorY))))
    (Default|ActivateCollision _asbp_interaction_actor_2 (LocalVariables|GetActivate))
    (else
      (bind _asbp_interaction_actor_3 (Utilities|Casting|CastToBP_InteractionActor (Variables|/Script/Engine.ChildActorComponent|GetChildActor (Variables|Default|GetChildActorAssign1))))
      (Default|ActivateCollision _asbp_interaction_actor_3 (LocalVariables|GetActivate))
      (bind _asbp_interaction_actor_4 (Utilities|Casting|CastToBP_InteractionActor (Variables|/Script/Engine.ChildActorComponent|GetChildActor (Variables|Default|GetChildActorAssign2))))
      (Default|ActivateCollision _asbp_interaction_actor_4 (LocalVariables|GetActivate))
      (bind _asbp_interaction_actor_5 (Utilities|Casting|CastToBP_InteractionActor (Variables|/Script/Engine.ChildActorComponent|GetChildActor (Variables|Default|GetChildActorAssign3))))
      (Default|ActivateCollision _asbp_interaction_actor_5 (LocalVariables|GetActivate))
      (if andXY
        (goto _label)))))

(fn OnRepDeactivateMissionEffect
  (Development|SetHiddeninGame (Variables|Default|Getclosing) false false))

(fn OnRepStartMission
  (CallFunction|EnableAssignInteractActors false true false))

(fn OnRepStopMission
  (bind _occupied (Variables|Default|GetOccupied))
  (CallFunction|EnableAssignInteractActors true true true)
  (Utilities|Array|SetArrayElem _occupied 2 false)
  (Utilities|Array|SetArrayElem _occupied 3 false)
  (Utilities|Array|SetArrayElem _occupied 4 false))