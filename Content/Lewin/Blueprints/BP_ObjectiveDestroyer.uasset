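; Actor that destroys an objective foliage instance where it spawns, with a destructible break effect.
; On BeginPlay a short upward trace finds the foliage instance and removes it, then damages the Destructible component.
; A timeline shrinks the debris while delays disable its collision and later destroy it.
; An OnlyDestroyObjective flag, set after a delay by an event intended for late-joining players, skips the effect.
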(event Custom|SetOnlyDestroyObjectiveMode
  ;[1 1 1] Destroy without destructable effect (for players who later joined the server)
  (Utilities|FlowControl|Delay 1.0)
  (Variables|Default|SetOnlyDestroyObjective true))

(event EventBeginPlay
  ;[1 1 1] Trace Instance and remove it
  (bind (_outhit _returnvalue) (Collision|LineTraceByChannel (Transformation|GetActorLocation) (+ (Transformation|GetActorLocation) "0, 0,10.000000") "TraceTypeQuery3" false 0 "None"))
  (if _returnvalue
    (bind _asfoliage_instanced_static_mesh_component (Utilities|Casting|CastToFoliageInstancedStaticMeshComponent (.HitComponent (Collision|BreakHitResult _outhit))))
    (Class|InstancedStaticMeshComponent|RemoveInstance _asfoliage_instanced_static_mesh_component (.HitItem (Collision|BreakHitResult _outhit)))
    (if (Variables|Default|GetOnlyDestroyObjective)
      ;[1 1 1] Destroy without destructable effect (for players who later joined the server)
      (Components|DestroyComponent (Variables|Default|GetDestructible))
      (else
        ;[1 1 1] Start Destruction effect
        (Utilities|FlowControl|Sequence
          (:then_0
            (Class|DestructibleComponent|ApplyDamage (Variables|Default|GetDestructible) 1.0 (Transformation|GetActorLocation) (Math|Vector|MakeVector 0.0 0.0 0.0) 0.0)
            (bind _newtrack_0 (Timeline|Disappear PlayFromStart)
              (:Update
                (Transformation|SetWorldScale3D (Variables|Default|GetDestructible) (Math|Vector|Lerp(Vector) (Math|Conversions|ToVector(Float) 1.0) (Math|Conversions|ToVector(Float) 0.0) _newtrack_0)))))
          (:then_1
            (Utilities|FlowControl|Delay 0.8)
            (Collision|SetCollisionEnabled (Variables|Default|GetDestructible) "NoCollision")
            (Class|PrimitiveComponent|SetLinearDamping (Variables|Default|GetDestructible) 0.3)
            (Utilities|FlowControl|Delay 1.5)
            (Components|DestroyComponent (Variables|Default|GetDestructible))))))))

(fn ConstructionScript)