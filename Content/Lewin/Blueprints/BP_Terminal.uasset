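; Replicated rover console terminal that players focus on and occupy, showing the linked rover's scene-capture feed and battery level.
; RoverID selects table data at BeginPlay, when a transition actor also spawns, and TerminalSpecialityToggler selects a variant without battery and joystick.
; OnRep functions drive screen material, intro widget, bouncing screensaver, access-denied text and rover special mode, which has per-type conditions.
; A one-second timer samples rover battery, which Tick eases into a liquid-fill material.
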(event OnComponentBeginOverlap(Box)
  (params (OverlappedComponent :type Primitive%20Component%20Object%20Reference) (OtherActor :type Actor%20Object%20Reference) (OtherComp :type Primitive%20Component%20Object%20Reference) (OtherBodyIndex :type Integer) (bFromSweep :type Boolean) (SweepResult :type Hit%20Result%20Structure%20%28by%20ref%29))
  ;[1 1 1] Reset interation trace
  (Class|BPOutline|ResetInteractionTrace(Message) OtherActor))

(event Custom|ShowInteractionWidget
  (params (bNewVisibility :type Boolean))
  ;[1 1 1] Show interaction widget
  (Rendering|SetVisibility (Variables|Default|GetWidgetInteraction) bNewVisibility false)
  (CallFunction|ShowOutline bNewVisibility))

(event Custom|ToggleOnAndSetRover
  (params (On :type Boolean) (CurrentRoverPawn :type Pawn%20Object%20Reference) (SceneCaptureMaterialIndex :type Integer))
  ;[1 1 1] Turn on/off terminal and setup rover reference corresponding scene capture material for screen
  (bind _output_get (Variables|Default|SetTurnedOn On))
  (if _output_get
    (Variables|Default|SetSceneCaptureMaterialIndex SceneCaptureMaterialIndex)
    (if (not (Variables|Default|GetTerminalSpecialityToggler))
      (bind _output_get_2 (Variables|Default|SetCurrentRoverPawn CurrentRoverPawn))
      (CallFunction|SetCurrentRover (Variables|Default|GetCounterTerminal) _output_get_2)
      (CallFunction|UpdateRoverData))
    (else
      (Variables|Default|SetCurrentRoverPawn 0)
      (Variables|Default|SetSpecialModeActive false)
      (if (not (Variables|Default|GetTerminalSpecialityToggler))
        (Utilities|Time|ClearandInvalidateTimerbyHandle (Variables|Default|GetUpdateRoverDataTimer))))))

(event Custom|ToggleSpecialMode
  ;[1 1 1] Toggle special mode
  (if (Variables|Default|GetSpecialModeActive)
    (bind _asparent_rover (Utilities|Casting|CastToParentRover (Variables|Default|GetCurrentRoverPawn)))
    (if (not (Utilities|Enum|Equal(Enum) (Variables|/Game/CustomVehicle/ParentRover.ParentRover_C|GetRoverType _asparent_rover) "NewEnumerator4"))
      (Variables|Default|SetSpecialModeActive false))
    (else
      (bind _asparent_rover_2 (Utilities|Casting|CastToParentRover (Variables|Default|GetCurrentRoverPawn)))
      (if (Utilities|Enum|Equal(Enum) (Variables|/Game/CustomVehicle/ParentRover.ParentRover_C|GetRoverType _asparent_rover_2) "NewEnumerator2")
        (if (Variables|/Game/CustomVehicle/ParentRover.ParentRover_C|GetCanScan _asparent_rover_2)
          (Variables|Default|SetSpecialModeActive true :!label _label))
        (elif (Utilities|Enum|Equal(Enum) (Variables|/Game/CustomVehicle/ParentRover.ParentRover_C|GetRoverType _asparent_rover_2) "NewEnumerator4")
          (bind _yes_sir (CallFunction|HasReturnerMainObjective))
          (if _yes_sir
            (goto _label))
          (else
            (goto _label)))))))

(event Custom|HideWidgetScreen
  ;[1 1 1] HideScreen
  (Variables|Default|SetHideWidgetWB (not (Variables|Default|GetHideWidgetWB))))

(event Custom|ChangeMovementStickMode
  (params (CurrentMovementStickMode :type E_TerminalMovementState%20Enum :default "NewEnumerator1"))
  ;[1 1 1] Update Movement Stick on server
  (Variables|Default|SetCurrentMovementStickMode CurrentMovementStickMode))

(event Custom|UpdateRoverData
  ;[1 1 1] Update data from rover
  (bind _returnvalue (Utilities|Time|SetTimerbyEvent (delegate Custom|UpdateData) 1.0 true))
  (Variables|Default|SetUpdateRoverDataTimer _returnvalue))

(event Custom|UpdateData
  ;[1 1 1] Update data from rover
  (bind _asparent_rover (Utilities|Casting|CastToParentRover (Variables|Default|GetCurrentRoverPawn)))
  (Variables|Default|SetBattery (/ (Variables|/Game/CustomVehicle/ParentRover.ParentRover_C|GetCurrentBattery _asparent_rover) (Variables|/Game/CustomVehicle/ParentRover.ParentRover_C|GetMaxBattery _asparent_rover))))

(event Custom|DenyAccess
  ;[1 1 1] Deny Access and show for all
  (Variables|Default|SetAccessDenied true)
  (Utilities|FlowControl|Delay 1.5)
  (Variables|Default|SetAccessDenied false))

(event Custom|ToggleHideBlackBG
  (params (NewHidden :type Boolean) (Duration :type Float%20%28single-precision%29))
  ;[1 1 1] Toggle hide background plane right behind monitor
  (Utilities|FlowControl|Delay Duration)
  (Development|SetHiddeninGame (Variables|Default|GetBlackBG) NewHidden false))

(event Custom|LocallyBlenOutGlass
  (params (Disappear :type Boolean) (Duration :type Float%20%28single-precision%29))
  ;[1 1 1] Blend out Glass locally to improve enter transition experience
  (Utilities|IsValid (Variables|Default|GetGlassInst)
    (:Is%20Valid
      _)
    (:Is%20Not%20Valid
      (bind _returnvalue (Rendering|Material|CreateDynamicMaterialInstance (Variables|Default|Getconsole_screen) 0 "/Game/Lewin/Blueprints/TestMaterials/M_Glass_Inst.M_Glass_Inst" "None" :!class /Script/Engine.PrimitiveComponent))
      (Variables|Default|SetGlassInst _returnvalue)))
  (Rendering|Material|SetMaterial (Variables|Default|Getconsole_screen) 0 (Variables|Default|GetGlassInst))
  (if Disappear
    (Components|Timeline|SetPlayRate (Variables|Default|GetBlendOutGlass) (/ 1.0 Duration))
    (bind _newtrack_0 (Timeline|BlendOutGlass PlayFromStart)
      (:Update
        (Rendering|Material|SetScalarParameterValue (Variables|Default|GetGlassInst) "OpacityMultiplier" (Math|Float|Lerp 1.0 0.0 _newtrack_0) :!class /Script/Engine.MaterialInstanceDynamic)))
    (else
      (Rendering|Material|SetScalarParameterValue (Variables|Default|GetGlassInst) "OpacityMultiplier" 1.0 :!class /Script/Engine.MaterialInstanceDynamic))))

(event Custom|SetSpecialModeDirectly
  (params (SpecialModeActive :type Boolean))
  ;[1 1 1] Toggle special mode
  (Variables|Default|SetSpecialModeActive SpecialModeActive))

(event Custom|PlayAnimationScreenSaver
  (params (In :type Boolean))
  (if In
    (Transformation|SetRelativeLocation (Variables|Default|GetPatch) (Math|Vector|MakeVector (Math|Random|RandomFloatinRange 0.0 6e+01) (Math|Random|RandomFloatinRange 0.0 6e+01) 0.0) false false)
    (bind _returnvalue (Utilities|Time|SetTimerbyFunctionName 0 "SP" 0.01 true))
    (else
      (Utilities|Time|ClearandInvalidateTimerbyHandle _returnvalue))))

(event Custom|HideInteraction
  (params (NewHidden :type Boolean))
  ;[1 1 1] Toggle Hide interaction widget
  (Development|SetHiddeninGame (Variables|Default|GetWidgetInteraction) NewHidden false))

(event Custom|UpdateOpeningPercent
  (params (newPercent :type Float%20%28single-precision%29))
  ;[1 1 1] UpdateOpeningProgress
  (bind _aswb_interaction (Utilities|Casting|CastToWB_Interaction (UserInterface|GetUserWidgetObject (Variables|Default|GetWidgetInteraction))))
  (Default|SetProgress _aswb_interaction newPercent))

(event Custom|ShowOutline
  (params (show :type Boolean))
  ;[1 1 1] Toggle Outline
  (Rendering|SetRenderCustomDepth (Variables|Default|Getconsole_table) show))

(event Custom|StartWidgetScreenAnimation
  ;[1 1 1] Start widget Screen animation
  (Variables|Default|SetStartAnimation (not (Variables|Default|GetStartAnimation))))

(event Custom|SetOccupiedOnServer
  (params (Occupied :type Boolean))
  ;[1 1 1] Set Occupied On Server and update interaction feedback
  (bind _output_get (Variables|Default|SetOccupied Occupied))
  (CallFunction|UpdateInteractionWidgetMulticast (not _output_get)))

(event Custom|UpdateInteractionWidgetMulticast
  (params (bNewVisibility :type Boolean))
  ;[1 1 1] Set Occupied On Server and update interaction feedback
  (if bNewVisibility
    (if (Variables|Default|GetFocused)
      (CallFunction|ShowInteractionWidget bNewVisibility :!label _label))
    (else
      (goto _label))))

(event Custom|SetCurrentRover
  (params (CurrentRoverPawn :type Pawn%20Object%20Reference))
  ;[1 1 1] Update Rover reference on server
  (Variables|Default|SetCurrentRoverPawn CurrentRoverPawn))

(event Custom|SetTerminalScreen
  (params (ScreenOn :type Boolean))
  ;[1 1 1] Replicated Change Terminal Screen Material
  (Variables|Default|SetScreenOn ScreenOn))

(event EventBeginPlay
  ;[1 1 1] Event Begin Play
  ;;[1 1 1] Get Rover Data from DataTable and Spawn Transition Pawn
  (Variables|Default|SetRoverData (CallFunction|GetRoverDatabyID))
  (bind _returnvalue (Game|SpawnActorfromClass "/Game/Lewin/Blueprints/CurrentlyNotRelevant/BP_TransitionTerminal.BP_TransitionTerminal_C" (Transformation|GetWorldTransform (Variables|Default|GetArrowView)) "Undefined" 0 0))
  (Variables|Default|SetTransitionActorRef _returnvalue)
  (CallFunction|TerminalTypeEventBeginPlay)
  (Utilities|FlowControl|Delay 7.0))

(event EventTick
  (params (DeltaSeconds :type Float%20%28single-precision%29))
  ;[1 1 1] Eventing for smooth finterp of battery level
  (if (not (Variables|Default|GetTerminalSpecialityToggler))
    (if (not (Math|Float|NearlyEqual(Float) (Variables|Default|GetCurrentBatteryFinterp) (Variables|Default|GetBatteryTarget) 0.002))
      (bind _output_get (Variables|Default|SetCurrentBatteryFinterp (Math|Interpolation|FInterpTo (Variables|Default|GetCurrentBatteryFinterp) (Variables|Default|GetBatteryTarget) DeltaSeconds (Variables|Default|GetBatteryFillSmoothSpeed))))
      (Rendering|Material|SetScalarParameterValue (Variables|Default|GetLiquidInstanceMAT) "Liquid_FillHeight" (Math|Float|Lerp -0.4 0.5 _output_get) :!class /Script/Engine.MaterialInstanceDynamic))))

(event EventOutlineChar
  (params (In :type Boolean) (Chat :type Character%20Object%20Reference))
  ;[1 1 1] Locally show outline & interaction widget (only if not occupied)
  (if In
    (if (Variables|Default|GetTurnedOn)
      (if (Collision|IsOverlappingActor (Variables|Default|GetBox) Chat :!class /Script/Engine.PrimitiveComponent)
        (bind _output_get (Variables|Default|SetFocused In :!label _label))
        (if _output_get
          (if (not (Variables|Default|GetOccupied))
            (CallFunction|ShowInteractionWidget (Variables|Default|GetFocused) :!label _label_2))
          (else
            (goto _label_2)))))
    (else
      (goto _label))))

(fn ConstructionScript
  (CallFunction|TerminalTypeConstruct)
  ;[1 1 1] Dev
  (Rendering|Components|TextRender|SetText (Variables|Default|GetTextRender) (Utilities|Text|FormatText "TM_ID: {ID}" (Variables|Default|GetTerminalID))))

(fn GetRoverDatabyID
  (bind _outrownames (DataTable|GetDataTableRowNames "/Game/Balduin/RoverTable.RoverTable"))
  (for _array_element _outrownames
    (bind _returnvalue (Utilities|GetDataTableRow "/Game/Balduin/RoverTable.RoverTable" _array_element)
      (:then
        (if (== (.ID (Utilities|Struct|BreakST_Rover _returnvalue)) (Variables|Default|GetRoverID))
          (return _returnvalue))))))

(fn OnRepScreenon
  (bind _roverdata (Variables|Default|GetRoverData))
  (bind _scenecapturematerials (Utilities|Struct|BreakST_Rover _roverdata))
  (if (Variables|Default|GetScreenOn)
    (if (<= (Utilities|Array|Length _scenecapturematerials) 0)
      ;[1 1 1] Cleint doesn't know RoverData when joining and this on rep get called before EventBegin Play
      (Rendering|Material|SetMaterial (Variables|Default|GetScreenMaterial) 0 (Utilities|Array|Get(acopy) (Utilities|Struct|BreakST_Rover (CallFunction|GetRoverDatabyID)) (Variables|Default|GetSceneCaptureMaterialIndex)))
      (else
        (Rendering|Material|SetMaterial (Variables|Default|GetScreenMaterial) 0 (Utilities|Array|Get(acopy) _scenecapturematerials (Variables|Default|GetSceneCaptureMaterialIndex)))))
    (CallFunction|ToggleHideBlackBG true 2.0)
    (else
      (Rendering|Material|SetMaterial (Variables|Default|GetScreenMaterial) 0 (Variables|Default|GetScreenOffMaterial))
      (CallFunction|ToggleHideBlackBG false 0.0))))

(fn OnRepStartAnimation
  (Development|SetHiddeninGame (Variables|Default|GetScreenWidget) false false)
  (Development|SetHiddeninGame (Variables|Default|GetPatch) true false)
  (bind _aswb_terminal_screen (Utilities|Casting|CastToWB_TerminalScreen (UserInterface|GetUserWidgetObject (Variables|Default|GetScreenWidget))))
  (Default|StartAnimation _aswb_terminal_screen (Utilities|Struct|BreakST_Rover (Variables|Default|GetRoverData))))

(fn OnRepSpecialModeActive
  (bind _specialmodeactive (Variables|Default|GetSpecialModeActive))
  (bind _currentroverpawn (Variables|Default|GetCurrentRoverPawn))
  (Rendering|Components|TextRender|SetText (Variables|Default|GetSpecialInfo) (select (Variables|Default|GetSpecialModeActive) (Utilities|Text|MakeLiteralText "1") (Utilities|Text|MakeLiteralText "0")))
  (Utilities|IsValid _currentroverpawn
    (:Is%20Valid
      (bind _asparent_rover (Utilities|Casting|CastToParentRover _currentroverpawn))
      (Default|ActivateSpecialMode _asparent_rover _specialmodeactive)
      (Class|BPRoverChildInterface|RunSpecialMode(Message) _asparent_rover _specialmodeactive))))

(fn OnRepHideWidgetWB
  (Development|SetHiddeninGame (Variables|Default|GetScreenWidget) true false)
  (Development|SetHiddeninGame (Variables|Default|GetPatch) false false))

(fn OnRepBattery
  (Utilities|IsValid (Variables|Default|GetLiquidInstanceMAT)
    (:Is%20Valid
      (Variables|Default|SetBatteryTarget (Variables|Default|GetBattery)))))

(fn OnRepAccessDenied
  (Development|SetHiddeninGame (Variables|Default|GetACCESS%20DENIED%20Text) (not (Variables|Default|GetAccessDenied)) false))

(fn TerminalTypeConstruct
  ;[1 1 1] Dev
  (Rendering|Components|TextRender|SetTextRenderColor (Variables|Default|GetTextRender) (select (Variables|Default|GetTerminalSpecialityToggler) (Math|Color|MakeColor 0 0 255 1) (Math|Color|MakeColor 255 255 255 1)))
  (Rendering|SetVisibility (Variables|Default|GetSpecialInfo) (Variables|Default|GetTerminalSpecialityToggler) false)
  (if (Variables|Default|GetTerminalSpecialityToggler)
    (Rendering|SetVisibility (Variables|Default|Getbattery_handle) false true)))

(fn TerminalTypeEventBeginPlay
  (if (Variables|Default|GetTerminalSpecialityToggler)
    (Class|SkeletalMeshComponent|SetAnimClass (Variables|Default|Getjoystick_active_skeletal)))
  (bind _returnvalue (Rendering|Material|CreateDynamicMaterialInstance (Variables|Default|GetLiquid) 0 "/Game/other/RealLiquidX/M/MI_LiquidX_02.MI_LiquidX_02" "None" :!class /Script/Engine.PrimitiveComponent))
  (bind _output_get (Variables|Default|SetLiquidInstanceMAT _returnvalue))
  (Rendering|Material|SetMaterial (Variables|Default|GetLiquid) 0 _output_get)
  (Utilities|IsValid (Variables|Default|GetCurrentRoverPawn)
    (:Is%20Valid
      (CallFunction|UpdateData))))

(fn HasReturnerMainObjective
  (bind _asbp_our_game_state (Utilities|Casting|CastToBP_OurGameState (Game|GetGameState)))
  (bind _outrownames (DataTable|GetDataTableRowNames "/Game/Balduin/Objectives.Objectives"))
  (for _array_element _outrownames
    (bind _returnvalue (Utilities|GetDataTableRow "/Game/Balduin/Objectives.Objectives" _array_element)
      (:then
        (if (Utilities|Enum|Equal(Enum) (.Type (Utilities|Struct|BreakST_Objective _returnvalue)) "NewEnumerator1")
          (if (Utilities|Array|ContainsItem (Variables|/Game/Lewin/Blueprints/BP_OurGameState.BP_OurGameState_C|GetObjectivesInReturner _asbp_our_game_state) (.ID (Utilities|Struct|BreakST_Objective _returnvalue)))
            (return true))))))
  (return false))

(fn OnRepTurnedon
  (if (not (Variables|Default|GetTerminalSpecialityToggler))
    (Development|SetHiddeninGame (Variables|Default|GetPatch) (not (Variables|Default|GetTurnedOn)) false)
    (CallFunction|PlayAnimationScreenSaver (Variables|Default|GetTurnedOn))))

(fn SP
  (Transformation|AddRelativeLocation (Variables|Default|GetPatch) (* (Variables|Default|GetCurrentPatchDirection) (Variables|Default|GetPatchSpeed)) false false)
  (if (> (.Y (Math|Vector|BreakVector (Variables|/Script/Engine.SceneComponent|GetRelativeLocation (Variables|Default|GetPatch)))) 6e+01)
    (if (> (.X (Math|Vector|BreakVector (Variables|Default|GetCurrentPatchDirection))) 0.0)
      (Variables|Default|SetCurrentPatchDirection "0.500000,-1.000000, 0")
      (else
        (Variables|Default|SetCurrentPatchDirection "-0.500000,-1.000000, 0")))
    (elif (< (.Y (Math|Vector|BreakVector (Variables|/Script/Engine.SceneComponent|GetRelativeLocation (Variables|Default|GetPatch)))) 0.0)
      (if (> (.X (Math|Vector|BreakVector (Variables|Default|GetCurrentPatchDirection))) 0.0)
        (Variables|Default|SetCurrentPatchDirection "0.500000,1.000000, 0")
        (else
          (Variables|Default|SetCurrentPatchDirection "-0.500000,1.000000, 0")))
      (elif (> (.X (Math|Vector|BreakVector (Variables|/Script/Engine.SceneComponent|GetRelativeLocation (Variables|Default|GetPatch)))) 6e+01)
        (if (> (.Y (Math|Vector|BreakVector (Variables|Default|GetCurrentPatchDirection))) 0.0)
          (Variables|Default|SetCurrentPatchDirection "-0.500000,1.000000, 0")
          (else
            (Variables|Default|SetCurrentPatchDirection "0.500000,1.000000, 0")))
        (elif (< (.X (Math|Vector|BreakVector (Variables|/Script/Engine.SceneComponent|GetRelativeLocation (Variables|Default|GetPatch)))) 0.0)
          (if (> (.Y (Math|Vector|BreakVector (Variables|Default|GetCurrentPatchDirection))) 0.0)
            (Variables|Default|SetCurrentPatchDirection "0.500000,1.000000, 0")
            (else
              (Variables|Default|SetCurrentPatchDirection "-0.500000,1.000000, 0"))))))))