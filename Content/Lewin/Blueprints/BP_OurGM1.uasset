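; Multiplayer game mode for rover missions, with all event and function entries unwired, so none of its logic runs as saved.
; The disconnected graphs track players, arbitrate terminal and mission-selector occupancy, and start a table-driven mission once enough players are assigned.
; Mission setup would spawn rovers at matching spawn points, link them to terminals with render targets, activate the zone and refresh a rover map on a timer.
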(event Custom|SetMissionSelectorOccupied
  (params (MissionSelectorActor :type BP%20Mission%20Selector%20Object%20Reference) (Occupieds :type Boolean) (nID :type Integer) (RequestValidConnect :type Boolean) (PCForValidCheck :type Player%20Controller%20Object%20Reference)))

(event Custom|SetTerminalOccupied
  (params (Terminal :type BP%20Terminal%20Object%20Reference) (Occupied :type Boolean) (RequestValidConnect :type Boolean) (PCForValidCheck :type Player%20Controller%20Object%20Reference)))

(event Custom|ApplyRoverToTerminal
  (params (Terminal :type BP%20Terminal%20Object%20Reference) (NewPawn :type Pawn%20Object%20Reference)))

(event Custom|ThrowPlayersOutOfMissionAssignment)

(event Custom|CheckToStartMission
  (params (PC :type Player%20Controller%20Object%20Reference) (AssignIn? :type Boolean)))

(event Custom|DevstartMission
  (params (CurrentRunningMission :type Integer)))

(event EventBeginPlay)

(event EventPostLogin
  (params (NewPlayer :type Player%20Controller%20Object%20Reference))
  ;[1 1 1] Join & Leave tracking
)

(event EventOnLogout
  (params (ExitingController :type Controller%20Object%20Reference))
  ;[1 1 1] Join & Leave tracking
)

(fn ConstructionScript)

(fn GetMissionScreen)

(fn GetMissionSelector)

(fn SetupStartMission)

(fn TurnonTerminals)

(fn GetSpawnPointsArray)

(fn ActivateMissionZone)

(fn GetMissionZonebyID
  (params (ID :type Integer)))

(fn ActivateMapScreen)

(fn UpdateRoversonMap)

(fn GetRoverData
  (params (rover :type Parent%20Rover%20Object%20Reference)))