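; BP_MapScreen is an in-world map screen that shows a zone grid, rovers and scanning results through a WB_MapWideInfoScreen widget.
; Server-facing events store the zone, rover and scan data in variables, with RepNotify functions pushing it into the widget's map.
; Setup and rover updates flip booleans purely to fire their OnRep handlers, while scan results trigger their own.
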(event Custom|SetCurrentRovers
  (params (CurrentRovers :type Array%20of%20Parent%20Rover%20Object%20References))
  ;[1 1 1] Set Current Rover references
  (Variables|Default|SetCurrentRovers CurrentRovers))

(event Custom|SetupMapWidgetOnServer
  (params (ZoneRef :type BP%20Mission%20Zone%20Object%20Reference) (Rovers :type Array%20of%20Rover%20Map%20Update%20Structure%20Structures))
  ;[1 1 1] Setup
  (Variables|Default|SetZoneRef ZoneRef)
  (Variables|Default|SetRovers Rovers)
  (Variables|Default|SetSetupMap (not (Variables|Default|GetSetupMap))))

(event Custom|UpdateMapOnServer
  (params (RoverUpdateData :type Array%20of%20Rover%20Map%20Update%20Structure%20Structures))
  ;[1 1 1] Update Map Data (Rover)
  (Variables|Default|SetRover%20Update%20Data RoverUpdateData)
  (Variables|Default|SetUpdateMap (not (Variables|Default|GetUpdateMap))))

(event Custom|UpdateScanningZone
  (params (Result :type ST%20Scanning%20Zone%20Result%20Structure))
  ;[1 1 1] Update Map Data (Scanning)
  (Variables|Default|SetScanningResults Result))

(fn ConstructionScript)

(fn OnRepSetupMap
  (bind _zoneref (Variables|Default|GetZoneRef))
  (bind _aswb_map_wide_info_screen (Utilities|Casting|CastToWB_MapWideInfoScreen (UserInterface|GetUserWidgetObject (Variables|Default|GetScreenWidget))))
  (Default|Show _aswb_map_wide_info_screen)
  (Default|CreateGrid (Variables|/Game/Lewin/UI/WB_MapWideInfoScreen.WB_MapWideInfoScreen_C|GetWB_MapScreen _aswb_map_wide_info_screen) (Variables|/Game/Lewin/Blueprints/BP_MissionZone.BP_MissionZone_C|GetStartX _zoneref) (Variables|/Game/Lewin/Blueprints/BP_MissionZone.BP_MissionZone_C|GetGridLines _zoneref) (Variables|/Game/Lewin/Blueprints/BP_MissionZone.BP_MissionZone_C|GetDistancePerLine _zoneref) false (Variables|/Game/Lewin/Blueprints/BP_MissionZone.BP_MissionZone_C|GetStartY _zoneref))
  (Default|SetupMap (Variables|/Game/Lewin/UI/WB_MapWideInfoScreen.WB_MapWideInfoScreen_C|GetWB_MapScreen _aswb_map_wide_info_screen) (Transformation|GetActorLocation _zoneref) (Variables|/Game/Lewin/Blueprints/BP_MissionZone.BP_MissionZone_C|GetZeroDistance _zoneref) (Variables|Default|GetRovers)))

(fn OnRepUpdateMap
  (bind _aswb_map_wide_info_screen (Utilities|Casting|CastToWB_MapWideInfoScreen (UserInterface|GetUserWidgetObject (Variables|Default|GetScreenWidget))))
  (Default|UpdateMap2 (Variables|/Game/Lewin/UI/WB_MapWideInfoScreen.WB_MapWideInfoScreen_C|GetWB_MapScreen _aswb_map_wide_info_screen) (Variables|Default|GetRover%20Update%20Data) false))

(fn OnRepScanningResults
  (bind _aswb_map_wide_info_screen (Utilities|Casting|CastToWB_MapWideInfoScreen (UserInterface|GetUserWidgetObject (Variables|Default|GetScreenWidget))))
  (Default|UpdateScanningZone (Variables|/Game/Lewin/UI/WB_MapWideInfoScreen.WB_MapWideInfoScreen_C|GetWB_MapScreen _aswb_map_wide_info_screen) (Variables|Default|GetScanningResults)))