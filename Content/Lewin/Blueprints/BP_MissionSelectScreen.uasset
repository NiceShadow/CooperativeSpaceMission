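; In-world mission select screen actor hosting a map widget, with text renders for mission title and assigned player count.
; Looping timers step clamped X/Y values while input is held, and RepNotifies push them to the widget.
; Mission choice notifies BP_MissionSelector, and its RepNotify pulls the title from a data table.
; The player count RepNotify activates the selected mission on the widget once the minimum is met.
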(event Custom|IncreaseYvalue
  (params (add :type Boolean) (in :type Boolean))
  (bind _returnvalue (Math|Float|MakeLiteralFloat 0.1))
  (if in
    (bind _returnvalue_2 (Utilities|Time|SetTimerbyEvent (delegate Custom|CustomEvent_1) _returnvalue true (* _returnvalue -1.0)))
    (else
      (Utilities|Time|ClearandInvalidateTimerbyHandle _returnvalue_2))))

(event Custom|CustomEvent_1
  (Variables|Default|SetCurrentY_Value (Math|Integer|Clamp(Integer) (+ (Variables|Default|GetCurrentY_Value) (* (Math|Integer|SelectInt 1 -1 (stale Custom|IncreaseYvalue add)) 15)) 50 1015)))

(event Custom|IncreaseXvalue
  (params (add :type Boolean) (in :type Boolean))
  (bind _returnvalue (Math|Float|MakeLiteralFloat 0.1))
  (if in
    (bind _returnvalue_2 (Utilities|Time|SetTimerbyEvent (delegate Custom|CustomEvent_0) _returnvalue true (* _returnvalue -1.0)))
    (else
      (Utilities|Time|ClearandInvalidateTimerbyHandle _returnvalue_2))))

(event Custom|CustomEvent_0
  (Variables|Default|SetCurrentX_Value (Math|Integer|Clamp(Integer) (+ (Variables|Default|GetCurrentX_Value) (* (Math|Integer|SelectInt 1 -1 (stale Custom|IncreaseXvalue add)) 15)) 50 1855)))

(event Custom|UpdateMission
  (params (CurrentSelectedMissionIndex :type Integer))
  (Variables|Default|SetCurrentSelectedMissionIndex CurrentSelectedMissionIndex)
  (Utilities|IsValid (Variables|Default|GetMissionSelectorRef)
    (:Is%20Valid
      _)
    (:Is%20Not%20Valid
      (bind _outactors (Actor|GetAllActorsOfClass "/Game/Lewin/Blueprints/BP_MissionSelector.BP_MissionSelector_C"))
      (Variables|Default|SetMissionSelectorRef (Utilities|Array|Get(acopy) _outactors))))
  (Default|OnMissionActivated (Variables|Default|GetMissionSelectorRef) (>= (Variables|Default|GetCurrentSelectedMissionIndex) 0)))

(event Custom|UpdatePlayerInfo
  (params (CurrentPlayersAssigned :type Integer))
  (Variables|Default|SetCurrentPlayersAssigned CurrentPlayersAssigned))

(event Custom|CancelX
  (Utilities|Time|ClearandInvalidateTimerbyHandle (stale Custom|IncreaseXvalue _returnvalue_2)))

(event Custom|CancelY
  (Utilities|Time|ClearandInvalidateTimerbyHandle (stale Custom|IncreaseYvalue _returnvalue_2)))

(event EventBeginPlay
  (bind _aswb_mission_select_map (Utilities|Casting|CastToWB_MissionSelectMap (UserInterface|GetUserWidgetObject (Variables|Default|GetScreenWidget))))
  (Variables|/Game/Lewin/UI/WB_MissionSelectMap.WB_MissionSelectMap_C|SetMissionSelectSreenActor _aswb_mission_select_map self)
  (CallFunction|GetMissionData))

(fn ConstructionScript)

(fn OnRepCurrentXValue
  (bind _aswb_mission_select_map (Utilities|Casting|CastToWB_MissionSelectMap (UserInterface|GetWidget (Variables|Default|GetScreenWidget))))
  (Default|UpdateX _aswb_mission_select_map (Variables|Default|GetCurrentX_Value)))

(fn OnRepCurrentYValue
  (bind _aswb_mission_select_map (Utilities|Casting|CastToWB_MissionSelectMap (UserInterface|GetWidget (Variables|Default|GetScreenWidget))))
  (Default|UpdateY _aswb_mission_select_map (Variables|Default|GetCurrentY_Value)))

(fn OnRepCurrentSelectedMission
  (if (> (Variables|Default|GetCurrentSelectedMissionIndex) -1)
    (Rendering|SetVisibility (Variables|Default|GetTextRenderMissionTitle) true false)
    (bind _outrownames (DataTable|GetDataTableRowNames "/Game/Balduin/SelectMissionsTable.SelectMissionsTable"))
    (bind _returnvalue (Utilities|GetDataTableRow "/Game/Balduin/SelectMissionsTable.SelectMissionsTable" (Utilities|Array|Get(acopy) _outrownames (Variables|Default|GetCurrentSelectedMissionIndex)))
      (:then
        (Rendering|Components|TextRender|SetText (Variables|Default|GetTextRenderMissionTitle) (.Title (Utilities|Struct|BreakMissionSelect_Structure _returnvalue)))))
    (else
      (Rendering|SetVisibility (Variables|Default|GetTextRenderMissionTitle) false false))))

(fn GetMissionData
  (Utilities|Array|Clear (Variables|Default|GetAllMissions))
  (bind _outrownames (DataTable|GetDataTableRowNames "/Game/Balduin/SelectMissionsTable.SelectMissionsTable"))
  (for _array_element _outrownames
    (bind _returnvalue (Utilities|GetDataTableRow "/Game/Balduin/SelectMissionsTable.SelectMissionsTable" _array_element)
      (:then
        (Utilities|Array|Add (Variables|Default|GetAllMissions) _returnvalue)))))

(fn OnRepCurrentPlayersAssigned
  (Rendering|SetVisibility (Variables|Default|GetTextRenderPlayers) (> (Variables|Default|GetCurrentPlayersAssigned) 0) false)
  (Rendering|Components|TextRender|SetText (Variables|Default|GetTextRenderPlayers) (Utilities|Text|FormatText "Players: {amount}" (Variables|Default|GetCurrentPlayersAssigned)))
  (if (>= (Variables|Default|GetCurrentPlayersAssigned) (Variables|Default|GetMinimumPlayersToStart))
    (bind _aswb_mission_select_map (Utilities|Casting|CastToWB_MissionSelectMap (UserInterface|GetUserWidgetObject (Variables|Default|GetScreenWidget))))
    (Default|ActivateMission _aswb_mission_select_map (Variables|Default|GetCurrentSelectedMissionIndex))))