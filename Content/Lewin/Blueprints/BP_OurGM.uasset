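; BP_OurGM is the game mode that tracks joined player controllers and manages occupancy of terminals and mission selectors.
; PostLogin and OnLogout maintain the AllPCs list.
; Validated connect requests succeed only on a free terminal or selector slot, calling back into BP_OurPC before setting occupancy on the server; other requests set it directly.
; It also turns off released terminal screens and assigns rover pawns to terminals.
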(event Custom|SetMissionSelectorOccupied
  (params (MissionSelectorActor :type BP%20Mission%20Selector%20Object%20Reference) (Occupieds :type Boolean) (nID :type Integer) (RequestValidConnect :type Boolean) (PCForValidCheck :type Player%20Controller%20Object%20Reference))
  (if RequestValidConnect
    (if (not (Utilities|Array|Get(acopy) (Variables|/Game/Lewin/Blueprints/BP_MissionSelector.BP_MissionSelector_C|GetOccupied MissionSelectorActor) nID))
      (bind _asbp_our_pc (Utilities|Casting|CastToBP_OurPC PCForValidCheck))
      (Default|ConnecttoCurrentMissionSelector _asbp_our_pc)
      (Default|SetOccupiedonServer MissionSelectorActor Occupieds nID :!label _label))
    (else
      (goto _label))))

(event Custom|SetTerminalOccupied
  (params (Terminal :type BP%20Terminal%20Object%20Reference) (Occupied :type Boolean) (RequestValidConnect :type Boolean) (PCForValidCheck :type Player%20Controller%20Object%20Reference))
  (if RequestValidConnect
    (if (not (Variables|/Game/Lewin/Blueprints/BP_Terminal.BP_Terminal_C|GetOccupied Terminal))
      (bind _asbp_our_pc (Utilities|Casting|CastToBP_OurPC PCForValidCheck))
      (Default|ConnecttoCurrentTerminal _asbp_our_pc)
      (Default|SetOccupiedonServer Terminal Occupied :!label _label)
      (if (not Occupied)
        (Default|SetTerminalScreen Terminal false)))
    (else
      (goto _label))))

(event Custom|ApplyRoverToTerminal
  (params (Terminal :type BP%20Terminal%20Object%20Reference) (NewPawn :type Pawn%20Object%20Reference))
  (Variables|/Game/Lewin/Blueprints/BP_Terminal.BP_Terminal_C|SetCurrentRoverPawn Terminal NewPawn))

(event EventPostLogin
  (params (NewPlayer :type Player%20Controller%20Object%20Reference))
  ;[1 1 1] Join & Leave tracking
  (Utilities|Array|Add (Variables|Default|GetAllPCs) NewPlayer))

(event EventOnLogout
  (params (ExitingController :type Controller%20Object%20Reference))
  ;[1 1 1] Join & Leave tracking
  (bind _asplayer_controller (Utilities|Casting|CastToPlayerController ExitingController))
  (Utilities|Array|RemoveItem (Variables|Default|GetAllPCs) _asplayer_controller))

(fn ConstructionScript)