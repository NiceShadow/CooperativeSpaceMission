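; Circular mission boundary that warns and tracks the local player leaving the play area.
; Exiting the slightly smaller inner cylinder fades in the visible border, while exiting the outer one starts BP_OurPC's out-of-zone handling with origin and radius, and re-entry reverses each.
; A replicated Activate flag toggles collision on both cylinders.
; The construction script snaps scale to a coordinate grid, derives the radius and labels edge coordinates and width subdivisions.
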(event OnComponentBeginOverlap(CylinderOverlap)
  (params (OverlappedComponent :type Primitive%20Component%20Object%20Reference) (OtherActor :type Actor%20Object%20Reference) (OtherComp :type Primitive%20Component%20Object%20Reference) (OtherBodyIndex :type Integer) (bFromSweep :type Boolean) (SweepResult :type Hit%20Result%20Structure%20%28by%20ref%29))
  (if (== OtherActor (Game|Player|GetPlayerPawn 0))
    (CallFunction|ShowMissionZone false)))

(event OnComponentEndOverlap(CylinderOverlap)
  (params (OverlappedComponent :type Primitive%20Component%20Object%20Reference) (OtherActor :type Actor%20Object%20Reference) (OtherComp :type Primitive%20Component%20Object%20Reference) (OtherBodyIndex :type Integer))
  (if (== OtherActor (Game|Player|GetPlayerPawn 0))
    (CallFunction|ShowMissionZone true)))

(event OnComponentBeginOverlap(CylinderShow)
  (params (OverlappedComponent :type Primitive%20Component%20Object%20Reference) (OtherActor :type Actor%20Object%20Reference) (OtherComp :type Primitive%20Component%20Object%20Reference) (OtherBodyIndex :type Integer) (bFromSweep :type Boolean) (SweepResult :type Hit%20Result%20Structure%20%28by%20ref%29))
  (if (== OtherActor (Game|Player|GetPlayerPawn 0))
    (bind _asbp_our_pc (Utilities|Casting|CastToBP_OurPC (Game|GetPlayerController 0)))
    (Default|StartOutOfZone _asbp_our_pc false true "0, 0, 0" 0.0)))

(event OnComponentEndOverlap(CylinderShow)
  (params (OverlappedComponent :type Primitive%20Component%20Object%20Reference) (OtherActor :type Actor%20Object%20Reference) (OtherComp :type Primitive%20Component%20Object%20Reference) (OtherBodyIndex :type Integer))
  (if (== OtherActor (Game|Player|GetPlayerPawn 0))
    (bind _asbp_our_pc (Utilities|Casting|CastToBP_OurPC (Game|GetPlayerController 0)))
    (Default|StartOutOfZone _asbp_our_pc true true (Transformation|GetActorLocation) (Variables|Default|GetZeroDistance))))

(event Custom|ShowMissionZone
  (params (In :type Boolean))
  (if In
    (Development|SetHiddeninGame (Variables|Default|GetCylinderShow) false false)
    (CallFunction|SetupInstanceMATifNeeded)
    (bind _newtrack_0 (Timeline|Timeline_0 Play)
      (:Update
        (Rendering|Material|SetScalarParameterValue (Variables|Default|GetZoneInstanceMAT) "Opacity" _newtrack_0 :!class /Script/Engine.MaterialInstanceDynamic))
      (:Finished
        (if (not In)
          (Development|SetHiddeninGame (Variables|Default|GetCylinderShow) true false))))
    (else
      (CallFunction|SetupInstanceMATifNeeded)
      (Timeline|Timeline_0 Reverse))))

(event Custom|ActivateOnServer
  (params (Activate :type Boolean))
  (Variables|Default|SetActivate Activate))

(event Custom|ShowMissionZoneInstant
  (params (Show :type Boolean))
  (Development|SetHiddeninGame (Variables|Default|GetCylinderShow) (not Show) false))

(fn ConstructionScript
  (bind _coordinatedivider (Variables|Default|GetCoordinateDivider))
  (bind _coordinatedivider_2 (Variables|Default|GetCoordinateDivider))
  (bind _coordinatedivider_3 (Variables|Default|GetCoordinateDivider))
  (bind _coordinatedivider_4 (Variables|Default|GetCoordinateDivider))
  (bind _cylindershow (Variables|Default|GetCylinderShow))
  (bind _textrenderx (Variables|Default|GetTextRenderX))
  (bind _textrendery (Variables|Default|GetTextRenderY))
  (bind _textrendernx (Variables|Default|GetTextRenderNX))
  (bind _returnvalue (Transformation|GetWorldLocation _textrendernx))
  (bind _returnvalue_2 (Math|Conversions|ToFloat(Integer) _coordinatedivider_4))
  (bind _returnvalue_3 (Transformation|GetWorldScale _cylindershow))
  (bind _returnvalue_4 (Transformation|GetWorldLocation _textrenderx))
  (bind _returnvalue_5 (Transformation|GetWorldLocation _textrendery))
  (bind _x (Math|Vector|BreakVector _returnvalue))
  (bind _x_2 (Math|Vector|BreakVector _returnvalue_4))
  (bind _y (Math|Vector|BreakVector _returnvalue_5))
  (bind _returnvalue_6 (Class|KismetMathLibrary|VectorSnappedtoGrid _returnvalue_3 _returnvalue_2))
  (bind _returnvalue_7 (Math|Float|SnapToGrid(Float) _x_2 1e+03))
  (bind _returnvalue_8 (Math|Float|SnapToGrid(Float) _x 1e+03))
  (bind _returnvalue_9 (Math|Float|SnapToGrid(Float) _y 1e+03))
  (bind _returnvalue_10 (Math|Float|Truncate _returnvalue_8))
  (bind _returnvalue_11 (Math|Float|Truncate _returnvalue_7))
  (bind _returnvalue_12 (Math|Float|Truncate _returnvalue_9))
  (bind _returnvalue_13 (/ _returnvalue_10 _coordinatedivider_3))
  (bind _returnvalue_14 (/ _returnvalue_11 _coordinatedivider))
  (bind _returnvalue_15 (/ _returnvalue_12 _coordinatedivider_2))
  (Transformation|SetWorldScale3D (Variables|Default|GetCylinderShow) _returnvalue_6)
  (Transformation|SetWorldScale3D (Variables|Default|GetCylinderOverlap) (- _returnvalue_6 (Math|Conversions|ToVector(Float) (Variables|Default|GetDistanceOverlapAndVisualBorder))))
  (Variables|Default|SetZeroDistance (* (.X (Math|Vector|BreakVector _returnvalue_6)) 5e+01))
  (Transformation|SetWorldLocation (Variables|Default|GetTextRenderX) (+ (Transformation|GetActorLocation) (Math|Vector|MakeVector (Variables|Default|GetZeroDistance) 0.0 0.0)) false false)
  (Transformation|SetWorldLocation (Variables|Default|GetTextRenderX_Info) (- (+ (Transformation|GetActorLocation) (Math|Vector|MakeVector (Variables|Default|GetZeroDistance) 0.0 0.0)) "-10.000000, 0,100.000000") false false)
  (Rendering|Components|TextRender|SetText (Variables|Default|GetTextRenderX) (Utilities|Text|ToText(Integer) _returnvalue_14))
  (Variables|Default|SetStartX _returnvalue_14)
  (Transformation|SetWorldLocation (Variables|Default|GetTextRenderNX) (+ (Transformation|GetActorLocation) (Math|Vector|MakeVector (* (Variables|Default|GetZeroDistance) -1.0) 0.0 0.0)) false false)
  (Rendering|Components|TextRender|SetText (Variables|Default|GetTextRenderNX) (Utilities|Text|ToText(Integer) _returnvalue_13))
  (Transformation|SetWorldLocation (Variables|Default|GetTextRenderY) (+ (Transformation|GetActorLocation) (Math|Vector|MakeVector 0.0 (* (Variables|Default|GetZeroDistance) -1.0) 0.0)) false false)
  (Rendering|Components|TextRender|SetText (Variables|Default|GetTextRenderY) (Utilities|Text|ToText(Integer) _returnvalue_15))
  (Variables|Default|SetStartY _returnvalue_15)
  (Variables|Default|SetEndX _returnvalue_13)
  (LocalVariables|SetTotalXDistance (Math|Integer|Absolute(Integer) (- _returnvalue_14 _returnvalue_13)))
  (Rendering|Components|TextRender|SetText (Variables|Default|GetTextRenderX_Info) (Utilities|Text|ToText(String) (Utilities|String|Append (Utilities|String|ToString(Integer) (LocalVariables|GetTotalXDistance)) "____" "5x " (Utilities|String|ToString(Integer) (/ (LocalVariables|GetTotalXDistance) 4)) ";  " "7x " (Utilities|String|ToString(Integer) (/ (LocalVariables|GetTotalXDistance) 6)) ";  " "9x " (Utilities|String|ToString(Integer) (/ (LocalVariables|GetTotalXDistance) 8))))))

(fn SetupInstanceMATifNeeded
  (Utilities|IsValid (Variables|Default|GetZoneInstanceMAT)
    (:Is%20Not%20Valid
      (bind _returnvalue (Rendering|Material|CreateDynamicMaterialInstance "/Game/Lewin/Blueprints/TestMaterials/M_MissionZoneShow_Inst.M_MissionZoneShow_Inst" "None" "None" :!class /Script/Engine.KismetMaterialLibrary))
      (bind _output_get (Variables|Default|SetZoneInstanceMAT _returnvalue))
      (Rendering|Material|SetMaterial (Variables|Default|GetCylinderShow) 0 _output_get))))

(fn OnRepActivate
  (Collision|SetCollisionEnabled (Variables|Default|GetCylinderOverlap) (select (Variables|Default|GetActivate) "QueryAndPhysics" "NoCollision")))