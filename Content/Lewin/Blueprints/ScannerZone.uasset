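; Scanner zone actor that randomly generates nested, shrinking scan circles and picks objective locations inside them from foliage instances.
; GenerateOnServer takes zone radii and objective counts, then offsets each circle within the previous one and sphere-traces it to count candidate hits.
; Failed layouts are retried, with a delay once past an attempt cap.
; A valid layout gets shuffled picks from innermost zone outward, skipping already-traced instances, and is broadcast through FoundResult.
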(event Custom|PendingGenerate
  (Utilities|FlowControl|Delay (Variables|Default|GetUpdate))
  (CallFunction|GenerateRandomZones))

(event Custom|GenerateOnServer
  (params (Zones :type Array%20of%20Scanner%20Zones%20Structure%20Structures))
  (CallFunction|SetupandStartGenerating Zones))

(event EventBeginPlay)

(fn ConstructionScript)

(fn CreateCircle
  (params (InSphereRadius :type Float%20%28single-precision%29) (Target :type Sphere%20Component%20Object%20Reference) (Before :type Sphere%20Component%20Object%20Reference))
  (Components|Sphere|SetSphereRadius Target InSphereRadius true)
  (Transformation|SetWorldLocation Target (+ (Transformation|GetWorldLocation Before) (* (Math|Vector|RotateVector (Math|Vector|GetForwardVector (Transformation|GetActorRotation)) (Math|Rotator|MakeRotator 0.0 0.0 (Math|Conversions|ToFloat(Integer) (Math|Random|RandomIntegerinRange 0 360)))) (Math|Random|RandomIntegerinRange 20 (Math|Float|Truncate (- (Variables|/Script/Engine.SphereComponent|GetSphereRadius Before) InSphereRadius))))) false false))

(fn ScanCircle
  (params (InSphereRadius :type Float%20%28single-precision%29) (Target :type Sphere%20Component%20Object%20Reference) (Before :type Sphere%20Component%20Object%20Reference))
  (Components|Sphere|SetSphereRadius Target InSphereRadius true)
  (Transformation|SetWorldLocation Target (+ (Transformation|GetWorldLocation Before) (* (Math|Vector|RotateVector (Math|Vector|GetForwardVector (Transformation|GetActorRotation)) (Math|Rotator|MakeRotator 0.0 0.0 (Math|Conversions|ToFloat(Integer) (Math|Random|RandomIntegerinRange 0 360)))) (Math|Random|RandomIntegerinRange 20 (Math|Float|Truncate (- (Variables|/Script/Engine.SphereComponent|GetSphereRadius Before) InSphereRadius))))) false false))

(fn TrytoGenerateRandomZone
  (Utilities|Array|Clear (Variables|Default|GetFoundZoneLocs))
  (LocalVariables|SetLocationOfBiggerCircle (Transformation|GetActorLocation))
  (for (_array_element _array_index) (Variables|Default|GetZonesRadius)
    (if (> _array_index 0)
      (LocalVariables|SetLocationOfBiggerCircle (+ (LocalVariables|GetLocationOfBiggerCircle) (* (Math|Vector|RotateVector (Math|Vector|GetForwardVector (Transformation|GetActorRotation)) (Math|Rotator|MakeRotator 0.0 0.0 (Math|Conversions|ToFloat(Integer) (Math|Random|RandomIntegerinRange 0 360)))) (Math|Random|RandomIntegerinRange (/ _array_element 2) (Math|Float|Truncate (- (Math|Conversions|ToFloat(Integer) (Utilities|Array|Get(acopy) (Variables|Default|GetZonesRadius) (- _array_index 1))) (Math|Conversions|ToFloat(Integer) _array_element))))))))
    (bind _outhits (Collision|MultiSphereTraceByChannel (.Start (CallFunction|GetSphereTraceLocs (LocalVariables|GetLocationOfBiggerCircle))) (.End (CallFunction|GetSphereTraceLocs (LocalVariables|GetLocationOfBiggerCircle))) (Math|Conversions|ToFloat(Integer) _array_element) "TraceTypeQuery3" true 0 "None" true "(R=1.000000,G=0.000000,B=0.000000,A=1.000000)" "(R=0.000000,G=1.000000,B=0.000000,A=1.000000)" 3e+01))
    (Utilities|Array|Add (LocalVariables|GetAmountOfInstances) (Utilities|Array|Length _outhits))
    (Utilities|Array|Add (Variables|Default|GetFoundZoneLocs) (LocalVariables|GetLocationOfBiggerCircle)))
  (bind _output_get (LocalVariables|SetAmountOfInstancesReversed (LocalVariables|GetAmountOfInstances)))
  (Utilities|Array|Reverse _output_get)
  (for (_array_element_2 _array_index_2) (LocalVariables|GetAmountOfInstancesReversed)
    (if (>= (- _array_element_2 (LocalVariables|GetCurrentTotalAmountCount)) (Utilities|Array|Get(acopy) (Variables|Default|GetZonesObjectivesReversed) _array_index_2))
      (LocalVariables|SetCurrentTotalAmountCount (+ _array_element_2 (LocalVariables|GetCurrentTotalAmountCount)))
      (else
        (return false))))
  (return true))

(fn GenerateRandomZones
  (bind _returnvalue (Math|Random|RandomFloat))
  (bind _returnvalue_2 (Math|Random|RandomFloat))
  (bind _returnvalue_3 (Math|Random|RandomFloat))
  (bind _scanningzoneresults (Variables|Default|GetScanningZoneResults))
  (bind _scanningzoneresults_2 (Variables|Default|GetScanningZoneResults))
  (bind (_radiuslocations _objectivelocations) (Utilities|Struct|BreakScanningZoneResult_Structure _scanningzoneresults_2))
  (bind (_radiuslocations_2 _objectivelocations_2) (Utilities|Struct|BreakScanningZoneResult_Structure _scanningzoneresults))
  (bind _returnvalue_4 (Math|Color|MakeColor _returnvalue_2 _returnvalue_3 _returnvalue))
  (Utilities|Array|Clear (Variables|Default|GetObjectivesSelected))
  (bind _output_get (Variables|Default|SetZonesObjectivesReversed (Variables|Default|GetZonesAmountOfObjectives)))
  (Utilities|Array|Reverse _output_get)
  (bind _output_get_2 (Variables|Default|SetZonesRadiusReversed (Variables|Default|GetZonesRadius)))
  (Utilities|Array|Reverse _output_get_2)
  (Math|Integer|IncrementInt (LocalVariables|GetAttempts) :!label _label
    (:%20%20
      (Math|Integer|IncrementInt (Variables|Default|GetTotalAttempts)
        (:%20%20
          (bind _found (CallFunction|TrytoGenerateRandomZone))
          (if _found
            (Development|PrintString (Utilities|String|Append "Total Attempts to generate scan zones: " (Utilities|String|ToString(Integer) (Variables|Default|GetTotalAttempts))) true true "(R=0.001346,G=1.000000,B=0.000000,A=1.000000)" 3.0)
            (Utilities|Array|Clear (Utilities|Struct|BreakScanningZoneResult_Structure (Variables|Default|GetScanningZoneResults)))
            (bind _output_get_3 (Variables|Default|SetFoundReversed (Variables|Default|GetFoundZoneLocs)))
            (Utilities|Array|Reverse _output_get_3)
            (for (_array_element _array_index) (Variables|Default|GetFoundReversed)
              (Utilities|Array|Clear (LocalVariables|GetAllFound))
              (Utilities|Array|Clear (LocalVariables|GetCurrentHitItems))
              (bind _outhits (Collision|MultiSphereTraceByChannel (.Start (CallFunction|GetSphereTraceLocs _array_element)) (.End (CallFunction|GetSphereTraceLocs _array_element)) (Math|Conversions|ToFloat(Integer) (Utilities|Array|Get(acopy) (Variables|Default|GetZonesRadiusReversed) _array_index)) "TraceTypeQuery3" true 0 "None" true _returnvalue_4 _returnvalue_4 3e+01))
              (bind _output_get_4 (Variables|Default|SetCurrentResults _outhits))
              (for _array_element_2 _output_get_4
                (if (not (Utilities|Array|ContainsItem (LocalVariables|GetAlreadyTraced) (.HitItem (Collision|BreakHitResult _array_element_2))))
                  (if (not (Utilities|Array|ContainsItem (Variables|Default|GetObjectivesSelected) (.HitItem (Collision|BreakHitResult _array_element_2))))
                    (Utilities|Array|Add (LocalVariables|GetCurrentHitItems) (.HitItem (Collision|BreakHitResult _array_element_2))))))
              (Utilities|Array|Shuffle (LocalVariables|GetCurrentHitItems))
              (for _array_element_3 (Variables|Default|GetCurrentResults)
                (Utilities|Array|Add (LocalVariables|GetAlreadyTraced) (.HitItem (Collision|BreakHitResult _array_element_3))))
              (Utilities|Array|AppendArray (Variables|Default|GetObjectivesSelected) (.Instances (CallFunction|GetItemsThatNotHaveBeenSelected (LocalVariables|GetCurrentHitItems) (Utilities|Array|Get(acopy) (Variables|Default|GetZonesObjectivesReversed) _array_index) (Variables|Default|GetPrevoiusHit%20Indexes) (.HitComponent (Collision|BreakHitResult (Utilities|Array|Get(acopy) (Variables|Default|GetCurrentResults)))))))
              (Utilities|Struct|SetmembersinZoneLocs_Structure (Utilities|Array|Get(acopy) _objectivelocations_2 _array_index) (.Locations (CallFunction|GetItemsThatNotHaveBeenSelected (LocalVariables|GetCurrentHitItems) (Utilities|Array|Get(acopy) (Variables|Default|GetZonesObjectivesReversed) _array_index) (Variables|Default|GetPrevoiusHit%20Indexes) (.HitComponent (Collision|BreakHitResult (Utilities|Array|Get(acopy) (Variables|Default|GetCurrentResults)))))) (.Available (CallFunction|GetItemsThatNotHaveBeenSelected (LocalVariables|GetCurrentHitItems) (Utilities|Array|Get(acopy) (Variables|Default|GetZonesObjectivesReversed) _array_index) (Variables|Default|GetPrevoiusHit%20Indexes) (.HitComponent (Collision|BreakHitResult (Utilities|Array|Get(acopy) (Variables|Default|GetCurrentResults)))))))
              (Utilities|Array|Add _radiuslocations_2 _array_element))
            (Utilities|Array|Reverse _radiuslocations)
            (Utilities|Array|Reverse _objectivelocations)
            (Default|CallFoundResult (Variables|Default|GetScanningZoneResults))
            (elif (> (LocalVariables|GetAttempts) 2000)
              (CallFunction|PendingGenerate)
              (Development|PrintString "Failed")
              (else
                (goto _label)))))))))

(fn GetItemsThatNotHaveBeenSelected
  (params (HitIndexes :type Array%20of%20Integers) (TargetAmount :type Integer) (TargetArray :type Array%20of%20Integers) (InputPin :type Object%20Object%20Reference))
  (for _index (range 0 (- TargetAmount 1))
    (bind _asfoliage_instanced_static_mesh_component (Utilities|Casting|CastToFoliageInstancedStaticMeshComponent InputPin))
    (Utilities|Array|Add (LocalVariables|GetLocsToBeAdded) (.Location (Math|Transform|BreakTransform (.OutInstanceTransform (Components|InstancedStaticMesh|GetInstanceTransform _asfoliage_instanced_static_mesh_component (Utilities|Array|Get(acopy) HitIndexes _index) true)))))
    (Utilities|Array|Add (LocalVariables|GetAvailableAdded) true))
  (return (LocalVariables|GetInstancesToBeAdded) (LocalVariables|GetLocsToBeAdded) (LocalVariables|GetAvailableAdded)))

(fn DebugZones
  (params (DrawTime :type Float%20%28single-precision%29))
  (bind _returnvalue (Math|Random|RandomFloat))
  (bind _returnvalue_2 (Math|Random|RandomFloat))
  (bind _returnvalue_3 (Math|Random|RandomFloat))
  (bind _returnvalue_4 (Math|Color|MakeColor _returnvalue _returnvalue_2 _returnvalue_3))
  (for (_array_element _array_index) (Variables|Default|GetFoundZoneLocs)
    (Collision|MultiSphereTraceByChannel (.Start (CallFunction|GetSphereTraceLocs _array_element)) (.End (CallFunction|GetSphereTraceLocs _array_element)) (Math|Conversions|ToFloat(Integer) (Utilities|Array|Get(acopy) (Variables|Default|GetZonesRadius) _array_index)) "TraceTypeQuery3" true 0 "ForDuration" true _returnvalue_4 _returnvalue_4 DrawTime)))

(fn GetSphereTraceLocs
  (params (A :type Vector))
  (return (- A "0, 0,900.000000") (+ A "0, 0,900.000000")))

(fn SetupandStartGenerating
  (params (Zones :type Array%20of%20Scanner%20Zones%20Structure%20Structures))
  (Utilities|Array|SetArrayElem :TargetArray (LocalVariables|GetObjectiveLocs) :Index (Utilities|Array|LastIndex Zones) :bSizeToFit true)
  (Utilities|Struct|SetmembersinScanningZoneResult_Structure (Variables|Default|GetScanningZoneResults) (Utilities|Array|MakeArray "0, 0, 0") (LocalVariables|GetObjectiveLocs))
  (Utilities|Array|Clear (Variables|Default|GetZonesAmountOfObjectives))
  (Utilities|Array|Clear (Variables|Default|GetZonesRadius))
  (for _array_element Zones
    (Utilities|Array|Add (Variables|Default|GetZonesRadius) (.ZoneRadius (Utilities|Struct|BreakScannerZones_Structure _array_element)))
    (Utilities|Array|Add (Variables|Default|GetZonesAmountOfObjectives) (.AmountOfBonusObjects (Utilities|Struct|BreakScannerZones_Structure _array_element))))
  (CallFunction|GenerateRandomZones))