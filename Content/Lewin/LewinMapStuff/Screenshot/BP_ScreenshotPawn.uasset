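; BP_ScreenshotPawn is a pawn that swings its spring arm through a fixed yaw arc, apparently for screenshot or showcase shots of a map.
; A timeline interpolates the arm's relative yaw between two hardcoded angles, leaving pitch and roll untouched.
; BeginPlay scales the timeline's play rate by the Seconds variable to set the sweep duration.
; Enter plays the sweep from the start, and Delete reverses it from the end.
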(event EventBeginPlay
  (Components|Timeline|SetPlayRate (Variables|Default|GetTimeline_0) (/ 1.0 (Variables|Default|GetSeconds))))

(event Input|KeyboardEvents|Enter
  (params (Key :type Key%20Structure))
  (bind _springarm (Variables|Default|GetSpringArm))
  (bind _relativerotation (Variables|/Script/Engine.SceneComponent|GetRelativeRotation _springarm))
  (bind (_roll _pitch) (Math|Rotator|BreakRotator _relativerotation))
  (:Pressed
    (bind _newtrack_0 (Timeline|Timeline_0 PlayFromStart)
      (:Update
        (Transformation|SetRelativeRotation (Variables|Default|GetSpringArm) (Math|Rotator|MakeRotator _roll _pitch (Math|Float|Lerp 108.058968 2e+01 _newtrack_0)) false false)))))

(event Input|KeyboardEvents|Delete
  (params (Key :type Key%20Structure))
  (bind _springarm (Variables|Default|GetSpringArm))
  (bind _relativerotation (Variables|/Script/Engine.SceneComponent|GetRelativeRotation _springarm))
  (bind (_roll _pitch) (Math|Rotator|BreakRotator _relativerotation))
  (:Pressed
    (bind _newtrack_0 (Timeline|Timeline_0 ReverseFromEnd)
      (:Update
        (Transformation|SetRelativeRotation (Variables|Default|GetSpringArm) (Math|Rotator|MakeRotator _roll _pitch (Math|Float|Lerp 108.058968 2e+01 _newtrack_0)) false false)))))

(fn ConstructionScript)