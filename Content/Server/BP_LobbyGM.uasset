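; Server game mode for a multiplayer lobby that handles player joins, kicks, exclusive character selection, chat and the start of the match.
; It tracks player controllers, kicks joins beyond four players and frees characters left unclaimed after logout.
; It approves character picks against an availability array and fans character lists, player data, chat and countdown out to each BP_LobbyPC.
; StartGame shows loading screens, then issues servertravel to MAP_Demo.
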(event Custom|UpdatePlayerList
  (Variables|Default|SetAllPlayerData (CallFunction|GetAllPlayerData))
  (for _array_element (Variables|Default|GetAllPCs)
    (bind _asbp_lobby_pc (Utilities|Casting|CastToBP_LobbyPC _array_element))
    (Default|UpdatePlayerList _asbp_lobby_pc (Variables|Default|GetAllPlayerData))))

(event Custom|SelectCharacter
  (params (Index :type Integer) (PC :type Player%20Controller%20Object%20Reference))
  (if (Utilities|Array|Get(acopy) (Variables|Default|GetAvailableCharacters) Index)
    (Utilities|Array|SetArrayElem (Variables|Default|GetAvailableCharacters) Index false)
    (bind _asbp_lobby_pc (Utilities|Casting|CastToBP_LobbyPC PC))
    (if (>= (Variables|/Game/Server/BP_LobbyPC.BP_LobbyPC_C|GetSelectedCharacterIndex _asbp_lobby_pc) 0)
      (Utilities|Array|SetArrayElem (Variables|Default|GetAvailableCharacters) (Variables|/Game/Server/BP_LobbyPC.BP_LobbyPC_C|GetSelectedCharacterIndex _asbp_lobby_pc) true)
      (Default|ApprovedSelectCharacter _asbp_lobby_pc Index)
      (else
        (Default|ApprovedSelectCharacter _asbp_lobby_pc Index)))))

(event Custom|DeselectCharacter
  (params (Index :type Integer) (PC :type Player%20Controller%20Object%20Reference))
  (Utilities|Array|SetArrayElem (Variables|Default|GetAvailableCharacters) Index true)
  (bind _asbp_lobby_pc (Utilities|Casting|CastToBP_LobbyPC PC))
  (Default|ApprovedSelectCharacter _asbp_lobby_pc -1))

(event Custom|UpdateCharacterList
  (for _array_element (Variables|Default|GetAllPCs)
    (bind _asbp_lobby_pc (Utilities|Casting|CastToBP_LobbyPC _array_element))
    (Default|UpdateCharactersList _asbp_lobby_pc (Variables|Default|GetAvailableCharacters)))
  (CallFunction|UpdatePlayerList))

(event Custom|StartGame
  (for _array_element (Variables|Default|GetAllPCs)
    (bind _asbp_lobby_pc (Utilities|Casting|CastToBP_LobbyPC _array_element))
    (Default|ShowLoadingScreen _asbp_lobby_pc))
  (Development|ExecuteConsoleCommand (Utilities|String|Append "servertravel " "MAP_Demo") 0))

(event Custom|ShowCountdown
  (for _array_element (Variables|Default|GetAllPCs)
    (bind _asbp_lobby_pc (Utilities|Casting|CastToBP_LobbyPC _array_element))
    (Default|ShowCountdown _asbp_lobby_pc)))

(event Custom|AddTextMessage
  (params (PC :type Player%20Controller%20Object%20Reference) (Message :type String) (ServerMessage :type Boolean))
  (for _array_element (Variables|Default|GetAllPCs)
    (bind _asbp_lobby_pc (Utilities|Casting|CastToBP_LobbyPC _array_element))
    (Default|AddChatMessage _asbp_lobby_pc (Class|AdvancedSessionsLibrary|GetPlayerName PC) Message ServerMessage)))

(event Custom|KickPlayer
  (params (name :type String))
  (bind (_index _found) (CallFunction|FindPlayerIndexbyName name))
  (if _found
    (Class|AdvancedSessionsLibrary|KickPlayer (Utilities|Array|Get(acopy) (Variables|Default|GetAllPCs) _index) "No reason...")))

(event Custom|MakeCharacterAvailableAgain
  (for (_array_element _array_index) (Variables|Default|GetAvailableCharacters)
    (if (not _array_element)
      (Variables|Default|SetFoundPlayerWithCharacter false)
      (bind _array_element_2 (Utilities|Array|ForEachLoopwithBreak (Variables|Default|GetAllPCs) :!label _label)
        (:LoopBody
          (bind _asbp_lobby_pc (Utilities|Casting|CastToBP_LobbyPC _array_element_2))
          (if (== _array_index (Variables|/Game/Server/BP_LobbyPC.BP_LobbyPC_C|GetSelectedCharacterIndex _asbp_lobby_pc))
            (Variables|Default|SetFoundPlayerWithCharacter true)
            (goto _label Break)))
        (:Completed
          (if (not (Variables|Default|GetFoundPlayerWithCharacter))
            (Utilities|Array|SetArrayElem (Variables|Default|GetAvailableCharacters) _array_index true))))))
  (CallFunction|UpdateCharacterList))

(event EventPostLogin
  (params (NewPlayer :type Player%20Controller%20Object%20Reference))
  (Utilities|Array|Add (Variables|Default|GetAllPCs) NewPlayer)
  (CallFunction|AddTextMessage 0 (Utilities|String|Append (Class|AdvancedSessionsLibrary|GetPlayerName NewPlayer) " joined the game.") true)
  (if (> (Utilities|Array|Length (Variables|Default|GetAllPCs)) 4)
    (Class|AdvancedSessionsLibrary|KickPlayer NewPlayer "Too many players")
    (else
      (CallFunction|UpdateCharacterList))))

(event EventOnLogout
  (params (ExitingController :type Controller%20Object%20Reference))
  (bind _asplayer_controller (Utilities|Casting|CastToPlayerController ExitingController))
  (CallFunction|AddTextMessage 0 (Utilities|String|Append (Class|AdvancedSessionsLibrary|GetPlayerName _asplayer_controller) " left the game.") true)
  (Utilities|Array|RemoveItem (Variables|Default|GetAllPCs) _asplayer_controller)
  (CallFunction|MakeCharacterAvailableAgain))

(fn ConstructionScript)

(fn GetAllPlayerData
  (for _array_element (Variables|Default|GetAllPCs)
    (bind _asbp_lobby_pc (Utilities|Casting|CastToBP_LobbyPC _array_element))
    (Utilities|Array|Add (LocalVariables|GetallIDs) (Utilities|Struct|MakePlayerWidgetUpdate_Structure (Class|AdvancedSessionsLibrary|GetUniqueNetID _asbp_lobby_pc) (Variables|/Game/Server/BP_LobbyPC.BP_LobbyPC_C|GetSelectedCharacterIndex _asbp_lobby_pc) (Variables|/Game/Server/BP_LobbyPC.BP_LobbyPC_C|GetReadyServer _asbp_lobby_pc) (Class|AdvancedSessionsLibrary|GetPlayerName _asbp_lobby_pc)))
    (if (Variables|/Game/Server/BP_LobbyPC.BP_LobbyPC_C|GetReadyServer _asbp_lobby_pc)
      _))
  (return (LocalVariables|GetallIDs)))

(fn FindPlayerIndexbyName
  (params (A :type String))
  (for (_array_element _array_index) (Variables|Default|GetAllPCs)
    (if (Utilities|Enum|Equal(Enum) A (Class|AdvancedSessionsLibrary|GetPlayerName _array_element))
      (return _array_index true)))
  (return 0 false))