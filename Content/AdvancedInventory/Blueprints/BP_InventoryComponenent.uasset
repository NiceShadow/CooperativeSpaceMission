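; Inventory component for the local player that handles dropping, picking up, focusing and consuming items, plus chest, shop and crafting bench interaction.
; A looping timer line-traces from the camera to set the focused item or station and toggle its prompt.
; Overlap events show or hide chest UI, auto-collect items and refresh the ground-item list.
; Pickups and UI updates go through interface messages on the HUD and PlayerController; consuming runs on a cancellable montage timer.
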(event Custom|Reset
  ;[1 1 1] Looping timer for focusing an item / chest / shop / player
  (Utilities|FlowControl|DoOnce false) ; enters at Reset
)

(event Custom|ConsumedItem
  (params (ID :type Integer))
  (if (== ID 0)
    _))

(event Custom|Pickup
  (bind _focuseditem (Variables|Default|GetFocusedItem))
  (bind _focuseditem_2 (Variables|Default|GetFocusedItem))
  ;[1 1 1] Pick up a focused item
  (if (Variables|Default|GetisFocusingItem?)
    (Utilities|IsValid (Variables|Default|GetFocusedItem)
      (:Is%20Valid
        (if (not (Variables|/Script/Engine.Actor|GetbHidden (Variables|Default|GetFocusedItem)))
          (if (Variables|Default|GetFocusedItemIsNewItemType?)
            (bind _asbp_new_drop_item_actor_master (Utilities|Casting|CastToBP_NewDropItemActor_Master _focuseditem_2))
            (else
              (bind _asbp_old_drop_item_actor_master (Utilities|Casting|CastToBP_OldDropItemActor_Master _focuseditem_2))))
          ;;[0.4766 1 0.7282] new in v 1.6 (BugFix)
          (Class|BPInterfaceInventory|AddItemI(Message) (HUD|GetHUD (Game|GetPlayerController 0)) (.ID (Utilities|Struct|BreakItem_Structur (select (Variables|Default|GetFocusedItemIsNewItemType?) (Variables|/Game/AdvancedInventory/Blueprints/BP_NewDropItemActor_Master.BP_NewDropItemActor_Master_C|GetItemData _asbp_new_drop_item_actor_master) (Variables|/Game/AdvancedInventory/Blueprints/BP_OldDropItemActor_Master.BP_OldDropItemActor_Master_C|GetItemData _asbp_old_drop_item_actor_master)))) (.amount (Utilities|Struct|BreakItem_Structur (select (Variables|Default|GetFocusedItemIsNewItemType?) (Variables|/Game/AdvancedInventory/Blueprints/BP_NewDropItemActor_Master.BP_NewDropItemActor_Master_C|GetItemData _asbp_new_drop_item_actor_master) (Variables|/Game/AdvancedInventory/Blueprints/BP_OldDropItemActor_Master.BP_OldDropItemActor_Master_C|GetItemData _asbp_old_drop_item_actor_master)))) (select (.TransferWholeItemData? (Utilities|Struct|BreakItem_Structur (select (Variables|Default|GetFocusedItemIsNewItemType?) (Variables|/Game/AdvancedInventory/Blueprints/BP_NewDropItemActor_Master.BP_NewDropItemActor_Master_C|GetItemData _asbp_new_drop_item_actor_master) (Variables|/Game/AdvancedInventory/Blueprints/BP_OldDropItemActor_Master.BP_OldDropItemActor_Master_C|GetItemData _asbp_old_drop_item_actor_master)))) (select (Variables|Default|GetFocusedItemIsNewItemType?) (Variables|/Game/AdvancedInventory/Blueprints/BP_NewDropItemActor_Master.BP_NewDropItemActor_Master_C|GetItemData _asbp_new_drop_item_actor_master) (Variables|/Game/AdvancedInventory/Blueprints/BP_OldDropItemActor_Master.BP_OldDropItemActor_Master_C|GetItemData _asbp_old_drop_item_actor_master)) "") (.TransferWholeItemData? (Utilities|Struct|BreakItem_Structur (select (Variables|Default|GetFocusedItemIsNewItemType?) (Variables|/Game/AdvancedInventory/Blueprints/BP_NewDropItemActor_Master.BP_NewDropItemActor_Master_C|GetItemData _asbp_new_drop_item_actor_master) (Variables|/Game/AdvancedInventory/Blueprints/BP_OldDropItemActor_Master.BP_OldDropItemActor_Master_C|GetItemData _asbp_old_drop_item_actor_master)))) false (select (.isBackpack? (Utilities|Struct|BreakItem_Structur (select (Variables|Default|GetFocusedItemIsNewItemType?) (Variables|/Game/AdvancedInventory/Blueprints/BP_NewDropItemActor_Master.BP_NewDropItemActor_Master_C|GetItemData _asbp_new_drop_item_actor_master) (Variables|/Game/AdvancedInventory/Blueprints/BP_OldDropItemActor_Master.BP_OldDropItemActor_Master_C|GetItemData _asbp_old_drop_item_actor_master)))) (select (Variables|Default|GetFocusedItemIsNewItemType?) (Variables|/Game/AdvancedInventory/Blueprints/BP_NewDropItemActor_Master.BP_NewDropItemActor_Master_C|GetBackpackData _asbp_new_drop_item_actor_master) (Variables|/Game/AdvancedInventory/Blueprints/BP_OldDropItemActor_Master.BP_OldDropItemActor_Master_C|GetBackpackData _asbp_old_drop_item_actor_master)) ""))
          (Rendering|SetActorHiddenInGame _focuseditem true)
          (Class|BPInterfaceInventory|DestroyActorI(Message) (Game|GetPlayerController 0) _focuseditem)
          (CallFunction|Reset))))))

(event Custom|LinetraceLoop
  (bind _returnvalue (Game|GetPlayerCameraManager 0))
  (bind _returnvalue_2 (Camera|GetCameraLocation _returnvalue))
  ;[1 1 1] Looping timer for focusing an item / chest / shop / player
  (bind (_outhit _returnvalue_3) (Collision|LineTraceByChannel _returnvalue_2 (+ _returnvalue_2 (* (Math|Vector|GetForwardVector (Camera|GetCameraRotation _returnvalue)) 6.5e+02)) "TraceTypeQuery1" false (Utilities|Array|MakeArray (Game|GetPlayerCharacter 0)) "None"))
  (Variables|Default|SetCurrentHitActor (.HitActor (Collision|BreakHitResult _outhit)))
  (Utilities|FlowControl|Sequence
    (:then_0
      (Variables|Default|SetFocusedItemIsNewItemType? (== (Utilities|GetClass (Variables|Default|GetCurrentHitActor)) "/Game/AdvancedInventory/Blueprints/BP_NewDropItemActor_Master.BP_NewDropItemActor_Master_C"))
      (if (Math|Boolean|NANDBoolean _returnvalue_3 (Variables|Default|GetInspecting))
        (if (or (== (Utilities|GetClass (Variables|Default|GetCurrentHitActor)) "/Game/AdvancedInventory/Blueprints/BP_OldDropItemActor_Master.BP_OldDropItemActor_Master_C") (== (Utilities|GetClass (Variables|Default|GetCurrentHitActor)) "/Game/AdvancedInventory/Blueprints/BP_NewDropItemActor_Master.BP_NewDropItemActor_Master_C"))
          (Utilities|FlowControl|Sequence
            (:then_0
              (if (Variables|Default|GetFocusedItemIsNewItemType?)
                (bind _asbp_new_drop_item_actor_master (Utilities|Casting|CastToBP_NewDropItemActor_Master (Variables|Default|GetCurrentHitActor)))
                (else
                  (bind _asbp_old_drop_item_actor_master (Utilities|Casting|CastToBP_OldDropItemActor_Master (Variables|Default|GetCurrentHitActor)))))
              (if (Math|Boolean|ORBoolean (!= (.ID (Utilities|Struct|BreakItem_Structur (select (Variables|Default|GetFocusedItemIsNewItemType?) (Variables|/Game/AdvancedInventory/Blueprints/BP_NewDropItemActor_Master.BP_NewDropItemActor_Master_C|GetItemData _asbp_new_drop_item_actor_master) (Variables|/Game/AdvancedInventory/Blueprints/BP_OldDropItemActor_Master.BP_OldDropItemActor_Master_C|GetItemData _asbp_old_drop_item_actor_master)))) (Variables|Default|GetcompareID)) (!= (.amount (Utilities|Struct|BreakItem_Structur (select (Variables|Default|GetFocusedItemIsNewItemType?) (Variables|/Game/AdvancedInventory/Blueprints/BP_NewDropItemActor_Master.BP_NewDropItemActor_Master_C|GetItemData _asbp_new_drop_item_actor_master) (Variables|/Game/AdvancedInventory/Blueprints/BP_OldDropItemActor_Master.BP_OldDropItemActor_Master_C|GetItemData _asbp_old_drop_item_actor_master)))) (Variables|Default|GetcompareAmount)) (!= (Variables|Default|GetCurrentHitActor) (Variables|Default|GetFocusedItem)))
                (Variables|Default|SetcompareID (.ID (Utilities|Struct|BreakItem_Structur (select (Variables|Default|GetFocusedItemIsNewItemType?) (Variables|/Game/AdvancedInventory/Blueprints/BP_NewDropItemActor_Master.BP_NewDropItemActor_Master_C|GetItemData _asbp_new_drop_item_actor_master) (Variables|/Game/AdvancedInventory/Blueprints/BP_OldDropItemActor_Master.BP_OldDropItemActor_Master_C|GetItemData _asbp_old_drop_item_actor_master)))))
                (Variables|Default|SetcompareAmount (.amount (Utilities|Struct|BreakItem_Structur (select (Variables|Default|GetFocusedItemIsNewItemType?) (Variables|/Game/AdvancedInventory/Blueprints/BP_NewDropItemActor_Master.BP_NewDropItemActor_Master_C|GetItemData _asbp_new_drop_item_actor_master) (Variables|/Game/AdvancedInventory/Blueprints/BP_OldDropItemActor_Master.BP_OldDropItemActor_Master_C|GetItemData _asbp_old_drop_item_actor_master)))))
                (bind _inventory (Class|BPInterfaceInventory|GetInventoryRefI(Message) (HUD|GetHUD (Game|GetPlayerController 0))))
                (Utilities|IsValid _inventory
                  (:Is%20Valid
                    (if (Variables|Default|GetShowNewPickupInfo)
                      (if (and (!= (Variables|Default|GetCurrentHitActor) (Variables|Default|GetFocusedItem)) (Utilities|IsValid (Variables|Default|GetFocusedItem)))
                        (bind _asbp_new_drop_item_actor_master_2 (Utilities|Casting|CastToBP_NewDropItemActor_Master (Variables|Default|GetFocusedItem)))
                        (Default|ShowNewInfoWidget _asbp_new_drop_item_actor_master_2 false))
                      (if (Variables|Default|GetFocusedItemIsNewItemType?)
                        (Default|ShowNewInfoWidget _asbp_new_drop_item_actor_master true))
                      (else
                        (Default|ShowPickUpInfo _inventory true (select (Variables|Default|GetFocusedItemIsNewItemType?) (Variables|/Game/AdvancedInventory/Blueprints/BP_NewDropItemActor_Master.BP_NewDropItemActor_Master_C|GetItemData _asbp_new_drop_item_actor_master) (Variables|/Game/AdvancedInventory/Blueprints/BP_OldDropItemActor_Master.BP_OldDropItemActor_Master_C|GetItemData _asbp_old_drop_item_actor_master)))))
                    (Variables|Default|SetFocusedItem (Variables|Default|GetCurrentHitActor))
                    (if (not (Variables|Default|GetisFocusingItem?))
                      (Variables|Default|SetisFocusingItem? true))))))
            (:then_1
              (goto _label Reset)))
          (else
            (Utilities|FlowControl|DoOnce false :!label _label
              (:Completed
                (Variables|Default|SetcompareAmount -1)
                (Variables|Default|SetcompareID -1)
                (bind _inventory_2 (Class|BPInterfaceInventory|GetInventoryRefI(Message) (HUD|GetHUD (Game|GetPlayerController 0))))
                (Utilities|IsValid _inventory_2
                  (:Is%20Valid
                    (Variables|Default|SetisFocusingItem? false)
                    (if (Variables|Default|GetShowNewPickupInfo)
                      (if (Utilities|IsValid (Variables|Default|GetFocusedItem))
                        (bind _asbp_new_drop_item_actor_master_3 (Utilities|Casting|CastToBP_NewDropItemActor_Master (Variables|Default|GetFocusedItem)))
                        (Default|ShowNewInfoWidget _asbp_new_drop_item_actor_master_3 false))
                      (else
                        (Default|ShowPickUpInfo _inventory_2 false)))))))))
        (else
          (goto _label))))
    (:then_1
      (if (and (Math|Boolean|NANDBoolean _returnvalue_3 (Variables|Default|GetInspecting)) (< (.Distance (Collision|BreakHitResult _outhit)) (Variables|Default|GetMaxScanLenghtForChestFocus)))
        (if (!= (Variables|Default|GetCurrentHitActor) (Variables|Default|GetFocusedChest))
          (if (CallFunction|IsChestClass? (Utilities|GetClass (Variables|Default|GetCurrentHitActor)))
            (bind _asbp_chest (Utilities|Casting|CastToBP_Chest (Variables|Default|GetCurrentHitActor)))
            (if (or (Variables|/Game/AdvancedInventory/Blueprints/BP_Chest.BP_Chest_C|GetOnlyOpenOnInteraction _asbp_chest) (Variables|/Game/AdvancedInventory/Blueprints/BP_Chest.BP_Chest_C|GetisLootbox? _asbp_chest))
              (if (and (!= _asbp_chest (Variables|Default|GetFocusedChest)) (Utilities|IsValid (Variables|Default|GetFocusedChest)))
                (Default|ShowPressE (Variables|Default|GetFocusedChest) false))
              (Default|ShowPressE _asbp_chest true)
              (Variables|Default|SetFocusedChest _asbp_chest)
              (Variables|Default|SetisFocusingChest? true)
              (Class|BPInterfaceInventory|SetFocusedChestI(Message) (Game|GetPlayerController 0) (Variables|Default|GetFocusedChest) :!label _label_2)
              (else
                (if (Variables|Default|GetisFocusingChest?) :!label _label_3
                  (Default|ShowPressE (Variables|Default|GetFocusedChest) false)
                  (Default|UpdateOpeningProgress (Variables|Default|GetFocusedChest) 0.0)
                  (Variables|Default|SetFocusedChest 0)
                  (Variables|Default|SetisFocusingChest? false)
                  (goto _label_2)
                  (else
                    ;;[0.4766 1 0.7282] new in v 1.6
                    (if (Variables|Default|GetisFocusingShop?)
                      (Default|ShowPressInteractionWidget (Variables|Default|GetFocusedShop) false)
                      (Variables|Default|SetFocusedShop 0)
                      (Variables|Default|SetisFocusingShop? false)
                      (Class|BPInterfaceInventory|SetFocusedShopI(Message) (Game|GetPlayerController 0) (Variables|Default|GetFocusedShop) :!label _label_4)
                      (else
                        (if (Variables|Default|GetisFocusingCraftingBench) :!label _label_5
                          (Default|ShowPressInteractionWidget (Variables|Default|GetFocusedCraftingBench) false)
                          (Variables|Default|SetFocusedCraftingBench 0)
                          (Variables|Default|SetisFocusingCraftingBench false)
                          (bind _asbp_inventory_player_controller (Utilities|Casting|CastToBP_InventoryPlayerController (Game|GetPlayerController 0) :!label _label_6))
                          (Default|SetFocusedCraftingBench _asbp_inventory_player_controller (Variables|Default|GetFocusedCraftingBench)))))))))
            (else
              (Utilities|FlowControl|Sequence
                (:then_0
                  (goto _label_3))
                (:then_1
                  (if (== (Utilities|GetClass (Variables|Default|GetCurrentHitActor)) "/Game/AdvancedInventory/Blueprints/BP_Shop.BP_Shop_C") :!label _label_7
                    (bind _asbp_shop (Utilities|Casting|CastToBP_Shop (Variables|Default|GetCurrentHitActor)))
                    (if (and (!= _asbp_shop (Variables|Default|GetFocusedShop)) (Utilities|IsValid (Variables|Default|GetFocusedShop)))
                      (Default|ShowPressInteractionWidget (Variables|Default|GetFocusedShop) false))
                    (Default|ShowPressInteractionWidget _asbp_shop true)
                    (Variables|Default|SetFocusedShop _asbp_shop)
                    (Variables|Default|SetisFocusingShop? true)
                    (goto _label_4)
                    (else
                      (if (== (Utilities|GetClass (Variables|Default|GetCurrentHitActor)) "/Game/AdvancedInventory/Blueprints/BP_CraftingBench.BP_CraftingBench_C") :!label _label_8
                        (bind _asbp_crafting_bench (Utilities|Casting|CastToBP_CraftingBench (Variables|Default|GetCurrentHitActor)))
                        (if (and (!= _asbp_crafting_bench (Variables|Default|GetFocusedCraftingBench)) (Utilities|IsValid (Variables|Default|GetFocusedCraftingBench)))
                          (Default|ShowPressInteractionWidget (Variables|Default|GetFocusedCraftingBench) false))
                        (Default|ShowPressInteractionWidget _asbp_crafting_bench true)
                        (Variables|Default|SetFocusedCraftingBench _asbp_crafting_bench)
                        (Variables|Default|SetisFocusingCraftingBench true)
                        (goto _label_6)
                        (else
                          (goto _label_5)))))))))
          (elif (!= (Variables|Default|GetCurrentHitActor) (Variables|Default|GetFocusedShop))
            (goto _label_7)
            (elif (!= (Variables|Default|GetCurrentHitActor) (Variables|Default|GetFocusedCraftingBench))
              (goto _label_8))))
        (else
          (goto _label_3))))))

(event Custom|On%28End%29Overlap%20ItemRadiusForGroundList
  ;[1 1 1] Update the GroundItemList when the radius overlaps or ends to overlap an item
  (CallFunction|UpdateGroundItemList))

(event Custom|Reactivate
  ;[1 1 1] Auto Pickup Mode - The player automatically picks up an item when the character collides with it
  (bind _autopickupmode_ (Class|BPInterfaceInventory|GetAutoPickUpModeI(Message) (Game|GetPlayerController 0)))
  (if _autopickupmode_
    (if (== (Utilities|GetClass (stale Custom|PickUpAllItemsBeginOverlap Actor)) "/Game/AdvancedInventory/Blueprints/BP_NewDropItemActor_Master.BP_NewDropItemActor_Master_C")
      (bind _asbp_new_drop_item_actor_master (Utilities|Casting|CastToBP_NewDropItemActor_Master (stale Custom|PickUpAllItemsBeginOverlap Actor)))
      (Class|BPInterfaceInventory|AddItemI(Message) (HUD|GetHUD (Game|GetPlayerController 0)) (.ID (Utilities|Struct|BreakItem_Structur (select (== (Utilities|GetClass (stale Custom|PickUpAllItemsBeginOverlap Actor)) "/Game/AdvancedInventory/Blueprints/BP_OldDropItemActor_Master.BP_OldDropItemActor_Master_C") (Variables|/Game/AdvancedInventory/Blueprints/BP_OldDropItemActor_Master.BP_OldDropItemActor_Master_C|GetItemData (stale _asbp_old_drop_item_actor_master)) (Variables|/Game/AdvancedInventory/Blueprints/BP_NewDropItemActor_Master.BP_NewDropItemActor_Master_C|GetItemData _asbp_new_drop_item_actor_master)))) (.amount (Utilities|Struct|BreakItem_Structur (select (== (Utilities|GetClass (stale Custom|PickUpAllItemsBeginOverlap Actor)) "/Game/AdvancedInventory/Blueprints/BP_OldDropItemActor_Master.BP_OldDropItemActor_Master_C") (Variables|/Game/AdvancedInventory/Blueprints/BP_OldDropItemActor_Master.BP_OldDropItemActor_Master_C|GetItemData (stale _asbp_old_drop_item_actor_master)) (Variables|/Game/AdvancedInventory/Blueprints/BP_NewDropItemActor_Master.BP_NewDropItemActor_Master_C|GetItemData _asbp_new_drop_item_actor_master)))) (select (.TransferWholeItemData? (Utilities|Struct|BreakItem_Structur (select (== (Utilities|GetClass (stale Custom|PickUpAllItemsBeginOverlap Actor)) "/Game/AdvancedInventory/Blueprints/BP_OldDropItemActor_Master.BP_OldDropItemActor_Master_C") (Variables|/Game/AdvancedInventory/Blueprints/BP_OldDropItemActor_Master.BP_OldDropItemActor_Master_C|GetItemData (stale _asbp_old_drop_item_actor_master)) (Variables|/Game/AdvancedInventory/Blueprints/BP_NewDropItemActor_Master.BP_NewDropItemActor_Master_C|GetItemData _asbp_new_drop_item_actor_master)))) (select (== (Utilities|GetClass (stale Custom|PickUpAllItemsBeginOverlap Actor)) "/Game/AdvancedInventory/Blueprints/BP_OldDropItemActor_Master.BP_OldDropItemActor_Master_C") (Variables|/Game/AdvancedInventory/Blueprints/BP_OldDropItemActor_Master.BP_OldDropItemActor_Master_C|GetItemData (stale _asbp_old_drop_item_actor_master)) (Variables|/Game/AdvancedInventory/Blueprints/BP_NewDropItemActor_Master.BP_NewDropItemActor_Master_C|GetItemData _asbp_new_drop_item_actor_master)) "") (.TransferWholeItemData? (Utilities|Struct|BreakItem_Structur (select (== (Utilities|GetClass (stale Custom|PickUpAllItemsBeginOverlap Actor)) "/Game/AdvancedInventory/Blueprints/BP_OldDropItemActor_Master.BP_OldDropItemActor_Master_C") (Variables|/Game/AdvancedInventory/Blueprints/BP_OldDropItemActor_Master.BP_OldDropItemActor_Master_C|GetItemData (stale _asbp_old_drop_item_actor_master)) (Variables|/Game/AdvancedInventory/Blueprints/BP_NewDropItemActor_Master.BP_NewDropItemActor_Master_C|GetItemData _asbp_new_drop_item_actor_master)))) false (select (.isBackpack? (Utilities|Struct|BreakItem_Structur (select (== (Utilities|GetClass (stale Custom|PickUpAllItemsBeginOverlap Actor)) "/Game/AdvancedInventory/Blueprints/BP_OldDropItemActor_Master.BP_OldDropItemActor_Master_C") (Variables|/Game/AdvancedInventory/Blueprints/BP_OldDropItemActor_Master.BP_OldDropItemActor_Master_C|GetItemData (stale _asbp_old_drop_item_actor_master)) (Variables|/Game/AdvancedInventory/Blueprints/BP_NewDropItemActor_Master.BP_NewDropItemActor_Master_C|GetItemData _asbp_new_drop_item_actor_master)))) (select (== (Utilities|GetClass (stale Custom|PickUpAllItemsBeginOverlap Actor)) "/Game/AdvancedInventory/Blueprints/BP_OldDropItemActor_Master.BP_OldDropItemActor_Master_C") (Variables|/Game/AdvancedInventory/Blueprints/BP_OldDropItemActor_Master.BP_OldDropItemActor_Master_C|GetBackpackData (stale _asbp_old_drop_item_actor_master)) (Variables|/Game/AdvancedInventory/Blueprints/BP_NewDropItemActor_Master.BP_NewDropItemActor_Master_C|GetBackpackData _asbp_new_drop_item_actor_master)) "") :!label _label)
      ;;[0.4766 1 0.7282] new in v 1.6 (BugFix)
      (Rendering|SetActorHiddenInGame (stale Custom|PickUpAllItemsBeginOverlap Actor) true)
      (Class|BPInterfaceInventory|DestroyActorI(Message) (Game|GetPlayerController 0) (stale Custom|PickUpAllItemsBeginOverlap Actor))
      (CallFunction|Reset)
      (elif (== (Utilities|GetClass (stale Custom|PickUpAllItemsBeginOverlap Actor)) "/Game/AdvancedInventory/Blueprints/BP_OldDropItemActor_Master.BP_OldDropItemActor_Master_C")
        (bind _asbp_old_drop_item_actor_master (Utilities|Casting|CastToBP_OldDropItemActor_Master (stale Custom|PickUpAllItemsBeginOverlap Actor)))
        (goto _label)))))

(event Custom|ActorEndOverlap
  (params (Actor :type Actor%20Object%20Reference))
  (bind _returnvalue (Game|GetPlayerController 0))
  (bind _returnvalue_2 (Utilities|GetClass Actor))
  ;[1 1 1] Hide chestUI again
  (if (CallFunction|IsChestClass? _returnvalue_2)
    (Variables|Default|SetisOverlapping%20Chest? false)
    (bind _inventory (Class|BPInterfaceInventory|GetInventoryRefI(Message) (HUD|GetHUD (Game|GetPlayerController 0))))
    (Utilities|IsValid _inventory
      (:Is%20Valid
        (if (== (Variables|/Game/AdvancedInventory/Widgets/WB_ChestUI.WB_ChestUI_C|GetChest (Variables|/Game/AdvancedInventory/Widgets/WB_Inventory.WB_Inventory_C|GetChestUI _inventory)) Actor)
          (Default|Hide (Variables|/Game/AdvancedInventory/Widgets/WB_Inventory.WB_Inventory_C|GetChestUI _inventory))
          (Class|BPInterfaceInventory|SetIsinRadiusOfChestI(Message) _returnvalue false)
          (bind _asbp_inventory_player_controller (Utilities|Casting|CastToBP_InventoryPlayerController _returnvalue :!label _label))
          (Default|ShowInventory (Variables|/Game/AdvancedInventory/Blueprints/BP_InventoryPlayerController.BP_InventoryPlayerController_C|GetBP_PlayercontrollerComponent _asbp_inventory_player_controller) false true))))
    (elif (== _returnvalue_2 "/Game/AdvancedInventory/Blueprints/BP_Shop.BP_Shop_C")
      (Variables|Default|SetisOverlappingShop false)
      (bind _inventory_2 (Class|BPInterfaceInventory|GetInventoryRefI(Message) (HUD|GetHUD (Game|GetPlayerController 0))))
      (Utilities|IsValid _inventory_2
        (:Is%20Valid
          (if (== Actor (Variables|/Game/AdvancedInventory/Widgets/WB_ChestUI.WB_ChestUI_C|GetShop (Variables|/Game/AdvancedInventory/Widgets/WB_Inventory.WB_Inventory_C|GetChestUI _inventory_2)))
            (Default|Hide (Variables|/Game/AdvancedInventory/Widgets/WB_Inventory.WB_Inventory_C|GetChestUI _inventory_2))
            (goto _label))))
      (elif (== _returnvalue_2 "/Game/AdvancedInventory/Blueprints/BP_CraftingBench.BP_CraftingBench_C")
        (bind _inventory_3 (Class|BPInterfaceInventory|GetInventoryRefI(Message) (HUD|GetHUD (Game|GetPlayerController 0))))
        (Utilities|IsValid _inventory_3
          (:Is%20Valid
            (if (== Actor (Variables|/Game/AdvancedInventory/Widgets/WB_ChestUI.WB_ChestUI_C|GetCraftingBench (Variables|/Game/AdvancedInventory/Widgets/WB_Inventory.WB_Inventory_C|GetChestUI _inventory_3)))
              (Default|Hide (Variables|/Game/AdvancedInventory/Widgets/WB_Inventory.WB_Inventory_C|GetChestUI _inventory_3))
              (goto _label))))))))

(event Custom|DropEvent
  (params (ItemData :type Item%20Structur%20Structure) (BackpackData :type Backpack%20Data%20Structure%20Structure))
  (bind (_amount _stackable_) (Utilities|Struct|BreakItem_Structur ItemData))
  (bind _returnvalue (Game|GetPlayerCharacter 0))
  (bind _returnvalue_2 (> _amount 1))
  (bind _returnvalue_3 (Transformation|GetActorLocation _returnvalue))
  (bind _returnvalue_4 (not _stackable_))
  (bind (_x _y _z) (Math|Vector|BreakVector _returnvalue_3))
  (bind _returnvalue_5 (and _returnvalue_2 _returnvalue_4))
  ;[1 1 1] Drop an item
  (if _returnvalue_5
    (bind _output_get (Variables|Default|SetDropIndexFix (- _amount 1)))
    (for _index (range 0 _output_get)
      (bind _structout (Utilities|Struct|SetmembersinItem_Structur ItemData 1))
      (CallFunction|SpawnItemonServer (Math|Transform|MakeTransform (Math|Vector|MakeVector _x _y (+ 4e+01 _z)) (Math|Rotator|MakeRotator 0.0 0.0 (.Yaw (Math|Rotator|BreakRotator (Transformation|GetActorRotation _returnvalue))))) (Variables|Default|GetRandomItemDropSpeed) (select _returnvalue_5 _structout ItemData) (* (.Pitch (Math|Rotator|BreakRotator (Camera|GetCameraRotation (Game|GetPlayerCameraManager 0)))) 12.0) 0.0 true BackpackData))
    (else
      (CallFunction|SpawnItemonServer (Math|Transform|MakeTransform (Math|Vector|MakeVector _x _y (+ 4e+01 _z)) (Math|Rotator|MakeRotator 0.0 0.0 (.Yaw (Math|Rotator|BreakRotator (Transformation|GetActorRotation _returnvalue))))) (Variables|Default|GetRandomItemDropSpeed) (select _returnvalue_5 _structout ItemData) (* (.Pitch (Math|Rotator|BreakRotator (Camera|GetCameraRotation (Game|GetPlayerCameraManager 0)))) 12.0) 0.0 true BackpackData))))

(event Custom|SpawnItemOnServer
  (params (SpawnTransform :type Transform) (Speed :type Float%20%28single-precision%29) (ItemData :type Item%20Structur%20Structure) (zVelocity :type Float%20%28single-precision%29) (xVelocity :type Float%20%28single-precision%29) (SpawnNewItemType :type Boolean) (BackpackData :type Backpack%20Data%20Structure%20Structure))
  ;[1 1 1] Drop an item
  (if SpawnNewItemType
    (bind _returnvalue (Game|SpawnActorfromClass "/Game/AdvancedInventory/Blueprints/BP_NewDropItemActor_Master.BP_NewDropItemActor_Master_C" SpawnTransform "Undefined" 0 Speed ItemData zVelocity xVelocity false 0 1 BackpackData false false 0 0 0))
    ;;[0.4766 1 0.7282] new in v 1.6
    (Default|Update _returnvalue ItemData)
    (Default|UpdateBackpackData _returnvalue BackpackData)
    (else
      (Game|SpawnActorfromClass "/Game/AdvancedInventory/Blueprints/BP_OldDropItemActor_Master.BP_OldDropItemActor_Master_C" SpawnTransform "Undefined" 0 Speed ItemData zVelocity xVelocity false 0 1 BackpackData 0))))

(event Custom|StartLineTraceLoop
  ;[1 1 1] Looping timer for focusing an item / chest / shop / player
  (Utilities|Time|SetTimerbyEvent (delegate Custom|LinetraceLoop) 0.1 true))

(event Custom|Finished
  (bind _returnvalue (Game|GetPlayerCharacter 0))
  ;[0 1 0.04334] example: bandage
  (CallFunction|ConsumedItem (stale Custom|ConsumeItemEvent ID))
  (Class|BPInterfaceInventory|FinishedConsumeItemI(Message) (Game|GetPlayerController 0))
  (Variables|Default|SetIsConsumingSomething false)
  (Class|BPCharacterInterface|SetRightHandMeshVisibility(Message) _returnvalue true)
  (Class|BPCharacterInterface|CharacterPlayMontage(Message) _returnvalue 0 1.0 true false)
  (Default|ShowConsumingTime (stale Custom|ConsumeItemEvent InputPin) false)
  (bind _inventory (Class|BPInterfaceInventory|GetInventoryRefI(Message) (HUD|GetHUD (Game|GetPlayerController 0))))
  (Default|AddItemInfotoBox _inventory 1 false (.Name (Utilities|Struct|BreakItem_Structur (Variables|/Game/AdvancedInventory/Widgets/WB_Item.WB_Item_C|GetItemData (stale Custom|ConsumeItemEvent InputPin)))) (.image (Utilities|Struct|BreakItem_Structur (Variables|/Game/AdvancedInventory/Widgets/WB_Item.WB_Item_C|GetItemData (stale Custom|ConsumeItemEvent InputPin)))) false true))

(event Custom|Setup
  (params (CameraRef :type Camera%20Component%20Object%20Reference))
  ;[1 1 1] SetUp
  (Class|BPInterfaceInventory|SetInventoryComponentRefI(Message) (Game|GetPlayerController 0) self)
  (Variables|Default|SetCameraRef CameraRef))

(event Custom|ConsumeItemEvent
  (params (ID :type Integer) (InputPin :type WB%20Item%20Object%20Reference) (isFalling :type Boolean) (IndexOfMontageArray :type Integer))
  (bind _itemdata (Variables|/Game/AdvancedInventory/Widgets/WB_Item.WB_Item_C|GetItemData InputPin))
  (bind (_consumemontage _consumetime) (Utilities|Struct|BreakItem_Structur _itemdata))
  ;[1 1 1] Consume an item
  (if (not isFalling)
    ;[0 1 0.04334] example: bandage
    (if (or (== ID 9) false)
      (Variables|Default|SetIsConsumingSomething true)
      (Class|BPCharacterInterface|SetRightHandMeshVisibility(Message) (Game|GetPlayerCharacter 0) false)
      (Class|BPCharacterInterface|CharacterPlayMontage(Message) (Game|GetPlayerCharacter 0) (Utilities|Array|Get(acopy) _consumemontage IndexOfMontageArray) 1.5 false true)
      (bind _returnvalue (Utilities|Time|SetTimerbyEvent (delegate Custom|Finished) _consumetime))
      (bind _output_get (Variables|Default|SetConsumeItemTimer _returnvalue))
      (Default|ShowConsumingTime InputPin true _output_get))))

(event Custom|CancelConsume
  (params (Target :type WB%20Item%20Object%20Reference))
  ;[1 1 1] Cancel the consume of an item
  (Class|BPCharacterInterface|CharacterPlayMontage(Message) (Game|GetPlayerCharacter 0) 0 1.0 true false)
  (Utilities|Time|ClearandInvalidateTimerbyHandle (Variables|Default|GetConsumeItemTimer))
  (Variables|Default|SetIsConsumingSomething false)
  (Class|BPCharacterInterface|SetRightHandMeshVisibility(Message) (Game|GetPlayerCharacter 0) true)
  (Default|ShowConsumingTime Target false))

(event Custom|ActorBeginOverlap
  (params (Actor :type Actor%20Object%20Reference))
  (bind _returnvalue (Utilities|GetClass Actor))
  ;[1 1 1] Show the chestUI when the player enters the radius of a chest
  (if (CallFunction|IsChestClass? _returnvalue)
    (Variables|Default|SetisOverlapping%20Chest? true)
    (bind _asbp_chest (Utilities|Casting|CastToBP_Chest Actor))
    (if (not (or (Variables|/Game/AdvancedInventory/Blueprints/BP_Chest.BP_Chest_C|GetOnlyOpenOnInteraction _asbp_chest) (Variables|/Game/AdvancedInventory/Blueprints/BP_Chest.BP_Chest_C|GetisLootbox? _asbp_chest)))
      (bind _inventory (Class|BPInterfaceInventory|GetInventoryRefI(Message) (HUD|GetHUD (Game|GetPlayerController 0))))
      (Utilities|IsValid _inventory
        (:Is%20Valid
          (Default|UpateOwnChestUI (Variables|/Game/AdvancedInventory/Widgets/WB_Inventory.WB_Inventory_C|GetChestUI _inventory) _asbp_chest (Variables|/Game/AdvancedInventory/Blueprints/BP_Chest.BP_Chest_C|GetVisibility_items _asbp_chest) (Variables|/Game/AdvancedInventory/Blueprints/BP_Chest.BP_Chest_C|GetData_items _asbp_chest) (Variables|/Game/AdvancedInventory/Blueprints/BP_Chest.BP_Chest_C|GetBackpackData_Items _asbp_chest))
          (Default|Show (Variables|/Game/AdvancedInventory/Widgets/WB_Inventory.WB_Inventory_C|GetChestUI _inventory))
          (Class|BPInterfaceInventory|SetIsinRadiusOfChestI(Message) (Game|GetPlayerController 0) true))))
    (else
      ;;[0.4766 1 0.7282] new in v 1.6
      (if (== _returnvalue "/Game/AdvancedInventory/Blueprints/BP_Shop.BP_Shop_C")
        (Variables|Default|SetisOverlappingShop true)))))

(event Custom|PickUpAllItemsBeginOverlap
  (params (Actor :type Actor%20Object%20Reference))
  (bind _returnvalue (Utilities|GetClass Actor))
  (bind _returnvalue_2 (== _returnvalue "/Game/AdvancedInventory/Blueprints/BP_OldDropItemActor_Master.BP_OldDropItemActor_Master_C"))
  ;[1 1 1] Auto Pickup Mode - The player automatically picks up an item when the character collides with it
  ;;[0.4766 1 0.7282] new in v 1.6 (BugFix)
  (Utilities|IsValid Actor
    (:Is%20Valid
      (if (not (Variables|/Script/Engine.Actor|GetbHidden Actor))
        (if (== _returnvalue "/Game/AdvancedInventory/Blueprints/BP_NewDropItemActor_Master.BP_NewDropItemActor_Master_C")
          (bind _asbp_new_drop_item_actor_master (Utilities|Casting|CastToBP_NewDropItemActor_Master Actor))
          (Class|BPInterfaceInventory|AddItemI(Message) (HUD|GetHUD (Game|GetPlayerController 0)) (.ID (Utilities|Struct|BreakItem_Structur (select _returnvalue_2 (Variables|/Game/AdvancedInventory/Blueprints/BP_OldDropItemActor_Master.BP_OldDropItemActor_Master_C|GetItemData (stale _asbp_old_drop_item_actor_master)) (Variables|/Game/AdvancedInventory/Blueprints/BP_NewDropItemActor_Master.BP_NewDropItemActor_Master_C|GetItemData _asbp_new_drop_item_actor_master)))) (.amount (Utilities|Struct|BreakItem_Structur (select _returnvalue_2 (Variables|/Game/AdvancedInventory/Blueprints/BP_OldDropItemActor_Master.BP_OldDropItemActor_Master_C|GetItemData (stale _asbp_old_drop_item_actor_master)) (Variables|/Game/AdvancedInventory/Blueprints/BP_NewDropItemActor_Master.BP_NewDropItemActor_Master_C|GetItemData _asbp_new_drop_item_actor_master)))) (select (.TransferWholeItemData? (Utilities|Struct|BreakItem_Structur (select _returnvalue_2 (Variables|/Game/AdvancedInventory/Blueprints/BP_OldDropItemActor_Master.BP_OldDropItemActor_Master_C|GetItemData (stale _asbp_old_drop_item_actor_master)) (Variables|/Game/AdvancedInventory/Blueprints/BP_NewDropItemActor_Master.BP_NewDropItemActor_Master_C|GetItemData _asbp_new_drop_item_actor_master)))) (select _returnvalue_2 (Variables|/Game/AdvancedInventory/Blueprints/BP_OldDropItemActor_Master.BP_OldDropItemActor_Master_C|GetItemData (stale _asbp_old_drop_item_actor_master)) (Variables|/Game/AdvancedInventory/Blueprints/BP_NewDropItemActor_Master.BP_NewDropItemActor_Master_C|GetItemData _asbp_new_drop_item_actor_master)) "") (.TransferWholeItemData? (Utilities|Struct|BreakItem_Structur (select _returnvalue_2 (Variables|/Game/AdvancedInventory/Blueprints/BP_OldDropItemActor_Master.BP_OldDropItemActor_Master_C|GetItemData (stale _asbp_old_drop_item_actor_master)) (Variables|/Game/AdvancedInventory/Blueprints/BP_NewDropItemActor_Master.BP_NewDropItemActor_Master_C|GetItemData _asbp_new_drop_item_actor_master)))) false (select (.isBackpack? (Utilities|Struct|BreakItem_Structur (select _returnvalue_2 (Variables|/Game/AdvancedInventory/Blueprints/BP_OldDropItemActor_Master.BP_OldDropItemActor_Master_C|GetItemData (stale _asbp_old_drop_item_actor_master)) (Variables|/Game/AdvancedInventory/Blueprints/BP_NewDropItemActor_Master.BP_NewDropItemActor_Master_C|GetItemData _asbp_new_drop_item_actor_master)))) (select _returnvalue_2 (Variables|/Game/AdvancedInventory/Blueprints/BP_OldDropItemActor_Master.BP_OldDropItemActor_Master_C|GetBackpackData (stale _asbp_old_drop_item_actor_master)) (Variables|/Game/AdvancedInventory/Blueprints/BP_NewDropItemActor_Master.BP_NewDropItemActor_Master_C|GetBackpackData _asbp_new_drop_item_actor_master)) "") :!label _label)
          ;;[0.4766 1 0.7282] new in v 1.6 (BugFix)
          (Rendering|SetActorHiddenInGame Actor true)
          (Class|BPInterfaceInventory|DestroyActorI(Message) (Game|GetPlayerController 0) Actor)
          (CallFunction|Reset)
          (elif _returnvalue_2
            (bind _asbp_old_drop_item_actor_master (Utilities|Casting|CastToBP_OldDropItemActor_Master Actor))
            (goto _label)))))))

(event EventBeginPlay
  ;[1 1 1] Looping timer for focusing an item / chest / shop / player
  (CallFunction|StartLineTraceLoop))

(fn UpdateGroundItemList
  ;[1 1 1] Update GroundItemList - Clear all children from the list, get all items of the "ItemRadiusForGroundList"-Component and add the new GroundItem children
  (bind _inventory (Class|BPInterfaceInventory|GetInventoryRefI(Message) (HUD|GetHUD (Game|GetPlayerController 0))))
  (Utilities|IsValid _inventory
    (:Is%20Valid
      (Default|HideAll (Variables|/Game/AdvancedInventory/Widgets/WB_Inventory.WB_Inventory_C|GetGroundItems _inventory))
      (bind _groundradius (Class|BPInterfaceInventory|GetGroundRadiusI(Message) (Game|GetPlayerController 0)))
      (Utilities|IsValid _groundradius
        (:Is%20Valid
          (LocalVariables|SetNewItemType true)
          (for (_array_element _array_index) (Collision|GetOverlappingActors _groundradius "/Game/AdvancedInventory/Blueprints/BP_NewDropItemActor_Master.BP_NewDropItemActor_Master_C" :!class /Script/Engine.PrimitiveComponent)
            (bind _asbp_new_drop_item_actor_master (Utilities|Casting|CastToBP_NewDropItemActor_Master _array_element))
            (Default|SetChildData (Variables|/Game/AdvancedInventory/Widgets/WB_Inventory.WB_Inventory_C|GetGroundItems _inventory) _array_index _array_element (.amount (Utilities|Struct|BreakItem_Structur (Variables|/Game/AdvancedInventory/Blueprints/BP_NewDropItemActor_Master.BP_NewDropItemActor_Master_C|GetItemData _asbp_new_drop_item_actor_master))) (.image (Utilities|Struct|BreakItem_Structur (Variables|/Game/AdvancedInventory/Blueprints/BP_NewDropItemActor_Master.BP_NewDropItemActor_Master_C|GetItemData _asbp_new_drop_item_actor_master)))))
          (LocalVariables|SetNewItemType false)
          (for (_array_element_2 _array_index_2) (Collision|GetOverlappingActors _groundradius "/Game/AdvancedInventory/Blueprints/BP_OldDropItemActor_Master.BP_OldDropItemActor_Master_C" :!class /Script/Engine.PrimitiveComponent)
            (bind _asbp_old_drop_item_actor_master (Utilities|Casting|CastToBP_OldDropItemActor_Master _array_element_2))))))))

(fn IsChestClass?
  (params (NewParam :type Actor%20Class%20Reference))
  ;[0.121 1 0.142] Add here all children of 'BP_Chest'
  (return (or (== NewParam "/Game/AdvancedInventory/Blueprints/BP_Chest.BP_Chest_C") (== NewParam "/Game/AdvancedInventory/Blueprints/BP_Chest_Child.BP_Chest_Child_C"))))

(fn GetFocusedItemItemforInspect
  (bind _inventory (Class|BPInterfaceInventory|GetInventoryRefI(Message) (HUD|GetHUD (Game|GetPlayerController 0))))
  (if (Variables|/Game/AdvancedInventory/Widgets/WB_ItemInfo.WB_ItemInfo_C|GetActivated (Variables|/Game/AdvancedInventory/Widgets/WB_Inventory.WB_Inventory_C|GetItemInformation _inventory))
    (return true (Variables|/Game/AdvancedInventory/Widgets/WB_ItemInfo.WB_ItemInfo_C|GetItemData (Variables|/Game/AdvancedInventory/Widgets/WB_Inventory.WB_Inventory_C|GetItemInformation _inventory)))
    (elif (Variables|Default|GetisFocusingItem?)
      (Utilities|IsValid (Variables|Default|GetFocusedItem)
        (:Is%20Valid
          (bind _asbp_new_drop_item_actor_master (Utilities|Casting|CastToBP_NewDropItemActor_Master (Variables|Default|GetFocusedItem))
            (:then
              (return true (Variables|/Game/AdvancedInventory/Blueprints/BP_NewDropItemActor_Master.BP_NewDropItemActor_Master_C|GetItemData _asbp_new_drop_item_actor_master)))
            (:CastFailed
              (return false ""))))
        (:Is%20Not%20Valid
          (return false "")))
      (else
        (return false "")))))