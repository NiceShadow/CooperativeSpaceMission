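; Master actor for inventory ground items, showing a pickup info widget and animating hover and spin unless SavePerformance is set.
; Items initialize from Item_Table when pre-placed, or receive item or backpack data and launch via projectile movement.
; When movement stops, stackable items merge into overlapping same-ID drops, and crowded drops hop again.
; Items blocked by placed objects escape using stepped directional traces, recreating their projectile component to fall or relaunch.
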(event OnProjectileStop(ProjectileMovement)
  (params (ImpactResult :type Hit%20Result%20Structure%20%28by%20ref%29))
  ;[1 1 1] If another item with the same ID comes in the radius of this item, the items will be merged
  (Utilities|FlowControl|Sequence
    (:then_0
      (if (> (Utilities|Array|Length (Collision|GetOverlappingActors (Variables|Default|GetBox) "BP_NewDropItemActor_Master_C" :!class /Script/Engine.PrimitiveComponent)) 2)
        (CallFunction|ReactiveProjectileMovement true)))
    (:then_1
      (bind _array_element (Utilities|Array|ForEachLoopwithBreak (Collision|GetOverlappingActors "BP_NewDropItemActor_Master_C" :!class /Script/Engine.Actor) :!label _label)
        (:LoopBody
          (if (!= _array_element self)
            (bind _asbp_new_drop_item_actor_master (Utilities|Casting|CastToBP_NewDropItemActor_Master _array_element))
            (if (and (== (.ID (Utilities|Struct|BreakItem_Structur (Variables|BP_NewDropItemActor_Master_C|GetItemData _asbp_new_drop_item_actor_master))) (.ID (Utilities|Struct|BreakItem_Structur (Variables|Default|GetItemData)))) (.Stackable? (Utilities|Struct|BreakItem_Structur (Variables|Default|GetItemData))))
              (CallFunction|IncreaseAmountAnimation _asbp_new_drop_item_actor_master)
              (bind _structout (Utilities|Struct|SetmembersinItem_Structur (Variables|Default|GetItemData) (+ (.amount (Utilities|Struct|BreakItem_Structur (Variables|BP_NewDropItemActor_Master_C|GetItemData _asbp_new_drop_item_actor_master))) (.amount (Utilities|Struct|BreakItem_Structur (Variables|Default|GetItemData))))))
              (Variables|BP_NewDropItemActor_Master_C|SetItemData _asbp_new_drop_item_actor_master _structout)
              (Actor|DestroyActor)
              (goto _label Break))))))))

(event OnComponentBeginOverlap(BoxTop)
  (params (OverlappedComponent :type Primitive%20Component%20Object%20Reference) (OtherActor :type Actor%20Object%20Reference) (OtherComp :type Primitive%20Component%20Object%20Reference) (OtherBodyIndex :type Integer) (bFromSweep :type Boolean) (SweepResult :type Hit%20Result%20Structure%20%28by%20ref%29))
  ;[1 1 1] When the item collides with a PlacingObject, a new location is necessary
  (if (Variables|Default|GetFindWayOutIfBlockedByDefinedObject)
    (bind (_location _itemshouldfalldown_) (CallFunction|FindWayOut))
    (Transformation|SetActorLocation (Math|Vector|MakeVector (.X (Math|Vector|BreakVector _location)) (.Y (Math|Vector|BreakVector _location)) (+ (.Z (Math|Vector|BreakVector _location)) 1e+01)) false false)
    (if _itemshouldfalldown_
      (CallFunction|ReactiveProjectileMovement false))))

(event OnComponentEndOverlap(BoxDown)
  (params (OverlappedComponent :type Primitive%20Component%20Object%20Reference) (OtherActor :type Actor%20Object%20Reference) (OtherComp :type Primitive%20Component%20Object%20Reference) (OtherBodyIndex :type Integer))
  ;[1 1 1] When the item is on the top of a PlacingObject and this object gets destroyed ist is necessary that the item falls down
  (if (Variables|Default|GetFindWayOutIfBlockedByDefinedObject)
    (CallFunction|ReactiveProjectileMovement false)))

(event OnProjectileStop(NewProjectileMovement)
  (params (ImpactResult :type Hit%20Result%20Structure%20%28by%20ref%29))
  ;[1 1 1] If another item with the same ID comes in the radius of this item, the items will be merged
  (Utilities|FlowControl|Sequence
    (:then_0
      (if (> (Utilities|Array|Length (Collision|GetOverlappingActors (Variables|Default|GetBox) "BP_NewDropItemActor_Master_C" :!class /Script/Engine.PrimitiveComponent)) 2)
        (CallFunction|ReactiveProjectileMovement true)))
    (:then_1
      (bind _array_element (Utilities|Array|ForEachLoopwithBreak (Collision|GetOverlappingActors "BP_NewDropItemActor_Master_C" :!class /Script/Engine.Actor) :!label _label)
        (:LoopBody
          (if (!= _array_element self)
            (bind _asbp_new_drop_item_actor_master (Utilities|Casting|CastToBP_NewDropItemActor_Master _array_element))
            (if (and (== (.ID (Utilities|Struct|BreakItem_Structur (Variables|BP_NewDropItemActor_Master_C|GetItemData _asbp_new_drop_item_actor_master))) (.ID (Utilities|Struct|BreakItem_Structur (Variables|Default|GetItemData)))) (.Stackable? (Utilities|Struct|BreakItem_Structur (Variables|Default|GetItemData))))
              (CallFunction|IncreaseAmountAnimation _asbp_new_drop_item_actor_master)
              (bind _structout (Utilities|Struct|SetmembersinItem_Structur (Variables|Default|GetItemData) (+ (.amount (Utilities|Struct|BreakItem_Structur (Variables|BP_NewDropItemActor_Master_C|GetItemData _asbp_new_drop_item_actor_master))) (.amount (Utilities|Struct|BreakItem_Structur (Variables|Default|GetItemData))))))
              (Variables|BP_NewDropItemActor_Master_C|SetItemData _asbp_new_drop_item_actor_master _structout)
              (Actor|DestroyActor)
              (goto _label Break))))))))

(event Custom|UpdateAmount
  (params (amount :type Integer))
  ;[1 1 1] Update amount when a player picks up not 100% of the amount (only for Ground-pickup)
  (Utilities|Struct|SetmembersinItem_Structur (Variables|Default|GetItemData) amount)
  (Utilities|FlowControl|Delay 0.2)
  (Class|BPInterfaceInventory|UpdateGroundItemListI(Message) (Game|GetGameMode)))

(event Custom|ShowNewInfoWidget
  (params (Show? :type Boolean))
  ;[1 1 1] Show new info pick up widget
  (Development|SetHiddeninGame (Variables|Default|GetWidget) (not Show?) false)
  (bind _aswb_new_info_pick_up (Utilities|Casting|CastToWB_NewInfoPickUp (UserInterface|GetUserWidgetObject (Variables|Default|GetWidget))))
  (Default|SetItemData _aswb_new_info_pick_up (Variables|Default|GetItemData)))

(event Custom|IncreaseAmountAnimation
  ;[1 1 1] Animation of the scale when the amount is increased
  (if (not (Variables|Default|GetinProgress))
    (Variables|Default|SetinProgress true)
    (bind _output_get (Variables|Default|SetstartScale (Variables|/Script/Engine.SceneComponent|GetRelativeScale3D (Variables|Default|GetStaticMesh1))))
    (Variables|Default|SetendScale (* _output_get 1.2))
    (bind _newtrack_0 (Timeline|Timeline_0 PlayFromStart)
      (:Update
        (Transformation|SetRelativeScale3D (Variables|Default|GetStaticMesh1) (Math|Vector|Lerp(Vector) (Variables|Default|GetstartScale) (Variables|Default|GetendScale) _newtrack_0)))
      (:Finished
        (Variables|Default|SetinProgress false)))))

(event Custom|Update
  (params (ItemData :type Item%20Structur%20Structure))
  ;[1 1 1] Setup item
  ;;[0.4766 1 0.7282] new in v 1.6
  (Variables|Default|SetItemData ItemData)
  (Game|Components|ProjectileMovement|SetVelocityinLocalSpace (Variables|Default|GetProjectileMovement) (Math|Vector|MakeVector (+ 6e+02 (Variables|Default|GetxVelocity)) 0.0 (Variables|Default|GetzVelocity)))
  (Components|Movement|SetUpdatedComponent (Variables|Default|GetProjectileMovement) (Variables|Default|GetitemCollisionMesh))
  (Components|StaticMesh|SetStaticMesh (Variables|Default|GetStaticMesh1) (.StaticMesh (Utilities|Struct|BreakItem_Structur (Variables|Default|GetItemData))))
  (Transformation|SetRelativeTransform (Variables|Default|GetStaticMesh1) (select (Variables|Default|GetSavePerformance) (Math|Transform|MakeTransform (- (.Location (Math|Transform|BreakTransform (.DropTransform (Utilities|Struct|BreakItem_Structur (Variables|Default|GetItemData))))) "0, 0,28.000000") (.Rotation (Math|Transform|BreakTransform (.DropTransform (Utilities|Struct|BreakItem_Structur (Variables|Default|GetItemData))))) (.Scale (Math|Transform|BreakTransform (.DropTransform (Utilities|Struct|BreakItem_Structur (Variables|Default|GetItemData)))))) (.DropTransform (Utilities|Struct|BreakItem_Structur (Variables|Default|GetItemData)))) false false)
  (Utilities|FlowControl|Delay 0.2)
  (Collision|SetCollisionEnabled (Variables|Default|GetRadiusForItemMerging) "QueryOnly"))

(event Custom|UpdateBackpackData
  (params (BackpackData :type Backpack%20Data%20Structure%20Structure))
  (bind _itemdata (Variables|Default|GetItemData))
  (bind (_staticmesh _droptransform) (Utilities|Struct|BreakItem_Structur _itemdata))
  (bind (_location _rotation _scale) (Math|Transform|BreakTransform _droptransform))
  ;[1 1 1] Setup item
  ;;[0.4766 1 0.7282] new in v 1.6
  (Variables|Default|SetBackpackData BackpackData)
  (Game|Components|ProjectileMovement|SetVelocityinLocalSpace (Variables|Default|GetProjectileMovement) (Math|Vector|MakeVector (+ 6e+02 (Variables|Default|GetxVelocity)) 0.0 (Variables|Default|GetzVelocity)))
  (Components|Movement|SetUpdatedComponent (Variables|Default|GetProjectileMovement) (Variables|Default|GetitemCollisionMesh))
  (Components|StaticMesh|SetStaticMesh (Variables|Default|GetStaticMesh1) _staticmesh)
  (Transformation|SetRelativeTransform (Variables|Default|GetStaticMesh1) (select (Variables|Default|GetSavePerformance) (Math|Transform|MakeTransform (- _location "0, 0,28.000000") _rotation _scale) _droptransform) false false)
  (Utilities|FlowControl|Delay 0.2)
  (Collision|SetCollisionEnabled (Variables|Default|GetRadiusForItemMerging) "QueryOnly"))

(event Custom|ShowActorWhenItsFullyLoaded
  ;[1 1 1] Spawn At Start
  ;;[1 1 1] This could take a bit of time on clients: Unhides item when it's allowed to interact
  ;;;[0.4766 1 0.7282] new in v 1.6 (BugFix)
  (Rendering|SetActorHiddenInGame false))

(event EventBeginPlay
  (bind _returnvalue (Utilities|Name|MakeLiteralName "NewRow"))
  (bind _id_atstart (Variables|Default|GetID_AtStart))
  (bind _projectilemovement (Variables|Default|GetProjectileMovement))
  (bind _id_atstart_2 (Variables|Default|GetID_AtStart))
  (bind _returnvalue_2 (== _id_atstart_2 0))
  (bind _returnvalue_3 (- _id_atstart 1))
  (bind _returnvalue_4 (Utilities|String|ToString(Integer) _returnvalue_3))
  (bind _returnvalue_5 (Utilities|String|Append "NewRow_" _returnvalue_4))
  (bind _returnvalue_6 (Utilities|String|StringToName _returnvalue_5))
  (bind _returnvalue_7 (select _returnvalue_2 _returnvalue _returnvalue_6))
  ;[1 1 1] Spawn At Start
  (if (Variables|Default|GetisLoadFromSaveGame?)
    (Components|Activation|Deactivate _projectilemovement)
    (Variables|/Script/Engine.MovementComponent|SetVelocity _projectilemovement "0, 0, 0")
    (Components|Activation|Activate (Variables|Default|GetProjectileMovement) false))
  (if (Variables|Default|GetSavePerformance)
    _
    (else
      (Utilities|FlowControl|Sequence
        (:then_0
          _)
        (:then_1
          ;[1 1 1] Hover and rotation animation
          (Components|MoveComponentTo (Variables|Default|GetSpringArm) (Math|Vector|MakeVector 0.0 0.0 (Math|Random|RandomFloatinRange 2.0 3.5)) "0, 0, 0" true true 2.0 true :!label _label)
          (Components|MoveComponentTo (Variables|Default|GetSpringArm) (Math|Vector|MakeVector 0.0 0.0 (Math|Random|RandomFloatinRange -2.0 -3.5)) "0, 0, 0" true true 2.0 true)
          (goto _label))
        (:then_2
          (Components|MoveComponentTo (Variables|Default|GetRotationAnimation_Scene) "0, 0, 0" (Math|Rotator|MakeRotator 0.0 0.0 (+ (.Yaw (Math|Rotator|BreakRotator (Variables|/Script/Engine.SceneComponent|GetRelativeRotation (Variables|Default|GetRotationAnimation_Scene)))) 16.0)) false false 2.0 true :!label _label_2)
          (goto _label_2)))))
  (if (Variables|Default|GetSpawnAtStart?)
    (Networking|SwitchHasAuthority
      (:Authority
        (CallFunction|ShowActorwhenItsFullyLoaded))
      (:Remote
        _))
    (bind _returnvalue_8 (Class|DataTableFunctionLibrary|DoesDataTableRowExist "/Game/AdvancedInventory/Item_Table.Item_Table" _returnvalue_7))
    (if _returnvalue_8
      (bind _returnvalue_9 (Utilities|GetDataTableRow "/Game/AdvancedInventory/Item_Table.Item_Table" _returnvalue_7)
        (:then
          (bind _output_get (Variables|Default|SetItemData _returnvalue_9))
          (if (<= (Utilities|Struct|BreakWeaponData_Structure (.WeaponData (Utilities|Struct|BreakItem_Structur _output_get))) 0)
            (Utilities|Struct|SetmembersinItem_Structur _output_get (Variables|Default|GetAmount_AtStart))
            (else
              (Variables|Default|SetRandomAmmo (Math|Random|RandomIntegerinRange (Variables|Default|GetRandomAmmoMin) (Variables|Default|GetRandomAmmoMax)))
              (bind _structout (Utilities|Struct|SetmembersinWeaponData_Structure (.WeaponData (Utilities|Struct|BreakItem_Structur _output_get)) (Variables|Default|GetRandomAmmo)))
              (Utilities|Struct|SetmembersinItem_Structur (Variables|Default|GetItemData) (Variables|Default|GetAmount_AtStart) _structout)))
          ;[1 1 1] Setup item
          (Components|Movement|SetUpdatedComponent (Variables|Default|GetProjectileMovement) (Variables|Default|GetitemCollisionMesh) :!label _label_3)
          (Components|StaticMesh|SetStaticMesh (Variables|Default|GetStaticMesh1) (.StaticMesh (Utilities|Struct|BreakItem_Structur (Variables|Default|GetItemData))))
          (Transformation|SetRelativeTransform (Variables|Default|GetStaticMesh1) (select (Variables|Default|GetSavePerformance) (Math|Transform|MakeTransform (- (.Location (Math|Transform|BreakTransform (.DropTransform (Utilities|Struct|BreakItem_Structur (Variables|Default|GetItemData))))) "0, 0,28.000000") (.Rotation (Math|Transform|BreakTransform (.DropTransform (Utilities|Struct|BreakItem_Structur (Variables|Default|GetItemData))))) (.Scale (Math|Transform|BreakTransform (.DropTransform (Utilities|Struct|BreakItem_Structur (Variables|Default|GetItemData)))))) (.DropTransform (Utilities|Struct|BreakItem_Structur (Variables|Default|GetItemData)))) false false)
          (Utilities|FlowControl|Delay 0.2)
          (Collision|SetCollisionEnabled (Variables|Default|GetRadiusForItemMerging) "QueryOnly"))))
    (else
      ;;[1 1 1] This could take a bit of time on clients: Unhides item when it's allowed to interact
      ;;;[0.4766 1 0.7282] new in v 1.6 (BugFix)
      (Rendering|SetActorHiddenInGame false)
      (if (Variables|Default|GetisLoadFromSaveGame?)
        _
        (else
          _))
      (Game|Components|ProjectileMovement|SetVelocityinLocalSpace (Variables|Default|GetProjectileMovement) (Math|Vector|MakeVector (+ 6e+02 (Variables|Default|GetxVelocity)) 0.0 (Variables|Default|GetzVelocity)))
      (goto _label_3))))

(fn ConstructionScript
  (bind _returnvalue (Utilities|Name|MakeLiteralName "NewRow"))
  (bind _id_atstart (Variables|Default|GetID_AtStart))
  (bind _staticmesh1 (Variables|Default|GetStaticMesh1))
  (bind _id_atstart_2 (Variables|Default|GetID_AtStart))
  (bind _returnvalue_2 (== _id_atstart_2 0))
  (bind _returnvalue_3 (- _id_atstart 1))
  (bind _returnvalue_4 (Utilities|String|ToString(Integer) _returnvalue_3))
  (bind _returnvalue_5 (Utilities|String|Append "NewRow_" _returnvalue_4))
  (bind _returnvalue_6 (Utilities|String|StringToName _returnvalue_5))
  (bind _returnvalue_7 (select _returnvalue_2 _returnvalue _returnvalue_6))
  ;[1 1 1] Setup item for editor
  (if (Variables|Default|GetSpawnAtStart?)
    (bind _returnvalue_8 (Class|DataTableFunctionLibrary|DoesDataTableRowExist "/Game/AdvancedInventory/Item_Table.Item_Table" _returnvalue_7))
    (if _returnvalue_8
      (bind _returnvalue_9 (Utilities|GetDataTableRow "/Game/AdvancedInventory/Item_Table.Item_Table" _returnvalue_7)
        (:then
          (Components|StaticMesh|SetStaticMesh _staticmesh1 (.StaticMesh (Utilities|Struct|BreakItem_Structur _returnvalue_9)))
          (Transformation|SetRelativeTransform _staticmesh1 (.DropTransform (Utilities|Struct|BreakItem_Structur _returnvalue_9)) false false)
          (Rendering|SetVisibility (Variables|Default|GetitemCollisionMesh) false false))))))

(fn ReactiveProjectileMovement
  (params (drop? :type Boolean))
  (bind _projectilemovement (Variables|Default|GetProjectileMovement))
  ;[1 1 1] Destroy the current ProjectileComponent and create a new one
  (Utilities|IsValid _projectilemovement
    (:Is%20Valid
      (Components|DestroyComponent _projectilemovement))
    (:Is%20Not%20Valid
      (Utilities|IsValid (Variables|Default|GetNewProjectileMovement)
        (:Is%20Valid
          (Components|DestroyComponent (Variables|Default|GetNewProjectileMovement)))
        (:Is%20Not%20Valid
          _))))
  (bind _returnvalue (AddComponent|AddProjectileMovementComponent))
  (bind _output_get (Variables|Default|SetNewProjectileMovement _returnvalue))
  (if drop?
    (Game|Components|ProjectileMovement|SetVelocityinLocalSpace _output_get (Math|Vector|MakeVector 1.5e+02 1.5e+02 3.5e+02))
    (Variables|/Script/Engine.ProjectileMovementComponent|SetbShouldBounce _output_get true)
    (Variables|/Script/Engine.ProjectileMovementComponent|SetFriction _output_get 0.2)
    (Variables|/Script/Engine.ProjectileMovementComponent|SetBounciness _output_get 0.2)))

(fn FindWayOut
  ;[1 1 1] The function checks all directions (not bottom). Distance of Linetrace 0: Linetrace is still in a Object of the type "PlacingObject"   I   Distance of the Linetrace >0: Linetrace doesn't collide with a PlacingObject -> ReturnsLocation
  (Math|Integer|IncrementInt (LocalVariables|Getcount2) :!label _label
    (:%20%20
      (for _index (range 0 4)
        (bind _output_get (LocalVariables|SetcheckDirection (Utilities|Select :Index _index :Option%200 "0, 0,50.000000" :Option%201 "0,-50.000000, 0" :Option%202 "0,50.000000, 0" :Option%203 "50.000000, 0, 0" :Option%204 "-50.000000, 0, 0")))
        (bind _outhit (Collision|LineTraceByChannel (+ (* _output_get (+ (LocalVariables|Getcount2) 1)) (Transformation|GetActorLocation) "0,0.000000,15.000000") (+ (* _output_get (LocalVariables|Getcount2)) (Transformation|GetActorLocation) "0,0.000000,15.000000") "TraceTypeQuery3" false 0 "None"))
        (if (not (== (.Distance (Collision|BreakHitResult _outhit)) 0.0))
          (return (+ (.Location (Collision|BreakHitResult _outhit)) (select (== _index 0) "0, 0, 0" (LocalVariables|GetcheckDirection))) (not (== _index 0)))))
      (goto _label))))