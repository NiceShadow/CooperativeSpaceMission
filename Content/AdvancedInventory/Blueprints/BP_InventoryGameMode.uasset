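; Game mode for the inventory system, acting as the hub that syncs chests, campfire cooking, shops, ground items and chat across players.
; PostLogin collects controllers in AllPCs, and interface events relay updates to them, filtering cooking UI by each player's open chest.
; Chest updates, buying, selling and campfire toggling are delegated to BPGamemodeComponent.
; Save-load events restore chests and shops behind already-loaded checks, and destroy then respawn ground items.
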(event Custom|AddTextMessage
  (params (PC :type Player%20Controller%20Object%20Reference) (Message :type String) (ServerMessage :type Boolean))
  (for _array_element (Variables|Default|GetAll%20PCs)
    (bind _asbp_inventory_player_controller (Utilities|Casting|CastToBP_InventoryPlayerController _array_element))
    (Default|AddChatMessage _asbp_inventory_player_controller (Class|AdvancedSessionsLibrary|GetPlayerName PC) Message ServerMessage)))

(event EventPostLogin
  (params (NewPlayer :type Player%20Controller%20Object%20Reference))
  ;[1 1 1] Creates an array which contains all players on the server  (connect with "EventOnPostLogin")
  (Utilities|Array|Add (Variables|Default|GetAll%20PCs) NewPlayer))

(event EventUpdateGroundItemListI
  ;[1 1 1] Update GroundItemList on each player
  (for _array_element (Variables|Default|GetAll%20PCs)
    (Class|BPInterfaceInventory|UpdateGroundItemListI(Message) _array_element)))

(event EventBuyProductI
  (params (buyData :type Buy%20Product%20Structure%20Structure))
  ;[1 1 1] Buy product in shop
  (Default|BuyProduct (Variables|Default|GetBP_GamemodeComponent) buyData (Variables|Default|GetAll%20PCs)))

(event EventLoadShopsI
  (params (ShopsData :type Array%20of%20Shop%20Save%20Structure%20Structures))
  ;[1 1 1] Recieve data from save game and update all shops
  (if (not (Variables|Default|GetAlreadyLoadedShops?))
    (for _array_element ShopsData
      (Default|UpdateWholeShopData (.Shop (Utilities|Struct|BreakShopSave_Structure _array_element)) (.Products (Utilities|Struct|BreakShopSave_Structure _array_element))))))

(event EventToggleCampfireFireI
  (params (turnOn :type Boolean) (CestRef :type BP%20Chest%20Object%20Reference) (fromPC :type Player%20Controller%20Object%20Reference))
  (Default|ToggleCampfire (Variables|Default|GetBP_GamemodeComponent) turnOn CestRef (Variables|Default|GetAll%20PCs) fromPC))

(event EventTurnOffCampfireFireUII
  (params (Chest :type BP%20Chest%20Object%20Reference))
  (Utilities|IsValid Chest
    (:Is%20Valid
      (for _array_element (Variables|Default|GetAll%20PCs)
        (bind _chest (Class|BPInterfaceInventory|GetCurrentChestRefI(Message) _array_element))
        (if (== _chest Chest)
          (Class|BPInterfaceInventory|ToggleCampfireFireActorI(Message) _array_element false))))))

(event EventDestroyActorI
  (params (Actor :type Actor%20Object%20Reference))
  ;[1 1 1] Destroy an actor from the GameMode
  (Actor|DestroyActor Actor))

(event EventUpdateAmountOfASpecificItemI
  (params (Actor :type Actor%20Object%20Reference) (Amount :type Integer))
  ;[1 1 1] Update amount of a specific item
  (if (== (Utilities|GetClass Actor) "/Game/AdvancedInventory/Blueprints/BP_NewDropItemActor_Master.BP_NewDropItemActor_Master_C")
    (bind _asbp_new_drop_item_actor_master (Utilities|Casting|CastToBP_NewDropItemActor_Master Actor))
    (Default|UpdateAmount _asbp_new_drop_item_actor_master Amount)
    (else
      (bind _asbp_old_drop_item_actor_master (Utilities|Casting|CastToBP_OldDropItemActor_Master Actor))
      (Default|UpdateAmount _asbp_old_drop_item_actor_master Amount))))

(event EventUpdateChestGameModeI
  (params (UpdateChestData :type Update%20Chest%20Structure%20Structure))
  ;[1 1 1] UpdateChest
  (Default|UpdateChestFunction (Variables|Default|GetBP_GamemodeComponent) UpdateChestData (Variables|Default|GetAll%20PCs)))

(event EventLoadChestSlotsI
  (params (ChestSaveData :type Array%20of%20Chest%20Save%20Structure%20Structures) (OverwriteIfAlreadyLoaded? :type Boolean))
  ;[1 1 1] SaveGame: Load chest slots and call update for each player
  (if OverwriteIfAlreadyLoaded?
    (for _array_element ChestSaveData :!label _label
      (Utilities|IsValid (.Chest (Utilities|Struct|BreakChestSave_Structure _array_element))
        (:Is%20Valid
          (Default|UpdateWholeChestData (.Chest (Utilities|Struct|BreakChestSave_Structure _array_element)) (.Visibility_items (Utilities|Struct|BreakChestSave_Structure _array_element)) (.Data_items (Utilities|Struct|BreakChestSave_Structure _array_element)) (.BackPackData_items (Utilities|Struct|BreakChestSave_Structure _array_element))))))
    (Variables|Default|SetAlreadyLoadedChestSlots? true)
    (for _array_element_2 (Variables|Default|GetAll%20PCs)
      (Class|BPInterfaceInventory|UpdateOwnChestUII(Message) _array_element_2))
    (elif (not (Variables|Default|GetAlreadyLoadedChestSlots?))
      (goto _label))))

(event EventCheckCookingI
  (params (ChestRef :type BP%20Chest%20Object%20Reference) (ResetSecondsCooked :type Boolean) (ResetAtSlot :type Integer))
  ;[1 1 1] Update campfire UI
  (Utilities|IsValid ChestRef
    (:Is%20Valid
      (Default|CheckCooking ChestRef ResetSecondsCooked ResetAtSlot))))

(event EventUpdateCookingUII
  (params (Chest :type BP%20Chest%20Object%20Reference) (Percent :type Array%20of%20Integers) (RemoveFuelItem :type Boolean) (FuelReduceID :type Integer) (DecreaseCookingItemAndAdd :type Array%20of%20Booleans) (AddSlot :type Array%20of%20Integers) (AddID :type Array%20of%20Integers) (AmountsToAdd :type Array%20of%20Integers))
  ;[1 1 1] Update campfire UI
  (Utilities|IsValid Chest
    (:Is%20Valid
      (for _array_element (Variables|Default|GetAll%20PCs)
        (bind _chest (Class|BPInterfaceInventory|GetCurrentChestRefI(Message) _array_element))
        (if (== _chest Chest)
          (Class|BPInterfaceInventory|UpdateOwnCookingUII(Message) _array_element Percent RemoveFuelItem FuelReduceID DecreaseCookingItemAndAdd AddSlot AddID AmountsToAdd))))))

(event EventLoadGroundItemsI
  (params (items :type Array%20of%20Ground%20Item%20Save%20Structure%20Structures))
  ;[1 1 1] Load Ground item actors by destroying the existing ones and spawn new items based on save game
  (bind _outactors (Actor|GetAllActorsOfClass "/Game/AdvancedInventory/Blueprints/BP_NewDropItemActor_Master.BP_NewDropItemActor_Master_C"))
  (for _array_element _outactors
    (Actor|DestroyActor _array_element))
  (for _array_element_2 items
    (Game|SpawnActorfromClass "/Game/AdvancedInventory/Blueprints/BP_NewDropItemActor_Master.BP_NewDropItemActor_Master_C" (Math|Transform|MakeTransform (.location (Utilities|Struct|BreakGroundItemSave_Structure _array_element_2))) "Undefined" 0 0.0 (.itemdata (Utilities|Struct|BreakGroundItemSave_Structure _array_element_2)) 0.0 0.0 false 0 1 (.backpackData (Utilities|Struct|BreakGroundItemSave_Structure _array_element_2)) true false 0 0 0)))

(event EventSellProductI
  (params (product%20data :type Product%20Structure%20Structure))
  ;[1 1 1] Sell product in shop
  (Default|UpdateShop (Variables|Default|GetBP_GamemodeComponent) product%20data (Variables|Default|GetAll%20PCs)))

(fn ConstructionScript)

(fn GetAutoPickUpModeI
  (return false))

(fn GetCurrentChestRefI
  (return 0))

(fn GetCurrentShopRefI
  (return 0))

(fn GetCurrentSlotI
  (return 0))

(fn GetGroundRadiusI
  (return 0))

(fn GetInventoryRefI
  (return 0))

(fn GetMoneyI
  (params (inCurrency :type Currencies_Enumeration%20Enum :default "NewEnumerator0"))
  (return 0))

(fn GetUIRefI
  (return 0))