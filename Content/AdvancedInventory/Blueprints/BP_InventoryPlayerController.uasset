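; Player controller for a multiplayer inventory game, covering items, chests, shops, quests, chat, pausing and session invites.
; Input and interface events mostly forward to BPPlayercontrollerComponent, while quest events call server functions on CQuestComponent.
; BeginPlay builds the local quest UI, sets up the component, then after a delay loads data and starts a looping autosave.
; Slot loading requires a valid session code; chests, ground items and shops auto-save and auto-load only on the server.
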(event Custom|SetPlayerLocServer
  (params (Target :type Actor%20Object%20Reference) (NewLocation :type Vector))
  (CallFunction|SetPlayerLocMulticast Target NewLocation))

(event Custom|LoadEverything
  (bind _bp_playercontrollercomponent (Variables|Default|GetBP_PlayercontrollerComponent))
  ;[1 1 1] Save & Load System
  (bind _valid (Default|CorrectSessionCode (Variables|Default|GetBP_PlayercontrollerComponent)))
  (if _valid
    (Default|LoadSlots (Variables|Default|GetBP_PlayercontrollerComponent))
    (if (Networking|IsServer)
      (Default|LoadChestSlots _bp_playercontrollercomponent false)
      (Default|LoadGroundItems _bp_playercontrollercomponent)
      (Default|LoadShops _bp_playercontrollercomponent))))

(event Custom|SendChatMessage
  (params (PC :type Player%20Controller%20Object%20Reference) (Message :type String))
  ;[1 1 1] Chat system
  (bind _asbp_inventory_game_mode (Utilities|Casting|CastToBP_InventoryGameMode (Game|GetGameMode)))
  (Default|AddTextMessage _asbp_inventory_game_mode PC Message false))

(event Custom|AddChatMessage
  (params (Name :type String) (Message :type String) (ServerMessage :type Boolean))
  ;[1 1 1] Chat system
  (bind _ui_ref (Class|BPInterfaceInventory|GetUIRefI(Message) (HUD|GetHUD (Game|GetPlayerController 0))))
  (Utilities|IsValid _ui_ref
    (:Is%20Valid
      (Default|AddMessage (Variables|/Game/AdvancedInventory/Widgets/WB_UI.WB_UI_C|GetWB_GameChatWindow _ui_ref) Name Message ServerMessage))))

(event Custom|SetPlayerLocMulticast
  (params (Target :type Actor%20Object%20Reference) (NewLocation :type Vector))
  (Transformation|SetActorLocation Target NewLocation false false))

(event Custom|SaveNow
  ;[1 1 1] Save & Load System
  (CallFunction|SaveEverything))

(event Custom|SetChatActive
  (params (Active :type Boolean))
  ;[1 1 1] Chat system
  (Default|SetChatActive (Variables|Default|GetBP_PlayercontrollerComponent) Active))

(event Custom|InvitePlayer
  ;[1 1 1] Invite Player in game
  (bind _ui_ref (Class|BPInterfaceInventory|GetUIRefI(Message) (HUD|GetHUD (Game|GetPlayerController 0))))
  (if (Variables|/Game/Server/Widgets/WB_InvitePlayer.WB_InvitePlayer_C|Getshowing (Variables|/Game/AdvancedInventory/Widgets/WB_UI.WB_UI_C|GetWB_InvitePlayer _ui_ref))
    (Default|HideNow (Variables|/Game/AdvancedInventory/Widgets/WB_UI.WB_UI_C|GetWB_InvitePlayer _ui_ref))
    (Class|AdvancedFriendsLibrary|SendSessionInvitetoFriend (Game|GetPlayerController 0) (Variables|/Game/Server/Widgets/WB_InvitePlayer.WB_InvitePlayer_C|GetCurrentPlayer (Variables|/Game/AdvancedInventory/Widgets/WB_UI.WB_UI_C|GetWB_InvitePlayer _ui_ref))
      (:OnSuccess
        (Development|PrintString "SendInvite" true true "(R=0.093621,G=0.348958,B=0.000000,A=1.000000)"))
      (:OnFailure
        (Development|PrintString "FailedToInvite" true true "(R=1.000000,G=0.015526,B=0.000000,A=1.000000)")))))

(event Custom|SetFocusedCraftingBench
  (params (FocusedCraftingBench :type BP%20Crafting%20Bench%20Object%20Reference))
  (Variables|/Game/AdvancedInventory/Blueprints/BP_PlayercontrollerComponent.BP_PlayercontrollerComponent_C|SetFocusedCraftingBench (Variables|Default|GetBP_PlayercontrollerComponent) FocusedCraftingBench))

(event Custom|SaveEverything
  (bind _bp_playercontrollercomponent (Variables|Default|GetBP_PlayercontrollerComponent))
  ;[1 1 1] Save & Load System
  (Default|SaveSlots (Variables|Default|GetBP_PlayercontrollerComponent))
  (if (Networking|IsServer)
    (Default|SaveChestSlots _bp_playercontrollercomponent)
    (Default|SaveGroundItems _bp_playercontrollercomponent)
    (Default|SaveShops _bp_playercontrollercomponent)
    (bind _asfriends_intance (Utilities|Casting|CastToFriendsIntance (Game|GetGameInstance)))
    (Default|UpdateCurrentSlotDate _asfriends_intance)))

(event Custom|AutoSave
  ;[1 1 1] Save & Load System
  (Utilities|Time|SetTimerbyEvent (delegate Custom|SaveNow) 5.0 true -4.0))

(event Custom|CustomEvent
  ;[1 1 1] Quest stuff
  ;;[0 0.7084 1] Create Quest Interface and add it to viewport
  (|CallParentFunction)
  (if (Pawn|IsLocalController)
    (CallFunction|ConstructQuestUI)))

(event EventAbortQuest
  (params (QuestID :type Name :default "None"))
  ;[1 1 1] Quest stuff
  ;;[1 0 0.1152] SERVER // Manage Quest Events
  (Default|SERVER//RemoveQuest (Variables|Default|GetC_QuestComponent) QuestID))

(event EventTrackQuest
  (params (QuestID :type Name :default "None"))
  ;[1 1 1] Quest stuff
  ;;[1 0 0.1152] SERVER // Manage Quest Events
  (Default|SERVER//TrackQuest (Variables|Default|GetC_QuestComponent) QuestID))

(event EventUpdateOwnChestUII
  ;[1 1 1] update UI
  (Default|ReloadChestUIServer (Variables|Default|GetBP_PlayercontrollerComponent)))

(event EventUpdateChestI
  (params (UpdateChestData :type Update%20Chest%20Structure%20Structure))
  ;[1 1 1] Chest replication
  (Default|UpdateChest (Variables|Default|GetBP_PlayercontrollerComponent) UpdateChestData))

(event EventUpdateItemAmountI
  (params (Amount :type Integer) (Actor :type Actor%20Object%20Reference))
  ;[1 1 1] BP_NewDropItemActor_Master / BP_OldDropItemActor_Master
  (Default|UpdateItemAmount (Variables|Default|GetBP_PlayercontrollerComponent) Amount Actor))

(event EventAddQuestTaskAmount
  (params (QuestTaskID :type Name :default "None") (Amount :type Integer))
  ;[1 1 1] Quest stuff
  ;;[1 0 0.1152] SERVER // Manage Quest Events
  (Default|SERVER//AddQuestTaskAmount (Variables|Default|GetC_QuestComponent) QuestTaskID Amount))

(event EventSetAutoPickRadiusandGroundRadiusI
  (params (AutoPick :type Sphere%20Component%20Object%20Reference) (Ground :type Sphere%20Component%20Object%20Reference))
  ;[1 1 1] Setup and create references
  (Utilities|Struct|SetmembersinPlayercontrollerVariables_Structure (Variables|/Game/AdvancedInventory/Blueprints/BP_PlayercontrollerComponent.BP_PlayercontrollerComponent_C|GetpcMasterVariable (Variables|Default|GetBP_PlayercontrollerComponent)) AutoPick Ground))

(event EventUpdateElementinChestUII
  (params (UpdateChestData :type Update%20Chest%20Structure%20Structure))
  ;[1 1 1] Chest replication
  (Default|UpdateElementinChestUI (Variables|Default|GetBP_PlayercontrollerComponent) UpdateChestData))

(event EventEnableDragOPI
  (params (IsEnabled :type Boolean) (ItemData :type Item%20Structur%20Structure) (UpdateAmountBeforeDragOF_Item :type Integer))
  ;[1 1 1] Chest replication
  (Default|EnableDragOP (Variables|Default|GetBP_PlayercontrollerComponent) IsEnabled ItemData UpdateAmountBeforeDragOF_Item))

(event EventUpdateOtherItemI
  (params (ItemData :type Item%20Structur%20Structure) (BackpackData :type Backpack%20Data%20Structure%20Structure))
  ;[1 1 1] Chest replication
  (Default|UpdateOtherItem (Variables|Default|GetBP_PlayercontrollerComponent) ItemData BackpackData))

(event EventAddItemtoChestUII
  (params (ID :type Integer) (Amount :type Integer) (ShiftFromChest? :type Boolean))
  ;[1 1 1] Chest replication
  (Default|AddItemtoChestUI (Variables|Default|GetBP_PlayercontrollerComponent) ID Amount ShiftFromChest?))

(event EventAddItemI
  (params (ID_OfItem :type Integer) (Amount :type Integer) (Data :type Item%20Structur%20Structure) (TransferWholeItemData :type Boolean) (IsBackpack? :type Boolean) (BackpackData :type Backpack%20Data%20Structure%20Structure))
  ;[1 1 1] Add item
  (Default|AddItem (Variables|Default|GetBP_PlayercontrollerComponent) ID_OfItem Amount Data TransferWholeItemData IsBackpack? BackpackData))

(event EventAcceptQuest
  (params (QuestID :type Name :default "None"))
  ;[1 1 1] Quest stuff
  ;;[1 0 0.1152] SERVER // Manage Quest Events
  (Default|SERVER//AcceptQuest (Variables|Default|GetC_QuestComponent) QuestID))

(event EventSetIsinRadiusOfChestI
  (params (inRadius? :type Boolean))
  ;[1 1 1] other
  (Utilities|Struct|SetmembersinPlayercontrollerVariables_Structure (Variables|/Game/AdvancedInventory/Blueprints/BP_PlayercontrollerComponent.BP_PlayercontrollerComponent_C|GetpcMasterVariable (Variables|Default|GetBP_PlayercontrollerComponent)) inRadius?))

(event EventDestroyActorI
  (params (Actor :type Actor%20Object%20Reference))
  ;[1 1 1] BP_NewDropItemActor_Master / BP_OldDropItemActor_Master
  (Default|DestroyActorfromPC (Variables|Default|GetBP_PlayercontrollerComponent) Actor))

(event EventFinishedConsumeItemI
  ;[1 1 1] Mouse- and keyboardinput
  ;;[1 1 1] Equip and consume items from hotbar
  (Default|FinishedConsumeItem (Variables|Default|GetBP_PlayercontrollerComponent)))

(event EventAddItemsInstantI
  (params (itemsToAdd :type Array%20of%20Item%20Structur%20Structures))
  ;[1 1 1] Add items instantly to the inventory if the player opens a chest that has this function
  (Default|AddItemsInstant (Variables|Default|GetBP_PlayercontrollerComponent) itemsToAdd))

(event EventCheckCookingI
  (params (ChestRef :type BP%20Chest%20Object%20Reference) (ResetSecondsCooked :type Boolean) (ResetAtSlot :type Integer))
  ;[1 1 1] Update campfire UI
  (Default|CheckCooking (Variables|Default|GetBP_PlayercontrollerComponent) ResetSecondsCooked ResetAtSlot))

(event EventSetFocusedShopI
  (params (BP_ShopRef :type BP%20Shop%20Object%20Reference))
  ;[1 1 1] other
  ;;[0.4766 1 0.7282] new in v 1.6
  (Utilities|Struct|SetmembersinPlayercontrollerVariables_Structure (Variables|/Game/AdvancedInventory/Blueprints/BP_PlayercontrollerComponent.BP_PlayercontrollerComponent_C|GetpcMasterVariable (Variables|Default|GetBP_PlayercontrollerComponent)) BP_ShopRef))

(event EventUpdateOwnCookingUII
  (params (Percent :type Array%20of%20Integers) (RemoveFuelItem :type Boolean) (FuelReduceID :type Integer) (DecreaseCookingItemAndAdd :type Array%20of%20Booleans) (AddSlot :type Array%20of%20Integers) (AddID :type Array%20of%20Integers) (AddAmount :type Array%20of%20Integers))
  ;[1 1 1] Update campfire UI
  (Default|UpdateOwnCookingUI (Variables|Default|GetBP_PlayercontrollerComponent) Percent RemoveFuelItem FuelReduceID DecreaseCookingItemAndAdd AddSlot AddID AddAmount))

(event EventSellProductI
  (params (product%20data :type Product%20Structure%20Structure))
  ;[1 1 1] Shop replication
  (bind _structout (Utilities|Struct|SetmembersinProduct_Structure product%20data self))
  (Default|SellProduct (Variables|Default|GetBP_PlayercontrollerComponent) _structout))

(event EventSetShopRefI
  (params (CurrentShopRef :type BP%20Shop%20Object%20Reference))
  ;[1 1 1] Shop replication
  (Default|SetCurrentShopRef (Variables|Default|GetBP_PlayercontrollerComponent) CurrentShopRef))

(event EventUpdateShopUII
  (params (ShopRef :type BP%20Shop%20Object%20Reference) (products :type Array%20of%20Product%20Structure%20Structures))
  ;[1 1 1] Shop replication
  (Default|UpdateShopUIClient (Variables|Default|GetBP_PlayercontrollerComponent) ShopRef products))

(event EventCompleteQuest
  (params (Quest%20ID :type Name :default "None"))
  ;[1 1 1] Quest stuff
  ;;[1 0 0.1152] SERVER // Manage Quest Events
  (Default|SERVER//CompleteQuest (Variables|Default|GetC_QuestComponent) Quest%20ID))

(event EventBuyProductI
  (params (buyData :type Buy%20Product%20Structure%20Structure))
  ;[1 1 1] Shop replication
  (Default|BuyProduct (Variables|Default|GetBP_PlayercontrollerComponent) buyData))

(event EventAddProducttoPlayerI
  (params (itemToAdd :type Item%20Structur%20Structure) (price :type Integer))
  ;[1 1 1] Shop replication
  (Default|AddProducttoPlayer (Variables|Default|GetBP_PlayercontrollerComponent) itemToAdd))

(event EventAddMoneyAfterSelltoPlayerI
  (params (Money :type Integer))
  ;[1 1 1] Trade
  ;;[1 1 1] Money
  (Default|AddMoneyAfterSell (Variables|Default|GetBP_PlayercontrollerComponent) Money "NewEnumerator0"))

(event EventToggleCampfireFireI
  (params (turnOn :type Boolean) (CestRef :type BP%20Chest%20Object%20Reference) (fromPC :type Player%20Controller%20Object%20Reference))
  (Default|ToggleCampfire (Variables|Default|GetBP_PlayercontrollerComponent) turnOn CestRef fromPC))

(event EventUpdateMoneyI
  (params (newMoney :type Integer) (Currency :type Currencies_Enumeration%20Enum :default "NewEnumerator0"))
  ;[1 1 1] Trade
  ;;[1 1 1] Money
  (Default|UpdateMoney (Variables|Default|GetBP_PlayercontrollerComponent) newMoney Currency))

(event EventAddMoneytoPlayerI
  (params (MoneyToAdd :type Integer) (Currency :type Currencies_Enumeration%20Enum :default "NewEnumerator0"))
  ;[1 1 1] Trade
  ;;[1 1 1] Money
  (Default|AddMoneytoPlayer (Variables|Default|GetBP_PlayercontrollerComponent) MoneyToAdd Currency))

(event EventToggleCampfireFireActorI
  (params (TurnOn :type Boolean))
  (Default|ToggleCampfireFireUI (Variables|Default|GetBP_PlayercontrollerComponent) TurnOn))

(event EventUpdateEquipSlotI
  (params (EquipSlot :type Object%20Object%20Reference) (fromEquipSlot? :type Boolean) (itemRefOnlyForEquipSlot :type WB%20Item%20Object%20Reference))
  ;[1 1 1] Update for character
  (Default|(Un)EquipItemfromEquipSlot (Variables|Default|GetBP_PlayercontrollerComponent) EquipSlot fromEquipSlot? itemRefOnlyForEquipSlot))

(event EventDropItemI
  (params (Data :type Item%20Structur%20Structure) (BackpackData :type Backpack%20Data%20Structure%20Structure))
  ;[1 1 1] BP_NewDropItemActor_Master / BP_OldDropItemActor_Master
  (Default|DropEvent (Variables|Default|GetBP_PlayercontrollerComponent) Data BackpackData))

(event EventBeginPlay
  ;[1 1 1] Quest stuff
  (if (Pawn|IsLocalController)
    (CallFunction|ConstructQuestUI))
  ;[1 1 1] Setup and create references
  ;;[1 1 0 1 20] NOTE: You can't have 2 'EventBeginPlay' at the same time in one blueprint.
  ;; If you copy this BP make sure to add 'Setup' to your existing
  ;; 'EventBeginPlay' (if you have one)
  (Default|Setup (Variables|Default|GetBP_PlayercontrollerComponent))
  (Input|SetInputModeGameOnly self)
  (Utilities|FlowControl|Delay 1.0)
  (CallFunction|LoadEverything)
  (CallFunction|AutoSave))

(event EventUpdateHotbarSlotsI
  ;[1 1 1] Update for character
  (Default|GetNewSlotDataandCallUpdateforCharcater (Variables|Default|GetBP_PlayercontrollerComponent)))

(event EventSetFocusedChestI
  (params (FocusedChestRef :type BP%20Chest%20Object%20Reference))
  ;[1 1 1] other
  (Utilities|Struct|SetmembersinPlayercontrollerVariables_Structure (Variables|/Game/AdvancedInventory/Blueprints/BP_PlayercontrollerComponent.BP_PlayercontrollerComponent_C|GetpcMasterVariable (Variables|Default|GetBP_PlayercontrollerComponent)) FocusedChestRef 0.0))

(event EventSetInventoryComponentRefI
  (params (InventoryComponent :type BP%20Inventory%20Componenent%20Object%20Reference))
  ;[1 1 1] Setup and create references
  (Utilities|Struct|SetmembersinPlayercontrollerVariables_Structure (Variables|/Game/AdvancedInventory/Blueprints/BP_PlayercontrollerComponent.BP_PlayercontrollerComponent_C|GetpcMasterVariable (Variables|Default|GetBP_PlayercontrollerComponent)) InventoryComponent))

(event EventUpdateGroundItemListI
  ;[1 1 1] update UI
  (Default|UpdateGroundItemListPC (Variables|Default|GetBP_PlayercontrollerComponent)))

(event EventCancelShiftItemI
  ;[1 1 1] Chest replication
  (Default|CancelShiftItem (Variables|Default|GetBP_PlayercontrollerComponent)))

(event EventSetCurrentDragOPRefI
  (params (DragOP :type Drag%20Drop%20Operation%20Object%20Reference) (CurrentItem_Ref :type WB%20Item%20Object%20Reference) (ChestSlotIndex :type Integer))
  ;[1 1 1] Chest replication
  (Default|SetCurrentDragOPRef (Variables|Default|GetBP_PlayercontrollerComponent) DragOP CurrentItem_Ref ChestSlotIndex))

(event EventSetCurrentDragOPOtherRefI
  (params (DragOP_Other :type WB%20Item%20Object%20Reference))
  ;[1 1 1] Chest replication
  (Default|SetCurrentDragOPOtherRef (Variables|Default|GetBP_PlayercontrollerComponent) DragOP_Other))

(event EventSetChestRefI
  (params (CurrentChestRef :type BP%20Chest%20Object%20Reference))
  ;[1 1 1] Chest replication
  (Default|SetChestRef (Variables|Default|GetBP_PlayercontrollerComponent) CurrentChestRef))

(event Input|ActionEvents|InputActionInteractionChestOrShop
  (params (Key :type Key%20Structure :default "None"))
  (bind _bp_playercontrollercomponent (Variables|Default|GetBP_PlayercontrollerComponent))
  ;[1 1 1] other
  (:Pressed
    (Default|OpenChest _bp_playercontrollercomponent))
  (:Released
    (Default|StopOpenChest _bp_playercontrollercomponent)))

(event Input|ActionEvents|InputActionQuickEquipItem
  (params (Key :type Key%20Structure :default "None"))
  ;[1 1 1] Mouse- and keyboardinput
  ;;[1 1 1] Equip and consume items from hotbar
  (:Pressed
    (Default|EquiponRightClick (Variables|Default|GetBP_PlayercontrollerComponent))))

(event Input|ActionEvents|InputActionConsumeItem
  (params (Key :type Key%20Structure :default "None"))
  (bind _returnvalue (Game|GetPlayerCharacter 0))
  (bind _bp_playercontrollercomponent (Variables|Default|GetBP_PlayercontrollerComponent))
  ;[1 1 1] Mouse- and keyboardinput
  ;;[1 1 1] Equip and consume items from hotbar
  (:Pressed
    (Default|ConsumeItem _bp_playercontrollercomponent)
    (if (not (Utilities|Struct|BreakPlayercontrollerVariables_Structure (Variables|/Game/AdvancedInventory/Blueprints/BP_PlayercontrollerComponent.BP_PlayercontrollerComponent_C|GetpcMasterVariable (Variables|Default|GetBP_PlayercontrollerComponent))))
      (Class|BPCharacterInterface|AimCharacter(Message) _returnvalue true)))
  (:Released
    (Default|CancelConsumeItem _bp_playercontrollercomponent)
    (Class|BPCharacterInterface|AimCharacter(Message) _returnvalue false)))

(event Input|ActionEvents|InputActionInvitePlayer
  (params (Key :type Key%20Structure :default "None"))
  ;[1 1 1] Invite Player in game
  (:Pressed
    (CallFunction|InvitePlayer)))

(event Input|ActionEvents|InputActionPause
  (params (Key :type Key%20Structure :default "None"))
  (bind _bp_playercontrollercomponent (Variables|Default|GetBP_PlayercontrollerComponent))
  ;[1 1 1] Pause Game
  (:Pressed
    (if (== Key "Escape")
      (bind _inventory (Class|BPInterfaceInventory|GetInventoryRefI(Message) (HUD|GetHUD (Game|GetPlayerController 0))))
      (if (Widget|IsVisible (Variables|/Game/AdvancedInventory/Widgets/WB_Inventory.WB_Inventory_C|GetChestUI _inventory))
        (Default|Hide (Variables|/Game/AdvancedInventory/Widgets/WB_Inventory.WB_Inventory_C|GetChestUI _inventory))
        (Default|ShowInventory _bp_playercontrollercomponent false true)
        (elif (Variables|/Game/AdvancedInventory/Widgets/WB_Inventory.WB_Inventory_C|GetMainInventoryVisible? _inventory)
          (Default|ShowInventory _bp_playercontrollercomponent false false)
          (else
            (bind _ui_ref (Class|BPInterfaceInventory|GetUIRefI(Message) (HUD|GetHUD) :!label _label))
            (Default|TogglePause (Variables|/Game/AdvancedInventory/Widgets/WB_UI.WB_UI_C|GetWB_PauseMenu _ui_ref)))))
      (else
        (goto _label)))))

(event Input|KeyboardEvents|I
  (params (Key :type Key%20Structure :default "None"))
  ;[1 1 1] Setup and create references
  ;;[1 1 1] Show and hide the main inventory
  (:Pressed
    (Default|ToggleInventoryVisibility (Variables|Default|GetBP_PlayercontrollerComponent))))

(event Input|KeyboardEvents|P
  (params (Key :type Key%20Structure :default "None"))
  ;[1 1 1] Pause Game
  (:Pressed
    (bind _ui_ref (Class|BPInterfaceInventory|GetUIRefI(Message) (HUD|GetHUD)))
    (Default|TogglePause (Variables|/Game/AdvancedInventory/Widgets/WB_UI.WB_UI_C|GetWB_PauseMenu _ui_ref))))

(event Input|KeyboardEvents|7
  (params (Key :type Key%20Structure :default "None"))
  ;[1 1 1] Mouse- and keyboardinput
  (:Pressed
    (Default|ChangeSlot (Variables|Default|GetBP_PlayercontrollerComponent) false false 6)))

(event Input|KeyboardEvents|8
  (params (Key :type Key%20Structure :default "None"))
  ;[1 1 1] Mouse- and keyboardinput
  (:Pressed
    (Default|ChangeSlot (Variables|Default|GetBP_PlayercontrollerComponent) false false 7)))

(event Input|KeyboardEvents|9
  (params (Key :type Key%20Structure :default "None"))
  ;[1 1 1] Mouse- and keyboardinput
  (:Pressed
    (Default|ChangeSlot (Variables|Default|GetBP_PlayercontrollerComponent) false false 8)))

(event Input|MouseEvents|MouseWheelUp
  (params (Key :type Key%20Structure :default "None"))
  ;[1 1 1] Mouse- and keyboardinput
  (:Pressed
    (Default|ChangeSlot (Variables|Default|GetBP_PlayercontrollerComponent) true false)))

(event Input|KeyboardEvents|CtrlL
  (params (Key :type Key%20Structure :default "None"))
  (bind _bp_playercontrollercomponent (Variables|Default|GetBP_PlayercontrollerComponent))
  ;[1 1 1] Mouse- and keyboardinput
  ;;[1 1 1] Save & Load control
  (:Pressed
    (Default|LoadChestSlots _bp_playercontrollercomponent false)
    (Default|LoadGroundItems _bp_playercontrollercomponent)
    (Default|LoadShops _bp_playercontrollercomponent)))

(event Input|KeyboardEvents|CtrlO
  (params (Key :type Key%20Structure :default "None"))
  (bind _bp_playercontrollercomponent (Variables|Default|GetBP_PlayercontrollerComponent))
  ;[1 1 1] Mouse- and keyboardinput
  ;;[1 1 1] Save & Load control
  (:Pressed
    (Default|SaveChestSlots _bp_playercontrollercomponent)
    (Default|SaveGroundItems _bp_playercontrollercomponent)
    (Default|SaveShops _bp_playercontrollercomponent)))

(event Input|KeyboardEvents|O
  (params (Key :type Key%20Structure :default "None"))
  ;[1 1 1] Mouse- and keyboardinput
  ;;[1 1 1] Save & Load control
  (:Pressed
    (CallFunction|SaveEverything)))

(event Input|KeyboardEvents|1
  (params (Key :type Key%20Structure :default "None"))
  ;[1 1 1] Mouse- and keyboardinput
  (:Pressed
    (Default|ChangeSlot (Variables|Default|GetBP_PlayercontrollerComponent) false false)))

(event Input|KeyboardEvents|T
  (params (Key :type Key%20Structure :default "None"))
  ;[1 1 1] Chat system
  (:Pressed
    (Default|ToggleChat (Variables|Default|GetBP_PlayercontrollerComponent))))

(event Input|KeyboardEvents|H
  (params (Key :type Key%20Structure :default "None"))
  ;[1 1 1] Mouse- and keyboardinput
  ;;[1 1 1] Add items to inventory (for testing)
  (:Pressed
    (Default|AddItem :self (Variables|Default|GetBP_PlayercontrollerComponent) :ID_OfItem 10 :Amount 1)))

(event Input|KeyboardEvents|L
  (params (Key :type Key%20Structure :default "None"))
  ;[1 1 1] Mouse- and keyboardinput
  ;;[1 1 1] Save & Load control
  (:Pressed
    (CallFunction|LoadEverything)))

(event Input|MouseEvents|MouseWheelDown
  (params (Key :type Key%20Structure :default "None"))
  ;[1 1 1] Mouse- and keyboardinput
  (:Pressed
    (Default|ChangeSlot (Variables|Default|GetBP_PlayercontrollerComponent) false true)))

(event Input|KeyboardEvents|L
  (params (Key :type Key%20Structure :default "None"))
  ;[1 1 1] Quest stuff
  ;;[0 0.7084 1] Inputs
  (:Pressed
    (CallFunction|AddQuestTaskAmount "QT_OpenQuestInterface" 1)
    (Default|ToggleWidgetLayer (CallFunction|GetWidgetManager) "NewEnumerator1")))

(event Input|KeyboardEvents|2
  (params (Key :type Key%20Structure :default "None"))
  ;[1 1 1] Mouse- and keyboardinput
  (:Pressed
    (Default|ChangeSlot (Variables|Default|GetBP_PlayercontrollerComponent) false false 1)))

(event Input|KeyboardEvents|3
  (params (Key :type Key%20Structure :default "None"))
  ;[1 1 1] Mouse- and keyboardinput
  (:Pressed
    (Default|ChangeSlot (Variables|Default|GetBP_PlayercontrollerComponent) false false 2)))

(event Input|KeyboardEvents|G
  (params (Key :type Key%20Structure :default "None"))
  ;[1 1 1] Mouse- and keyboardinput
  ;;[1 1 1] Add items to inventory (for testing)
  (:Pressed
    (Default|AddItem :self (Variables|Default|GetBP_PlayercontrollerComponent) :Amount 20)))

(event Input|KeyboardEvents|J
  (params (Key :type Key%20Structure :default "None"))
  ;[1 1 1] Mouse- and keyboardinput
  ;;[1 1 1] Add items to inventory (for testing)
  (:Pressed
    (Default|AddItem :self (Variables|Default|GetBP_PlayercontrollerComponent) :ID_OfItem 5 :Amount 1)))

(event Input|KeyboardEvents|4
  (params (Key :type Key%20Structure :default "None"))
  ;[1 1 1] Mouse- and keyboardinput
  (:Pressed
    (Default|ChangeSlot (Variables|Default|GetBP_PlayercontrollerComponent) false false 3)))

(event Input|KeyboardEvents|5
  (params (Key :type Key%20Structure :default "None"))
  ;[1 1 1] Mouse- and keyboardinput
  (:Pressed
    (Default|ChangeSlot (Variables|Default|GetBP_PlayercontrollerComponent) false false 4)))

(event Input|KeyboardEvents|6
  (params (Key :type Key%20Structure :default "None"))
  ;[1 1 1] Mouse- and keyboardinput
  (:Pressed
    (Default|ChangeSlot (Variables|Default|GetBP_PlayercontrollerComponent) false false 5)))

(fn ConstructionScript)

(fn ConstructQuestUI
  (bind _returnvalue (CallFunction|GetWidgetManager))
  (bind (_questinterfacewidget _npcquestinterfacewidget _questtrackerwidget) (CallFunction|ConstructQuestInterface (Variables|Default|GetC_QuestComponent)))
  (Default|SetWidgetLayer _returnvalue "NewEnumerator1" (Utilities|Struct|MakeS_WidgetLayerInfo true _questinterfacewidget false false false))
  (Default|SetWidgetLayer _returnvalue "NewEnumerator2" (Utilities|Struct|MakeS_WidgetLayerInfo true _npcquestinterfacewidget false false false))
  (Default|SetWidgetLayer _returnvalue "NewEnumerator0" (Utilities|Struct|MakeS_WidgetLayerInfo false _questtrackerwidget true false false)))

(fn GetAutoPickUpModeI
  (return (Utilities|Struct|BreakPlayercontrollerVariables_Structure (Variables|/Game/AdvancedInventory/Blueprints/BP_PlayercontrollerComponent.BP_PlayercontrollerComponent_C|GetpcMasterVariable (Variables|Default|GetBP_PlayercontrollerComponent)))))

(fn GetCurrentChestRefI
  (return (Utilities|Struct|BreakPlayercontrollerVariables_Structure (Variables|/Game/AdvancedInventory/Blueprints/BP_PlayercontrollerComponent.BP_PlayercontrollerComponent_C|GetpcMasterVariable (Variables|Default|GetBP_PlayercontrollerComponent)))))

(fn GetCurrentShopRefI
  (return (Utilities|Struct|BreakPlayercontrollerVariables_Structure (Variables|/Game/AdvancedInventory/Blueprints/BP_PlayercontrollerComponent.BP_PlayercontrollerComponent_C|GetpcMasterVariable (Variables|Default|GetBP_PlayercontrollerComponent)))))

(fn GetCurrentSlotI
  (return (Utilities|Struct|BreakPlayercontrollerVariables_Structure (Variables|/Game/AdvancedInventory/Blueprints/BP_PlayercontrollerComponent.BP_PlayercontrollerComponent_C|GetpcMasterVariable (Variables|Default|GetBP_PlayercontrollerComponent)))))

(fn GetGroundRadiusI
  (return (Utilities|Struct|BreakPlayercontrollerVariables_Structure (Variables|/Game/AdvancedInventory/Blueprints/BP_PlayercontrollerComponent.BP_PlayercontrollerComponent_C|GetpcMasterVariable (Variables|Default|GetBP_PlayercontrollerComponent)))))

(fn GetInventoryRefI
  (return 0))

(fn GetIsConsumingAnItem?
  (return false))

(fn GetMoneyI
  (params (inCurrency :type Currencies_Enumeration%20Enum :default "NewEnumerator0"))
  (return 0))

(fn GetUIRefI
  (return 0))