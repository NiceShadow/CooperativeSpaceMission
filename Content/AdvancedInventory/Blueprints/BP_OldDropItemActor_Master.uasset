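; Dropped-item actor for the inventory system, either preloaded from the item data table by ID or launched as a projectile when spawned.
; When the projectile stops, it merges into an overlapping stackable item of the same ID, which plays a scale pulse.
; Overlapping an obstacle triggers expanding line traces to find free space, and recreating the projectile component lets items fall.
; Partial pickups update the amount and refresh the GameMode's ground-item list.
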(event OnProjectileStop(ProjectileMovement)
  (params (ImpactResult :type Hit%20Result%20Structure%20%28by%20ref%29))
  ;[1 1 1] If another item with the same ID comes in the radius of this item, the items will be merged
  (Utilities|FlowControl|Delay 0.25)
  (bind _array_element (Utilities|Array|ForEachLoopwithBreak (Collision|GetOverlappingActors "BP_OldDropItemActor_Master_C" :!class /Script/Engine.Actor) :!label _label)
    (:LoopBody
      (if (!= _array_element self)
        (bind _asbp_old_drop_item_actor_master (Utilities|Casting|CastToBP_OldDropItemActor_Master _array_element))
        (if (and (== (.ID (Utilities|Struct|BreakItem_Structur (Variables|BP_OldDropItemActor_Master_C|GetItemData _asbp_old_drop_item_actor_master))) (.ID (Utilities|Struct|BreakItem_Structur (Variables|Default|GetItemData)))) (.Stackable? (Utilities|Struct|BreakItem_Structur (Variables|Default|GetItemData))))
          (CallFunction|IncreaseAmountAnimation _asbp_old_drop_item_actor_master)
          (bind _structout (Utilities|Struct|SetmembersinItem_Structur (Variables|Default|GetItemData) (+ (.amount (Utilities|Struct|BreakItem_Structur (Variables|BP_OldDropItemActor_Master_C|GetItemData _asbp_old_drop_item_actor_master))) (.amount (Utilities|Struct|BreakItem_Structur (Variables|Default|GetItemData))))))
          (Variables|BP_OldDropItemActor_Master_C|SetItemData _asbp_old_drop_item_actor_master _structout)
          (Actor|DestroyActor)
          (goto _label Break))))))

(event OnComponentBeginOverlap(BoxTop)
  (params (OverlappedComponent :type Primitive%20Component%20Object%20Reference) (OtherActor :type Actor%20Object%20Reference) (OtherComp :type Primitive%20Component%20Object%20Reference) (OtherBodyIndex :type Integer) (bFromSweep :type Boolean) (SweepResult :type Hit%20Result%20Structure%20%28by%20ref%29))
  ;[1 1 1] If the item collides with a PlacingObject, a new location is necessary
  (bind (_location _itemshouldfalldown_) (CallFunction|FindWayOut))
  (Transformation|SetActorLocation (Math|Vector|MakeVector (.X (Math|Vector|BreakVector _location)) (.Y (Math|Vector|BreakVector _location)) (.Z (Math|Vector|BreakVector _location))) false false)
  (if _itemshouldfalldown_
    (CallFunction|ReactiveProjectileMovement)))

(event OnComponentEndOverlap(BoxDown)
  (params (OverlappedComponent :type Primitive%20Component%20Object%20Reference) (OtherActor :type Actor%20Object%20Reference) (OtherComp :type Primitive%20Component%20Object%20Reference) (OtherBodyIndex :type Integer))
  ;[1 1 1] When the item is on the top of a PlacingObject and this object gets destroyed ist is necessary that the item falls down
  (CallFunction|ReactiveProjectileMovement))

(event Custom|UpdateAmount
  (params (amount :type Integer))
  ;[1 1 1] Update the amount if a player picks up not 100% of the amount (only for Ground-pickup)
  (Utilities|Struct|SetmembersinItem_Structur (Variables|Default|GetItemData) amount)
  (Utilities|FlowControl|Delay 0.2)
  (Class|BPInterfaceInventory|UpdateGroundItemListI(Message) (Game|GetGameMode)))

(event Custom|IncreaseAmountAnimation
  ;[1 1 1] Animation of the scale when the amount is increased
  (if (not (Variables|Default|GetinProgress))
    (Variables|Default|SetinProgress true)
    (bind _output_get (Variables|Default|SetstartScale (Variables|/Script/Engine.SceneComponent|GetRelativeScale3D (Variables|Default|GetStaticMesh1))))
    (Variables|Default|SetendScale (* _output_get 1.2))
    (bind _newtrack_0 (Timeline|Timeline_0 PlayFromStart)
      (:Update
        (Transformation|SetRelativeScale3D (Variables|Default|GetStaticMesh1) (Math|Vector|Lerp(Vector) (Variables|Default|GetstartScale) (Variables|Default|GetendScale) _newtrack_0)))
      (:Finished
        (Variables|Default|SetinProgress false)))))

(event EventBeginPlay
  (bind _returnvalue (Utilities|Name|MakeLiteralName "NewRow"))
  (bind _id_atstart (Variables|Default|GetID_AtStart))
  (bind _id_atstart_2 (Variables|Default|GetID_AtStart))
  (bind _returnvalue_2 (== _id_atstart_2 0))
  (bind _returnvalue_3 (- _id_atstart 1))
  (bind _returnvalue_4 (Utilities|String|ToString(Integer) _returnvalue_3))
  (bind _returnvalue_5 (Utilities|String|Append "NewRow_" _returnvalue_4))
  (bind _returnvalue_6 (Utilities|String|StringToName _returnvalue_5))
  (bind _returnvalue_7 (select _returnvalue_2 _returnvalue _returnvalue_6))
  ;[1 1 1] Spawn At Start
  (if (Variables|Default|GetSpawnAtStart?)
    (bind _returnvalue_8 (Class|DataTableFunctionLibrary|DoesDataTableRowExist "/Game/AdvancedInventory/Item_Table.Item_Table" _returnvalue_7))
    (if _returnvalue_8
      (bind _returnvalue_9 (Utilities|GetDataTableRow "/Game/AdvancedInventory/Item_Table.Item_Table" _returnvalue_7)
        (:then
          (bind _output_get (Variables|Default|SetItemData _returnvalue_9))
          (Utilities|Struct|SetmembersinItem_Structur _output_get (Variables|Default|GetAmount_AtStart))
          ;[1 1 1] Setup item
          (Components|Movement|SetUpdatedComponent (Variables|Default|GetProjectileMovement) (Variables|Default|GetitemCollisionMesh) :!label _label)
          (Components|StaticMesh|SetStaticMesh (Variables|Default|GetStaticMesh1) (.StaticMesh (Utilities|Struct|BreakItem_Structur (Variables|Default|GetItemData))))
          (Transformation|SetRelativeTransform (Variables|Default|GetStaticMesh1) (.DropTransform (Utilities|Struct|BreakItem_Structur (Variables|Default|GetItemData))) false false))))
    (else
      (Game|Components|ProjectileMovement|SetVelocityinLocalSpace (Variables|Default|GetProjectileMovement) (Math|Vector|MakeVector (+ 6e+02 (Variables|Default|GetxVelocity)) 0.0 (Variables|Default|GetzVelocity)))
      (goto _label))))

(fn ConstructionScript
  (bind _returnvalue (Utilities|Name|MakeLiteralName "NewRow"))
  (bind _id_atstart (Variables|Default|GetID_AtStart))
  (bind _staticmesh1 (Variables|Default|GetStaticMesh1))
  (bind _id_atstart_2 (Variables|Default|GetID_AtStart))
  (bind _returnvalue_2 (== _id_atstart_2 0))
  (bind _returnvalue_3 (- _id_atstart 1))
  (bind _returnvalue_4 (Utilities|String|ToString(Integer) _returnvalue_3))
  (bind _returnvalue_5 (Utilities|String|Append "NewRow_" _returnvalue_4))
  (bind _returnvalue_6 (Utilities|String|StringToName _returnvalue_5))
  (bind _returnvalue_7 (select _returnvalue_2 _returnvalue _returnvalue_6))
  (if (Variables|Default|GetSpawnAtStart?)
    (bind _returnvalue_8 (Class|DataTableFunctionLibrary|DoesDataTableRowExist "/Game/AdvancedInventory/Item_Table.Item_Table" _returnvalue_7))
    (if _returnvalue_8
      (bind _returnvalue_9 (Utilities|GetDataTableRow "/Game/AdvancedInventory/Item_Table.Item_Table" _returnvalue_7)
        (:then
          (Components|StaticMesh|SetStaticMesh _staticmesh1 (.StaticMesh (Utilities|Struct|BreakItem_Structur _returnvalue_9)))
          (Transformation|SetRelativeTransform _staticmesh1 (.DropTransform (Utilities|Struct|BreakItem_Structur _returnvalue_9)) false false)
          (Rendering|SetVisibility (Variables|Default|GetitemCollisionMesh) false false))))))

(fn ReactiveProjectileMovement
  (bind _projectilemovement (Variables|Default|GetProjectileMovement))
  ;[1 1 1] Destroy the current ProjectileComponent and create a new one
  (Utilities|IsValid _projectilemovement
    (:Is%20Valid
      (Components|DestroyComponent _projectilemovement))
    (:Is%20Not%20Valid
      (Utilities|IsValid (Variables|Default|GetNewProjectileMovement)
        (:Is%20Valid
          (Components|DestroyComponent (Variables|Default|GetNewProjectileMovement)))
        (:Is%20Not%20Valid
          _))))
  (bind _returnvalue (AddComponent|AddProjectileMovementComponent))
  (Variables|Default|SetNewProjectileMovement _returnvalue))

(fn FindWayOut
  ;[1 1 1] The function checks all directions (not bottom). Distance of Linetrace 0: Linetrace is still in a Object of the type "PlacingObject"   I   Distance of the Linetrace >0: Linetrace doesn't collide with a PlacingObject -> ReturnsLocation
  (Math|Integer|IncrementInt (LocalVariables|Getcount2) :!label _label
    (:%20%20
      (for _index (range 0 4)
        (bind _output_get (LocalVariables|SetcheckDirection (Utilities|Select :Index _index :Option%200 "0, 0,50.000000" :Option%201 "0,-50.000000, 0" :Option%202 "0,50.000000, 0" :Option%203 "50.000000, 0, 0" :Option%204 "-50.000000, 0, 0")))
        (bind _outhit (Collision|LineTraceByChannel (+ (* _output_get (+ (LocalVariables|Getcount2) 1)) (Transformation|GetActorLocation) "0,0.000000,15.000000") (+ (* _output_get (LocalVariables|Getcount2)) (Transformation|GetActorLocation) "0,0.000000,15.000000") "TraceTypeQuery3" false 0 "None"))
        (if (not (== (.Distance (Collision|BreakHitResult _outhit)) 0.0))
          (return (+ (.Location (Collision|BreakHitResult _outhit)) (select (== _index 0) "0, 0, 0" (LocalVariables|GetcheckDirection))) (not (== _index 0)))))
      (goto _label))))