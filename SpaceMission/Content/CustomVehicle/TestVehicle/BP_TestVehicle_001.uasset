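; Test drivable vehicle pawn built on SimpleWheeledVehicleMovement, with input wired directly to per-wheel calls.
; MoveForward applies drive torque to all four wheels, and MoveRight steers wheels 0 and 1.
; Handbrake applies brake torque to wheels 1 and 3 (one steered, one unsteered) while held.
; LookUp and LookRight rotate the SpringArm for camera control by raw axis value, with no delta-time scaling or clamping.
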(event Input|ActionEvents|InputActionHandbrake
  (params (Key :type Key%20Structure :default "None"))
  (bind _simplewheeledvehiclemovement (Variables|Default|GetSimpleWheeledVehicleMovement))
  ;[1 1 1] Handbrake
  (:Pressed
    (Class|SimpleWheeledVehicleMovementComponent|SetBrakeTorque _simplewheeledvehiclemovement 2e+03 1)
    (Class|SimpleWheeledVehicleMovementComponent|SetBrakeTorque _simplewheeledvehiclemovement 2e+03 3))
  (:Released
    (Class|SimpleWheeledVehicleMovementComponent|SetBrakeTorque _simplewheeledvehiclemovement 0.0 1)
    (Class|SimpleWheeledVehicleMovementComponent|SetBrakeTorque _simplewheeledvehiclemovement 0.0 3)))

(event Input|AxisEvents|InputAxisLookUp
  (params (AxisValue :type Float%20%28single-precision%29))
  ;[1 1 1] Camera rotation
  (Transformation|AddRelativeRotation (Variables|Default|GetSpringArm) (Math|Rotator|MakeRotator 0.0 AxisValue 0.0) false false))

(event Input|AxisEvents|InputAxisLookRight
  (params (AxisValue :type Float%20%28single-precision%29))
  ;[1 1 1] Camera rotation
  (Transformation|AddRelativeRotation (Variables|Default|GetSpringArm) (Math|Rotator|MakeRotator 0.0 0.0 AxisValue) false false))

(event Input|AxisEvents|InputAxisMoveRight
  (params (AxisValue :type Float%20%28single-precision%29))
  (bind _returnvalue (* AxisValue 33.0))
  (bind _simplewheeledvehiclemovement (Variables|Default|GetSimpleWheeledVehicleMovement))
  ;[1 1 1] movement
  (Class|SimpleWheeledVehicleMovementComponent|SetSteerAngle _simplewheeledvehiclemovement _returnvalue)
  (Class|SimpleWheeledVehicleMovementComponent|SetSteerAngle _simplewheeledvehiclemovement _returnvalue 1))

(event Input|AxisEvents|InputAxisMoveForward
  (params (AxisValue :type Float%20%28single-precision%29))
  (bind _returnvalue (* AxisValue 5e+02))
  (bind _simplewheeledvehiclemovement (Variables|Default|GetSimpleWheeledVehicleMovement))
  ;[1 1 1] movement
  (Class|SimpleWheeledVehicleMovementComponent|SetDriveTorque _simplewheeledvehiclemovement _returnvalue 2)
  (Class|SimpleWheeledVehicleMovementComponent|SetDriveTorque _simplewheeledvehiclemovement _returnvalue 3)
  (Class|SimpleWheeledVehicleMovementComponent|SetDriveTorque _simplewheeledvehiclemovement _returnvalue)
  (Class|SimpleWheeledVehicleMovementComponent|SetDriveTorque _simplewheeledvehiclemovement _returnvalue 1))

(fn ConstructionScript)