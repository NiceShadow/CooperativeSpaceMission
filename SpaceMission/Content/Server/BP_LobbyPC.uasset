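; Lobby player controller that links each player's lobby UI to BP_LobbyGM for character selection, ready state, chat, countdown and game start.
; Player requests forward to the game mode, whose results return through events that update the LobbyRef widgets, with a delay if that reference is not yet valid.
; On BeginPlay it sets UI-only input, caps FPS and sets a timer to update the save slot date via FriendsIntance.
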(event Custom|UpdatePlayerList
  (params (IDs :type Array%20of%20Player%20Widget%20Update%20Structure%20Structures))
  (Utilities|IsValid (Variables|Default|GetLobbyRef)
    (:Is%20Valid
      _)
    (:Is%20Not%20Valid
      (Utilities|FlowControl|Delay 1.0)))
  (Default|UpdatePlayerList (Variables|Default|GetLobbyRef) IDs))

(event Custom|ApprovedSelectCharacter
  (params (Index :type Integer))
  (bind _output_get (Variables|Default|SetSelectedCharacterIndex Index))
  (CallFunction|SetCharIndexServer _output_get)
  (Default|EnableReadyButton (Variables|Default|GetLobbyRef) (>= _output_get 0))
  (if (and (not (>= _output_get 0)) (Variables|Default|GetReadyServer))
    (CallFunction|ToggleReady)))

(event Custom|ShowLoadingScreen
  (bind _returnvalue (UserInterface|CreateWidget "/Game/Server/Widgets/WB_LoadingScreen.WB_LoadingScreen_C"))
  (UserInterface|Viewport|AddtoViewport _returnvalue 1))

(event Custom|Setup
  (params (LobbyRef :type WB%20Lobby%20Object%20Reference))
  (Variables|Default|SetLobbyRef LobbyRef))

(event Custom|UpdateCharactersList
  (params (availableChars :type Array%20of%20Booleans))
  (Utilities|IsValid (Variables|Default|GetLobbyRef)
    (:Is%20Valid
      _)
    (:Is%20Not%20Valid
      (Utilities|FlowControl|Delay 1.0)))
  (Default|Update (Variables|/Game/Server/Widgets/WB_Lobby.WB_Lobby_C|GetWB_CharacterSelection (Variables|Default|GetLobbyRef)) availableChars))

(event Custom|SetReadyServer
  (params (ReadyServer :type Boolean))
  (Variables|Default|SetReadyServer ReadyServer))

(event Custom|SetCharIndexServer
  (params (SelectedCharacterIndex :type Integer))
  (Variables|Default|SetSelectedCharacterIndex SelectedCharacterIndex)
  (Default|UpdateCharacterList (CallFunction|GetLobbyGM)))

(event Custom|UpdateCharListGM
  (Default|UpdateCharacterList (CallFunction|GetLobbyGM)))

(event Custom|SendChatMessage
  (params (PC :type Player%20Controller%20Object%20Reference) (Message :type String))
  (Default|AddTextMessage (CallFunction|GetLobbyGM) PC Message false))

(event Custom|AddChatMessage
  (params (Name :type String) (Message :type String) (ServerMessage :type Boolean))
  (bind _lobbyref (Variables|Default|GetLobbyRef))
  (Utilities|IsValid _lobbyref
    (:Is%20Valid
      _)
    (:Is%20Not%20Valid
      (Utilities|FlowControl|Delay 1.0)))
  (Default|AddMessage (Variables|/Game/Server/Widgets/WB_Lobby.WB_Lobby_C|GetWB_LobbyChatWindow _lobbyref) Name Message ServerMessage))

(event Custom|UpdateDateInSaveList
  (bind _asfriends_intance (Utilities|Casting|CastToFriendsIntance (Game|GetGameInstance)))
  (Default|UpdateCurrentSlotDate _asfriends_intance))

(event Custom|UpdatePlayerListGM
  (Default|UpdatePlayerList (CallFunction|GetLobbyGM)))

(event Custom|AskServerToSelectCharacter
  (params (Index :type Integer))
  (if (== Index (Variables|Default|GetSelectedCharacterIndex))
    (CallFunction|DeselectCharacterServer Index)
    (bind _output_get (Variables|Default|SetSelectedCharacterIndex -1))
    (CallFunction|SetCharIndexServer _output_get)
    (else
      (CallFunction|AskServertoSelectCharacterServer Index))))

(event Custom|AskServerToSelectCharacterServer
  (params (Index :type Integer))
  (Default|SelectCharacter (CallFunction|GetLobbyGM) Index self))

(event Custom|DeselectCharacterServer
  (params (Index :type Integer))
  (Default|DeselectCharacter (CallFunction|GetLobbyGM) Index self))

(event Custom|ToggleReady
  (bind _output_get (Variables|Default|SetReadyServer (not (Variables|Default|GetReadyServer))))
  (CallFunction|SetReadyServer _output_get)
  (CallFunction|UpdatePlayerListGM))

(event Custom|StartGame
  (Default|StartGame (CallFunction|GetLobbyGM)))

(event Custom|ShowCountdown
  (Default|StartCountdown (Variables|Default|GetLobbyRef)))

(event Custom|CountdownGM
  (Default|ShowCountdown (CallFunction|GetLobbyGM)))

(event EventBeginPlay
  (bind _returnvalue (Math|Float|MakeLiteralFloat 3.0))
  (Variables|Default|SetbShowMouseCursor true)
  (Input|SetInputModeUIOnly self 0 "DoNotLock")
  (Development|ExecuteConsoleCommand "t. maxfps 80" 0)
  (Utilities|Time|SetTimerbyEvent (delegate Custom|UpdateDateInSaveList) _returnvalue false (* _returnvalue -1.0)))

(fn ConstructionScript)

(fn GetLobbyGM
  (bind _asbp_lobby_gm (Utilities|Casting|CastToBP_LobbyGM (Game|GetGameMode)))
  (return _asbp_lobby_gm))