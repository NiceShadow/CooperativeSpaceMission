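; BP_InventoryPlayerState is the inventory system's player state, storing the player's Gold, Silver and Prize Tickets balances.
; Through inventory interface functions, it adds to the chosen currency, then sends the new total to player controller 0 via an UpdateMoney message.
; GetMoney returns the balance for a requested currency, while the other interface getters are stubs returning empty or default values.
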(event EventAddMoneytoPlayerI
  (params (MoneyToAdd :type Integer) (Currency :type Currencies_Enumeration%20Enum :default "NewEnumerator0"))
  ;[1 1 1] Add money
  (switch Utilities|FlowControl|Switch|SwitchonCurrencies_Enumeration Currency
    (:NewEnumerator0
      (Variables|Default|SetGold (+ MoneyToAdd (Variables|Default|GetGold))))
    (:NewEnumerator1
      (Variables|Default|SetSilver (+ MoneyToAdd (Variables|Default|GetSilver))))
    (:NewEnumerator2
      (Variables|Default|SetPrizeTickets (+ MoneyToAdd (Variables|Default|GetPrizeTickets)))))
  (Class|BPInterfaceInventory|UpdateMoneyI(Message) (Game|GetPlayerController 0) (Utilities|Select :Index Currency :NewEnumerator0 (Variables|Default|GetGold) :NewEnumerator1 (Variables|Default|GetSilver) :NewEnumerator2 (Variables|Default|GetPrizeTickets)) Currency))

(fn ConstructionScript)

(fn GetAutoPickUpModeI
  (return false))

(fn GetCurrentChestRefI
  (return 0))

(fn GetCurrentShopRefI
  (return 0))

(fn GetCurrentSlotI
  (return 0))

(fn GetGroundRadiusI
  (return 0))

(fn GetInventoryRefI
  (return 0))

(fn GetMoneyI
  (params (inCurrency :type Currencies_Enumeration%20Enum :default "NewEnumerator0"))
  (return (Utilities|Select :Index inCurrency :NewEnumerator0 (Variables|Default|GetGold) :NewEnumerator1 (Variables|Default|GetSilver) :NewEnumerator2 (Variables|Default|GetPrizeTickets))))

(fn GetUIRefI
  (return 0))