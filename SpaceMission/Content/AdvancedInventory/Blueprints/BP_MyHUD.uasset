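; BP_MyHUD is the HUD Blueprint for the inventory system, creating the main WB_UI widget and exposing it to other objects through interface-style functions.
; Setup runs on BeginPlay and, in packaged distribution builds, also shows a loading screen briefly.
; Events forward item adding, crafting refreshes, visibility toggles and first hotbar slot selection to the inventory widget, also managing the crosshair.
; Only the UI and inventory getters are implemented; the others are stubs.
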(event Custom|Setup
  ;[1 1 1] Setup
  ;;[1 1 1] Create UI and add it to viewport
  (bind _returnvalue (UserInterface|CreateWidget "/Game/AdvancedInventory/Widgets/WB_UI.WB_UI_C"))
  (bind _output_get (Variables|Default|SetUI_Ref _returnvalue))
  (UserInterface|Viewport|AddtoViewport _output_get 0)
  (if (Class|KismetSystemLibrary|IsPackagedforDistribution)
    (bind _returnvalue_2 (UserInterface|CreateWidget "/Game/Server/Widgets/WB_LoadingScreen.WB_LoadingScreen_C"))
    (UserInterface|Viewport|AddtoViewport _returnvalue_2 1)
    (Utilities|FlowControl|Delay 2.0)
    (Default|Hide _returnvalue_2)))

(event EventBeginPlay
  ;[1 1 1] Setup
  ;;[1 1 0 1 20] NOTE: You can't have 2 'EventBeginPlay' at the same time in one blueprint.
  ;; If you copy this BP make sure to add 'Setup' to your existing
  ;; 'EventBeginPlay' (if you have one)
  (CallFunction|Setup))

(event EventToggleInventoryVisibilityI
  (params (Show? :type Boolean) (OnlyInteraction :type Boolean))
  (bind _ui_ref (Variables|Default|GetUI_Ref))
  (bind _ui_ref_2 (Variables|Default|GetUI_Ref))
  (bind _inventory (Variables|/Game/AdvancedInventory/Widgets/WB_UI.WB_UI_C|GetInventory _ui_ref_2))
  (bind _crosshairswitcher (Variables|/Game/AdvancedInventory/Widgets/WB_UI.WB_UI_C|GetCrosshairSwitcher _ui_ref))
  ;[1 1 1] Toggle visibility of main inventory
  (Utilities|IsValid _ui_ref_2
    (:Is%20Valid
      (if OnlyInteraction
        _
        (else
          (Default|ShowHideInventory _inventory Show?)))
      (if Show?
        (Widget|SetVisibility _crosshairswitcher "Collapsed")
        (if (not Show?) :!label _label
          (Widget|SetVisibility (Variables|/Game/AdvancedInventory/Widgets/WB_Inventory.WB_Inventory_C|GetRightClickMenuRef _inventory) "Collapsed"))
        (elif OnlyInteraction
          (Widget|SetVisibility _crosshairswitcher "Visible" :!label _label_2)
          (goto _label)
          (elif (not (Widget|IsVisible (Variables|/Game/AdvancedInventory/Widgets/WB_Inventory.WB_Inventory_C|GetChestUI (Variables|/Game/AdvancedInventory/Widgets/WB_UI.WB_UI_C|GetInventory _ui_ref))))
            (goto _label_2)))))))

(event EventAddItemI
  (params (ID_OfItem :type Integer) (Amount :type Integer) (Data :type Item%20Structur%20Structure) (TransferWholeItemData :type Boolean) (IsBackpack? :type Boolean) (BackpackData :type Backpack%20Data%20Structure%20Structure))
  (bind _ui_ref (Variables|Default|GetUI_Ref))
  ;[1 1 1] Add item to inventory
  (Utilities|IsValid _ui_ref
    (:Is%20Valid
      (Default|AddItem (Variables|/Game/AdvancedInventory/Widgets/WB_UI.WB_UI_C|GetInventory _ui_ref) ID_OfItem Amount false 0 Data TransferWholeItemData false BackpackData 0.0))))

(event EventSelectFirstSlotinHotbarI
  ;[1 1 1] Setup
  (bind _aswb_slot (Utilities|Casting|CastToWB_Slot (Class|PanelWidget|GetChildat (Variables|/Game/AdvancedInventory/Widgets/WB_Inventory.WB_Inventory_C|GetHotbar (Variables|/Game/AdvancedInventory/Widgets/WB_UI.WB_UI_C|GetInventory (Variables|Default|GetUI_Ref))))))
  (Default|Select _aswb_slot true))

(event EventUpdateCraftItemsI
  (bind _ui_ref (Variables|Default|GetUI_Ref))
  ;[1 1 1] Update craftable items
  (Utilities|IsValid _ui_ref
    (:Is%20Valid
      (Default|UpdateCraftItems (Variables|/Game/AdvancedInventory/Widgets/WB_UI.WB_UI_C|GetInventory _ui_ref) false))))

(fn ConstructionScript)

(fn GetAutoPickUpModeI
  (return false))

(fn GetCurrentChestRefI
  (return 0))

(fn GetCurrentShopRefI
  (return 0))

(fn GetCurrentSlotI
  (return 0))

(fn GetGroundRadiusI
  (return 0))

(fn GetInventoryRefI
  (bind _ui_ref (Variables|Default|GetUI_Ref))
  (Utilities|IsValid _ui_ref
    (:Is%20Valid
      (return (Variables|/Game/AdvancedInventory/Widgets/WB_UI.WB_UI_C|GetInventory _ui_ref)))))

(fn GetMoneyI
  (params (inCurrency :type Currencies_Enumeration%20Enum :default "NewEnumerator0"))
  (return 0))

(fn GetUIRefI
  (bind _ui_ref (Variables|Default|GetUI_Ref))
  (Utilities|IsValid _ui_ref
    (:Is%20Valid
      (return _ui_ref))))