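; BP_InterfaceInventory is the Blueprint Interface of the inventory system, declaring messages that let actors, components and UI communicate without casting.
; It covers item add, drop and pickup, hotbar and equip slots, drag operations, chests, crafting, campfire cooking, shops, money and player trading.
; It holds only signatures: getters return references or values, while the other functions pass updates, focus changes and save-load data to implementers.
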(fn DestroyActorI
  (params (Actor :type Actor%20Object%20Reference)))

(fn UpdateGroundItemListI)

(fn ToggleInventoryVisibilityI
  (params (Show? :type Boolean) (OnlyInteraction :type Boolean)))

(fn DropItemI
  (params (Data :type Item%20Structur%20Structure) (BackpackData :type Backpack%20Data%20Structure%20Structure)))

(fn GetInventoryRefI
  (return 0))

(fn AddItemI
  (params (ID_OfItem :type Integer) (Amount :type Integer) (Data :type Item%20Structur%20Structure) (TransferWholeItemData :type Boolean) (IsBackpack? :type Boolean) (BackpackData :type Backpack%20Data%20Structure%20Structure)))

(fn SelectFirstSlotinHotbarI)

(fn UpdateHotbarSlotsI)

(fn UpdateEquipSlotI
  (params (EquipSlot :type Object%20Object%20Reference) (fromEquipSlot? :type Boolean) (itemRefOnlyForEquipSlot :type WB%20Item%20Object%20Reference)))

(fn CancelShiftItemI)

(fn SetCurrentDragOPRefI
  (params (DragOP :type Drag%20Drop%20Operation%20Object%20Reference) (CurrentItem_Ref :type WB%20Item%20Object%20Reference) (ChestSlotIndex :type Integer)))

(fn SetCurrentDragOPOtherRefI
  (params (DragOP_Other :type WB%20Item%20Object%20Reference)))

(fn SetChestRefI
  (params (CurrentChestRef :type BP%20Chest%20Object%20Reference)))

(fn UpdateChestI
  (params (UpdateChestData :type Update%20Chest%20Structure%20Structure)))

(fn GetCurrentChestRefI
  (return 0))

(fn UpdateItemAmountI
  (params (Amount :type Integer) (Actor :type Actor%20Object%20Reference)))

(fn SetInventoryComponentRefI
  (params (InventoryComponent :type BP%20Inventory%20Componenent%20Object%20Reference)))

(fn GetAutoPickUpModeI
  (return false))

(fn GetGroundRadiusI
  (return 0))

(fn SetAutoPickRadiusandGroundRadiusI
  (params (AutoPick :type Sphere%20Component%20Object%20Reference) (Ground :type Sphere%20Component%20Object%20Reference)))

(fn GetCurrentSlotI
  (return 0))

(fn UpdateElementinChestUII
  (params (UpdateChestData :type Update%20Chest%20Structure%20Structure)))

(fn EnableDragOPI
  (params (IsEnabled :type Boolean) (ItemData :type Item%20Structur%20Structure) (UpdateAmountBeforeDragOF_Item :type Integer)))

(fn UpdateOtherItemI
  (params (ItemData :type Item%20Structur%20Structure) (BackpackData :type Backpack%20Data%20Structure%20Structure)))

(fn AddItemtoChestUII
  (params (ID :type Integer) (Amount :type Integer) (ShiftFromChest? :type Boolean)))

(fn UpdateAmountOfASpecificItemI
  (params (Actor :type Actor%20Object%20Reference) (Amount :type Integer)))

(fn UpdateChestGameModeI
  (params (UpdateChestData :type Update%20Chest%20Structure%20Structure)))

(fn LoadChestSlotsI
  (params (ChestSaveData :type Array%20of%20Chest%20Save%20Structure%20Structures) (OverwriteIfAlreadyLoaded? :type Boolean)))

(fn UpdateOwnChestUII)

(fn UpdateCraftItemsI)

(fn OpenChestwithKeyI)

(fn SetFocusedChestI
  (params (FocusedChestRef :type BP%20Chest%20Object%20Reference)))

(fn SetIsinRadiusOfChestI
  (params (inRadius? :type Boolean)))

(fn FinishedConsumeItemI)

(fn AddItemsInstantI
  (params (itemsToAdd :type Array%20of%20Item%20Structur%20Structures)))

(fn CheckCookingI
  (params (ChestRef :type BP%20Chest%20Object%20Reference) (ResetSecondsCooked :type Boolean) (ResetAtSlot :type Integer)))

(fn UpdateCookingUII
  (params (Chest :type BP%20Chest%20Object%20Reference) (Percent :type Array%20of%20Integers) (RemoveFuelItem :type Boolean) (FuelReduceID :type Integer) (DecreaseCookingItemAndAdd :type Array%20of%20Booleans) (AddSlot :type Array%20of%20Integers) (AddID :type Array%20of%20Integers) (AmountsToAdd :type Array%20of%20Integers)))

(fn UpdateOwnCookingUII
  (params (Percent :type Array%20of%20Integers) (RemoveFuelItem :type Boolean) (FuelReduceID :type Integer) (DecreaseCookingItemAndAdd :type Array%20of%20Booleans) (AddSlot :type Array%20of%20Integers) (AddID :type Array%20of%20Integers) (AddAmount :type Array%20of%20Integers)))

(fn GetUIRefI
  (return 0))

(fn LoadGroundItemsI
  (params (items :type Array%20of%20Ground%20Item%20Save%20Structure%20Structures)))

(fn SetFocusedShopI
  (params (BP_ShopRef :type BP%20Shop%20Object%20Reference)))

(fn SetShopRefI
  (params (CurrentShopRef :type BP%20Shop%20Object%20Reference)))

(fn SellProductI
  (params (product%20data :type Product%20Structure%20Structure)))

(fn UpdateShopUII
  (params (ShopRef :type BP%20Shop%20Object%20Reference) (products :type Array%20of%20Product%20Structure%20Structures)))

(fn GetCurrentShopRefI
  (return 0))

(fn BuyProductI
  (params (buyData :type Buy%20Product%20Structure%20Structure)))

(fn AddProducttoPlayerI
  (params (itemToAdd :type Item%20Structur%20Structure) (price :type Integer)))

(fn AddMoneyAfterSelltoPlayerI
  (params (Money :type Integer)))

(fn AddMoneytoPlayerI
  (params (MoneyToAdd :type Integer) (Currency :type Currencies_Enumeration%20Enum :default "Currencies_Enumeration_MAX")))

(fn UpdateMoneyI
  (params (newMoney :type Integer) (Currency :type Currencies_Enumeration%20Enum :default "Currencies_Enumeration_MAX")))

(fn SetFocusedCharacterI
  (params (CharacterRef :type Actor%20Object%20Reference)))

(fn AskPlayertoTradeI
  (params (fromPC :type Player%20Controller%20Object%20Reference)))

(fn UpdateTradeUII
  (params (data :type Update%20Trade%20UI%20Structure%20Structure) (FromPC :type Player%20Controller%20Object%20Reference)))

(fn UpdateOtherTadeUII
  (params (data :type Update%20Trade%20UI%20Structure%20Structure)))

(fn TradeAlreadyCanceledI)

(fn GetMoneyI
  (params (inCurrency :type Currencies_Enumeration%20Enum :default "Currencies_Enumeration_MAX"))
  (return 0))

(fn LoadShopsI
  (params (ShopsData :type Array%20of%20Shop%20Save%20Structure%20Structures)))

(fn ToggleCampfireFireI
  (params (turnOn :type Boolean) (CestRef :type BP%20Chest%20Object%20Reference) (fromPC :type Player%20Controller%20Object%20Reference)))

(fn ToggleCampfireFireActorI
  (params (TurnOn :type Boolean)))

(fn TurnOffCampfireFireUII
  (params (Chest :type BP%20Chest%20Object%20Reference)))