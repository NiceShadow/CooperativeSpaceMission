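; Shop actor that holds a product list and toggles a press-F interaction widget for opening it.
; On BeginPlay, each AI starting product rolls against its offer probability and gets a random amount if stackable, with authority adding successes.
; Products combine item DataTable rows, found by NewRow_N names derived from ID, with amount-based AI prices and hardcoded per-ID descriptions.
; Events add single products or replace the whole list for game loading.
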(event Custom|AddProduct
  (params (product%20data :type Product%20Structure%20Structure))
  ;[1 1 1] Add product to products array on server
  (Utilities|Array|Add (Variables|Default|GetProducts) product%20data))

(event Custom|UpdateWholeShopData
  (params (Products :type Array%20of%20Product%20Structure%20Structures))
  ;[1 1 1] Update product array on server (needed for LoadGame)
  (Variables|Default|SetProducts Products))

(event Custom|ShowPressInteractionWidget
  (params (Show? :type Boolean))
  ;[1 1 1] Show interaction widget locally to open the shop
  (Development|SetHiddeninGame (Variables|Default|GetPressF_Widget) (not Show?) false))

(event EventBeginPlay
  ;[1 1 1] Setup
  (for _array_element (Variables|Default|GetAI_StartingProducts)
    (bind (_add_ _productdata) (CallFunction|CreateAIStartingProducts _array_element))
    (if _add_
      (Networking|SwitchHasAuthority
        (:Authority
          (CallFunction|AddProduct _productdata))))))

(fn ConstructionScript)

(fn CreateAIStartingProducts
  (params (AI_ShopProduct_Structure :type AI%20Shop%20Product%20Structure%20Structure%20%28by%20ref%29))
  (LocalVariables|SetAI_StartingProduct_Local AI_ShopProduct_Structure)
  ;[1 1 1] Generate random number and continue based on probability
  (bind _output_get (LocalVariables|SetRandomProbability_Local (Math|Random|RandomIntegerinRange 0 100)))
  (if (>= (Utilities|Struct|BreakAI_ShopProduct_Structure (LocalVariables|GetAI_StartingProduct_Local)) _output_get)
    ;[1 1 1] Save item data based on ID in variable
    (LocalVariables|SetCurrentItemData_Local (CallFunction|GetItemDatabyID (Utilities|Struct|BreakAI_ShopProduct_Structure (LocalVariables|GetAI_StartingProduct_Local))))
    ;[1 1 1] set amount
    (if (not (.Stackable? (Utilities|Struct|BreakItem_Structur (LocalVariables|GetCurrentItemData_Local))))
      (LocalVariables|SetAmount_Local 1)
      (else
        (LocalVariables|SetAmount_Local (Math|Random|RandomIntegerinRange (.AmountMin (Utilities|Struct|BreakAI_ShopProduct_Structure (LocalVariables|GetAI_StartingProduct_Local))) (.AmountMax (Utilities|Struct|BreakAI_ShopProduct_Structure (LocalVariables|GetAI_StartingProduct_Local)))))))
    ;[1 1 1] Prevent adding if amount is 0 or less
    (if (> (LocalVariables|GetAmount_Local) 0)
      ;[1 1 1] Update amount in item data
      (Utilities|Struct|SetmembersinItem_Structur (LocalVariables|GetCurrentItemData_Local) (LocalVariables|GetAmount_Local))
      ;[1 1 1] Set quantitiy
      (LocalVariables|SetQuantity_Local 1)
      (return true (Utilities|Struct|MakeProduct_Structure (LocalVariables|GetCurrentItemData_Local) (Math|Float|Truncate (* (LocalVariables|GetAmount_Local) (.BuyPriceAi (Utilities|Struct|BreakItem_Structur (LocalVariables|GetCurrentItemData_Local))))) (LocalVariables|GetQuantity_Local) (LocalVariables|GetAmount_Local) (CallFunction|AIDescriptionbyID (.ID (Utilities|Struct|BreakItem_Structur (LocalVariables|GetCurrentItemData_Local)))) 0 "ShopOwner"))
      (else
        (return false "")))
    (else
      (return false ""))))

(fn GetItemDatabyID
  (params (ID :type Integer))
  (bind _returnvalue (Utilities|GetDataTableRow "/Game/AdvancedInventory/Item_Table.Item_Table" (select (== ID 0) (Utilities|Name|MakeLiteralName "NewRow") (Utilities|String|StringToName (Utilities|String|Append "NewRow_" (Utilities|String|ToString(Integer) (- ID 1))))))
    (:then
      (return _returnvalue))))

(fn AIDescriptionbyID
  (params (ID :type Integer))
  (switch int ID
    (:Default
      (return "Change the AI Description in BP_Shop -> AI_DescriptionByID"))
    (:0
      (return "Wood for a cheap price!"))
    (:1
      (return "Stone!"))))